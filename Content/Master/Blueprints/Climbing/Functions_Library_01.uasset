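; Blueprint function library of helpers for the climbing system, built on ALS component-and-transform structs.
; FL_WorldToLocal(Matrix) converts a world transform into its component's local space by multiplying it with the inverse of that component's scale-free world matrix, keeping the component reference.
; Climbing Foot IKTrace declares character, direction, sphere radius, offset and debug inputs for a foot IK trace, but its body is empty.
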(fn `Climbing Foot IKTrace`
  (params (character :type "Character Object Reference") (center :type "Vector Structure") (direction :type "Vector Structure") (`Down/UpTraceHeight` :type "Vector2D Structure") (`sphere radius` :type "Float (double-precision)") (`debug type` :type "EDrawDebugTrace Enum" :default "None") (`right offset` :type "Float (double-precision)")))

(fn `FL_WorldToLocal(Matrix)`
  (params (World :type "/Game/AdvancedLocomotionV4/Data/Structs/ALS_ComponentAndTransform Structure (by ref)"))
  (returns (Local :type "/Game/AdvancedLocomotionV4/Data/Structs/ALS_ComponentAndTransform Structure"))
  (bind (_transform _component) (break `/Game/AdvancedLocomotionV4/Data/Structs/ALS_ComponentAndTransform` World))
  (bind (_world_transform _world_component) (break `/Game/AdvancedLocomotionV4/Data/Structs/ALS_ComponentAndTransform` (`local.World`)))
  (return (make `/Game/AdvancedLocomotionV4/Data/Structs/ALS_ComponentAndTransform` (`KismetMathLibrary.Conv_MatrixToTransform` (* (`KismetMathLibrary.Conv_TransformToMatrix` _transform) (`KismetMathLibrary.Matrix_GetInverse` (`KismetMathLibrary.Matrix_GetMatrixWithoutScale` (`KismetMathLibrary.Conv_TransformToMatrix` (`SceneComponent.K2_GetComponentToWorld` _component)))))) _world_component)))