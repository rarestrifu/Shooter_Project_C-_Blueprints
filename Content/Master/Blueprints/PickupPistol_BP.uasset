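; Pistol pickup actor that shows a pickup prompt and flags the player as able to pick up the pistol.
; A trigger component caches the overlapping Player_BP and toggles an in-range state.
; While in range, Tick compares camera forward against the Arrow's forward by dot product, requiring roughly opposed directions.
; The result sets or clears the player's WeaponPickupUI text and CanPickUpPistol; the pickup itself is not handled here.
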(event `self.ReceiveBeginPlay`)

(event `self.ReceiveTick`
  (params (DeltaSeconds :type "Float (single-precision)"))
  (bind _player_ref (`self.Player Ref`))
  (bind _player_ref_2 (`self.Player Ref`))
  (bind _returnvalue (`KismetSystemLibrary.IsValid` (`self.Player Ref`)))
  (if (and (`self.In Range?`) _returnvalue)
    (if (`KismetMathLibrary.InRange_FloatFloat` (`KismetMathLibrary.Dot_VectorVector` (`self.GetActorForwardVector` (`GameplayStatics.GetPlayerCameraManager` 0)) (`SceneComponent.GetForwardVector` (`self.Arrow`))) -1.0 -0.75)
      (`TextBlock.SetText` (`/Game/Master/UI/Weapons_Pickup.PickupText` (`/Game/Master/Blueprints/Player_BP.WeaponPickup_UI` _player_ref)) "Pickup Pistol (E)")
      (set `/Game/Master/Blueprints/Player_BP.Can Pick up Pistol?` true _player_ref)
      (else
        (`TextBlock.SetText` (`/Game/Master/UI/Weapons_Pickup.PickupText` (`/Game/Master/Blueprints/Player_BP.WeaponPickup_UI` _player_ref_2)) "" :!label _label)
        (set `/Game/Master/Blueprints/Player_BP.Can Pick up Pistol?` false _player_ref_2)))
    (elif _returnvalue
      (goto _label))))

(event `self.Trigger.OnComponentBeginOverlap`
  (params (OverlappedComponent :type "PrimitiveComponent Object Reference") (OtherActor :type "Actor Object Reference") (OtherComp :type "PrimitiveComponent Object Reference") (OtherBodyIndex :type Integer) (bFromSweep :type Boolean) (SweepResult :type "HitResult Structure (by ref)"))
  (bind _asplayer_bp (cast `/Game/Master/Blueprints/Player_BP` OtherActor))
  (set `self.Player Ref` _asplayer_bp)
  (set `self.In Range?` true))

(event `self.Trigger.OnComponentEndOverlap`
  (params (OverlappedComponent :type "PrimitiveComponent Object Reference") (OtherActor :type "Actor Object Reference") (OtherComp :type "PrimitiveComponent Object Reference") (OtherBodyIndex :type Integer))
  (cast `/Game/Master/Blueprints/Player_BP` OtherActor)
  (set `self.In Range?` false))

(fn `UserConstructionScript`)