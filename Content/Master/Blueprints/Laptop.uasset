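; A laptop actor that the player can access, with a screen showing security camera feeds.
; On Tick, a distance check, pawn sphere trace and camera-to-arrow dot product detect a nearby player facing the laptop.
; This toggles the player's enter-view flag and an "Access Laptop" prompt, and hands the player a laptop reference.
; ChangeCamera puts the indexed security camera's render material on the Cameras component's widget.
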(event `self.ReceiveBeginPlay`
  (bind _asplayer_bp (cast `/Game/Master/Blueprints/Player_BP` (`GameplayStatics.GetPlayerCharacter` 0)))
  (set `self.Player` _asplayer_bp)
  (bind _returnvalue (`|CreateWidget` "/Game/Master/UI/LaptopEnterWidget.LaptopEnterWidget_C"))
  (bind _output_get (set `self.Laptop UI` _returnvalue))
  (`UserWidget.AddToViewport` _output_get 0))

(event `Change Camera`
  (params (Index :type Integer))
  (`self.Change Render Material` (`/Game/Master/Blueprints/SurveillanceCamera.Render Material` (`|GetArrayItem` (`self.SecurityCameras`) Index))))

(event `self.ReceiveTick`
  (params (DeltaSeconds :type "Float (single-precision)"))
  (bind _returnvalue (`self.K2_GetActorLocation`))
  (bind _player (`self.Player`))
  (if (< (`KismetMathLibrary.Vector_Distance` (`self.K2_GetActorLocation`) (`self.K2_GetActorLocation` (`GameplayStatics.GetPlayerCharacter` 0))) 600.0)
    (bind _outhit (`KismetSystemLibrary.SphereTraceSingleForObjects` _returnvalue _returnvalue 100.0 (`|MakeArray` "ObjectTypeQuery3" :!type "EObjectTypeQuery Enum")))
    (cast `/Game/Master/Blueprints/Player_BP` (`.HitActor` (`GameplayStatics.BreakHitResult` _outhit))
      (:`then`
        (if (`KismetMathLibrary.InRange_FloatFloat` (`KismetMathLibrary.Dot_VectorVector` (`self.GetActorForwardVector` (`GameplayStatics.GetPlayerCameraManager` 0)) (`SceneComponent.GetForwardVector` (`self.Arrow`))) -1.0 -0.5)
          (set `/Game/Master/Blueprints/Player_BP.Can Enter Laptop View?` true _player)
          (set `/Game/Master/Blueprints/Player_BP.Laptop Entering Ref` self _player)
          (`TextBlock.SetText` (`/Game/Master/UI/LaptopEnterWidget.LaptopText` (`self.Laptop UI`)) "Access Laptop")
          (else
            (set `/Game/Master/Blueprints/Player_BP.Can Enter Laptop View?` false _player :!label _label)
            (`TextBlock.SetText` (`/Game/Master/UI/LaptopEnterWidget.LaptopText` (`self.Laptop UI`)) ""))))
      (:`CastFailed`
        (goto _label)))))

(fn `Change Render Material`
  (params (Material :type "MaterialInterface Object Reference"))
  (bind _aslaptop_widget (cast `/Game/Master/UI/LaptopWidget` (`WidgetComponent.GetUserWidgetObject` (`self.Cameras`))))
  (`Image.SetBrushFromMaterial` (`/Game/Master/UI/LaptopWidget.Render` _aslaptop_widget) Material))

(fn `UserConstructionScript`)