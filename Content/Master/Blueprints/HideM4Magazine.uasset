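; Animation notify that shows or hides the magazine on the player's M4 rifle during an animation.
; When it fires, it casts the mesh owner to Player_BP, gets M4_BP from the RifleActor child actor, and sets the Magazine component's hidden-in-game state from its Hide variable.
; The change does not propagate to child components.
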(fn `GetNotifyName`
  (returns (ReturnValue :type String))
  (return ""))

(fn `Received_Notify`
  (params (MeshComp :type "SkeletalMeshComponent Object Reference") (Animation :type "AnimSequenceBase Object Reference"))
  (returns (ReturnValue :type Boolean))
  (bind _asplayer_bp (cast `/Game/Master/Blueprints/Player_BP` (`ActorComponent.GetOwner` MeshComp)))
  (bind _asm4_bp (cast `/Game/Master/Blueprints/M4_BP` (`ChildActorComponent.ChildActor` (`/Game/Master/Blueprints/Player_BP.RifleActor` _asplayer_bp))))
  (`SceneComponent.SetHiddenInGame` (`/Game/Master/Blueprints/M4_BP.Magazine` _asm4_bp) (`self.Hide?`) false)
  (return false))