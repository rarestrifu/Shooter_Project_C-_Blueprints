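; Animation notify that hides or shows the clip bone on the pistol's mesh.
; When it fires, it casts the animated mesh's owner to Pistol_BP and does nothing if that fails.
; A Hide flag selects whether Clip_Bone on PistolMesh is hidden or unhidden, so one notify class covers both directions.
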(fn `GetNotifyName`
  (returns (ReturnValue :type String))
  (return ""))

(fn `Received_Notify`
  (params (MeshComp :type "SkeletalMeshComponent Object Reference") (Animation :type "AnimSequenceBase Object Reference"))
  (returns (ReturnValue :type Boolean))
  (bind _aspistol_bp (cast `/Game/Master/Blueprints/Pistol_BP` (`ActorComponent.GetOwner` MeshComp)))
  (if (`self.Hide?`)
    (bind _pistolmesh (`/Game/Master/Blueprints/Pistol_BP.PistolMesh` _aspistol_bp))
    (`SkinnedMeshComponent.HideBoneByName` _pistolmesh "Clip_Bone" "PBO_None")
    (return false)
    (else
      (`SkinnedMeshComponent.UnHideBoneByName` _pistolmesh "Clip_Bone")
      (return false))))