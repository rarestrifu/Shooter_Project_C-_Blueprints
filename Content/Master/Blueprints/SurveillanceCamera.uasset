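; Security camera that sweeps between two arrow limits, detects the player and can be destroyed.
; Tick runs the timeline sweep and, within range, a forward line trace plus sphere trace that builds TimeSeen.
; At full TimeSeen, Seen turns light and lens red, starts alarm music and tracks the player, resuming patrol via retriggerable delay.
; Explode/Deactivate kills the light, darkens the lens, droops the mesh and stops tick.
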(event `self.ReceiveBeginPlay`
  (bind _asplayer_bp (cast `/Game/Master/Blueprints/Player_BP` (`GameplayStatics.GetPlayerCharacter` 0)))
  (set `self.Player` _asplayer_bp))

(event `Explode/Deactivate`
  (bind _seenmusic (`self.SeenMusic`))
  (bind (_relativerotation_roll _relativerotation_pitch _relativerotation_yaw) (`KismetMathLibrary.BreakRotator` (`SceneComponent.RelativeRotation` (`self.CameraMesh`))))
  (`/Engine/EditorBlueprintResources/StandardMacros.DoOnce` false
    (:`Completed`
      (set `self.Destroyed` true)
      (`LightComponent.SetIntensity` (`self.SpotLight`) 0.0)
      (bind _returnvalue (`PrimitiveComponent.CreateDynamicMaterialInstance` (`self.CameraMesh`) 0 "/Game/SplinterCellMain/Blueprints_Main/Security_Cameras/Materials/M_Security_Camera_Master.M_Security_Camera_Master" "None"))
      (`MaterialInstanceDynamic.SetVectorParameterValue` _returnvalue "Lens color 1" (struct :`A` 1.0))
      (`KismetSystemLibrary.Delay` 0.05)
      (`GameplayStatics.PlaySoundAtLocation` "/Game/Master/Audio/Camera_Sounds/CameraBreaking.CameraBreaking" (`self.K2_GetActorLocation`) (struct) 2.0 1.0 0.0 "/Game/Master/Audio/Lights_Sounds/Lights_Attn.Lights_Attn" null null)
      (bind (_direction _newtrack_0) (`Timeline|Deactivate` :!via `PlayFromStart`)
        (:`Update`
          (`SceneComponent.K2_SetRelativeRotation` (`self.CameraMesh`) (`KismetMathLibrary.MakeRotator` _relativerotation_roll (`KismetMathLibrary.Lerp` _relativerotation_pitch -70.0 _newtrack_0) _relativerotation_yaw) false false)
          (`/Engine/EditorBlueprintResources/StandardMacros.IsValid` _seenmusic
            (:`Is Valid`
              (`ActorComponent.K2_DestroyComponent` _seenmusic))
            (:`Is Not Valid`
              _))
          (`self.SetActorTickEnabled` false))))))

(event `Call AI`)

(event `self.ReceiveTick`
  (params (DeltaSeconds :type "Float (single-precision)"))
  (bind _cameramesh (`self.CameraMesh`))
  (bind _player (`self.Player`))
  (bind _seenmusic (`self.SeenMusic`))
  (bind _meshfwdvector (`self.MeshFwdVector`))
  (bind _returnvalue (`SceneComponent.K2_GetComponentLocation` _meshfwdvector))
  (bind (_returnvalue_roll _returnvalue_pitch) (`KismetMathLibrary.BreakRotator` (`SceneComponent.K2_GetComponentRotation` (`self.CameraMesh`))))
  (bind (_returnvalue_roll_2 _returnvalue_pitch_2) (`KismetMathLibrary.BreakRotator` (`SceneComponent.K2_GetComponentRotation` (`self.CameraMesh`))))
  (bind (_returnvalue_roll_3 _returnvalue_pitch_3) (`KismetMathLibrary.BreakRotator` (`SceneComponent.K2_GetComponentRotation` (`self.CameraMesh`))))
  (bind (_relativerotation_roll _relativerotation_pitch _relativerotation_yaw) (`KismetMathLibrary.BreakRotator` (`SceneComponent.RelativeRotation` (`self.CameraMesh`))))
  (bind (_relativerotation_roll_2 _relativerotation_pitch_2) (`KismetMathLibrary.BreakRotator` (`SceneComponent.RelativeRotation` (`self.ArrowNone`))))
  (bind (_relativerotation_roll_3 _relativerotation_pitch_3 _relativerotation_yaw_2) (`KismetMathLibrary.BreakRotator` (`SceneComponent.RelativeRotation` (`self.CameraMesh`))))
  (bind (_relativerotation_roll_4 _relativerotation_pitch_4 _relativerotation_yaw_3) (`KismetMathLibrary.BreakRotator` (`SceneComponent.RelativeRotation` (`self.CameraMesh`))))
  (bind (_relativerotation_roll_5 _relativerotation_pitch_5 _relativerotation_yaw_4) (`KismetMathLibrary.BreakRotator` (`SceneComponent.RelativeRotation` (`self.CameraMesh`))))
  (bind (_relativerotation_roll_6 _relativerotation_pitch_6 _relativerotation_yaw_5) (`KismetMathLibrary.BreakRotator` (`SceneComponent.RelativeRotation` (`self.CameraMesh`))))
  (bind (_relativerotation_roll_7 _relativerotation_pitch_7 _relativerotation_yaw_6) (`KismetMathLibrary.BreakRotator` (`SceneComponent.RelativeRotation` (`self.ArrowLeft`))))
  (bind (_relativerotation_roll_8 _relativerotation_pitch_8 _relativerotation_yaw_7) (`KismetMathLibrary.BreakRotator` (`SceneComponent.RelativeRotation` (`self.ArrowRight`))))
  (bind _returnvalue_2 (`KismetMathLibrary.FindLookAtRotation` (`SceneComponent.K2_GetComponentLocation` (`self.CameraMesh`)) (`self.K2_GetActorLocation` (`GameplayStatics.GetPlayerCharacter` 0))))
  (bind _returnvalue_3 (+ (`SceneComponent.K2_GetComponentLocation` _cameramesh) (0.0 0.0 15.0)))
  (if (not (`self.Destroyed`))
    (`|ExecutionSequence`
      (:`then_0`
        (switch `/Game/Master/Enums/CameraRot` (`self.CameraRot`)
          (:`NewEnumerator0`
            (`|ExecutionSequence`
              (:`then_0`
                (`/Engine/EditorBlueprintResources/StandardMacros.DoOnce` false :!label _label
                  (:`Completed`
                    (bind (_direction _newtrack_0) (`Timeline|Timeline_0` :!via `PlayFromStart` :!label _label_2)
                      (:`Update`
                        (bind (_returnvalue_roll_4 _returnvalue_pitch_4 _returnvalue_yaw) (`KismetMathLibrary.BreakRotator` (`KismetMathLibrary.RLerp` (`SceneComponent.RelativeRotation` (`self.ArrowLeft`)) (`SceneComponent.RelativeRotation` (`self.ArrowRight`)) _newtrack_0)))
                        (`SceneComponent.K2_SetRelativeRotation` (`self.CameraMesh`) (`KismetMathLibrary.MakeRotator` _returnvalue_roll_3 _returnvalue_pitch_3 _returnvalue_yaw) false false))
                      (:`Finished`
                        (`KismetSystemLibrary.Delay` 2.0)
                        (set `self.CameraRot` "NewEnumerator1"))))))
              (:`then_1`
                (goto _label_3 :!via `Reset`))
              (:`then_2`
                (goto _label_5 :!via `Reset`))))
          (:`NewEnumerator1`
            (`|ExecutionSequence`
              (:`then_0`
                (`/Engine/EditorBlueprintResources/StandardMacros.DoOnce` false :!label _label_3
                  (:`Completed`
                    (bind (_direction_2 _newtrack_0_2) (`Timeline|Timeline_1` :!via `PlayFromStart` :!label _label_4)
                      (:`Update`
                        (bind (_returnvalue_roll_5 _returnvalue_pitch_5 _returnvalue_yaw_2) (`KismetMathLibrary.BreakRotator` (`KismetMathLibrary.RLerp` (`SceneComponent.RelativeRotation` (`self.ArrowRight`)) (`SceneComponent.RelativeRotation` (`self.ArrowLeft`)) _newtrack_0_2)))
                        (`SceneComponent.K2_SetRelativeRotation` (`self.CameraMesh`) (`KismetMathLibrary.MakeRotator` _returnvalue_roll_2 _returnvalue_pitch_2 _returnvalue_yaw_2) false false))
                      (:`Finished`
                        (`KismetSystemLibrary.Delay` 2.0)
                        (set `self.CameraRot` "NewEnumerator0"))))))
              (:`then_1`
                (goto _label :!via `Reset`))
              (:`then_2`
                (goto _label_5 :!via `Reset`))))
          (:`NewEnumerator2`
            (`/Engine/EditorBlueprintResources/StandardMacros.DoOnce` false :!label _label_5
              (:`Completed`
                (bind (_direction_3 _newtrack_0_3) (`Timeline|Set Rot 1` :!via `PlayFromStart` :!label _label_6)
                  (:`Update`
                    (bind (_returnvalue_roll_6 _returnvalue_pitch_6 _returnvalue_yaw_3) (`KismetMathLibrary.BreakRotator` (`KismetMathLibrary.RLerp` (`self.Last None Rotation`) (`SceneComponent.RelativeRotation` (`self.ArrowLeft`)) _newtrack_0_3)))
                    (`SceneComponent.K2_SetRelativeRotation` (`self.CameraMesh`) (`KismetMathLibrary.MakeRotator` _returnvalue_roll _returnvalue_pitch _returnvalue_yaw_3) false false))
                  (:`Finished`
                    (`KismetSystemLibrary.Delay` 2.0)
                    (set `self.CameraRot` "NewEnumerator0"))))))
          (:`NewEnumerator3`
            (`|ExecutionSequence`
              (:`then_0`
                (goto _label_6 :!via `Stop`))
              (:`then_1`
                (goto _label_2 :!via `Stop`))
              (:`then_2`
                (goto _label_4 :!via `Stop`))
              (:`then_3`
                (goto _label_3 :!via `Reset`))
              (:`then_4`
                (goto _label :!via `Reset`))
              (:`then_5`
                (goto _label_5 :!via `Reset`))))))
      (:`then_1`
        (if (== (`self.TimeSeen`) 1.0)
          (set `self.CameraRot` "NewEnumerator3")
          (`|ExecutionSequence`
            (:`then_0`
              (`/Engine/EditorBlueprintResources/StandardMacros.DoOnce` false :!label _label_7
                (:`Completed`
                  (set `self.Seeing Player` true)
                  (if (not (`/Game/Master/Blueprints/Player_BP.Alarm Playing` _player))
                    (bind _returnvalue_4 (`GameplayStatics.SpawnSound2D` "/Game/Master/Audio/Music/Blueprint_Music_Alarm01.Blueprint_Music_Alarm01" 1.0 1.0 0.0 null))
                    (set `self.SeenMusic` _returnvalue_4)
                    (set `/Game/Master/Blueprints/Player_BP.Alarm Playing` true _player))
                  (`LightComponent.SetLightColor` (`self.SpotLight`) (struct :`R` 0.286458 :`G` 0.002763 :`A` 1.0) true)
                  (bind _returnvalue_5 (`PrimitiveComponent.CreateDynamicMaterialInstance` (`self.CameraMesh`) 0 "/Game/SplinterCellMain/Blueprints_Main/Security_Cameras/Materials/M_Security_Camera_Master.M_Security_Camera_Master" "None"))
                  (`MaterialInstanceDynamic.SetVectorParameterValue` _returnvalue_5 "Lens color 1" (struct :`R` 0.432292 :`B` 0.016117 :`A` 1.0)))))
            (:`then_1`
              (if (`self.Rotated?`)
                (bind _outhit (`KismetSystemLibrary.LineTraceSingle` :`Start` _returnvalue_3 :`End` (select `bool` (`self.Seeing Player`) :`false` (+ _returnvalue_3 (* (`SceneComponent.GetForwardVector` _cameramesh) 1200.0)) :`true` (`self.K2_GetActorLocation` (`GameplayStatics.GetPlayerCharacter` 0))) :`TraceChannel` "TraceTypeQuery1" :`DrawDebugType` (`self.Debug Camera`)))
                (bind (_bblockinghit _binitialoverlap _time _distance _location _impactpoint _normal _impactnormal _physmat _hitactor _hitcomponent) (`GameplayStatics.BreakHitResult` _outhit))
                (if _bblockinghit
                  (if (== _hitactor (`GameplayStatics.GetPlayerCharacter` 0))
                    (if (`KismetMathLibrary.InRange_FloatFloat` _relativerotation_yaw_3 _relativerotation_yaw_6 _relativerotation_yaw_7)
                      (set `self.Can Come Back?` false :!label _label_8)
                      (set `self.Seeing Player` true)
                      (`SceneComponent.K2_SetWorldRotation` (`self.CameraMesh`) _returnvalue_2 false false)
                      (set `self.Last Rot Yaw` (.yaw _returnvalue_2))
                      (set `self.CameraRot` "NewEnumerator3")
                      (`KismetSystemLibrary.RetriggerableDelay` 5.0 :!label _label_9)
                      (if (`KismetMathLibrary.InRange_FloatFloat` _relativerotation_yaw_4 79.0 81.0 false false)
                        (set `self.CameraRot` "NewEnumerator1")
                        (set `self.Last Right Rotation` (`SceneComponent.RelativeRotation` (`self.CameraMesh`)))
                        (set `self.TimeSeen` 0.0)
                        (`ActorComponent.K2_DestroyComponent` (`self.SeenMusic`))
                        (`|ExecutionSequence`
                          (:`then_0`
                            (goto _label_10 :!via `Reset`))
                          (:`then_1`
                            (goto _label_7 :!via `Reset`)))
                        (elif (`KismetMathLibrary.InRange_FloatFloat` _relativerotation_yaw_2 -81.0 -79.0)
                          (set `self.CameraRot` "NewEnumerator0")
                          (set `self.Last Left Rotation` (`SceneComponent.RelativeRotation` (`self.CameraMesh`)))
                          (set `self.TimeSeen` 0.0)
                          (`ActorComponent.K2_DestroyComponent` (`self.SeenMusic`))
                          (`|ExecutionSequence`
                            (:`then_0`
                              (goto _label_7 :!via `Reset`))
                            (:`then_1`
                              (goto _label_10 :!via `Reset`)))
                          (else
                            (set `self.CameraRot` "NewEnumerator2")
                            (set `self.Last None Rotation` (`KismetMathLibrary.MakeRotator` _relativerotation_roll_2 _relativerotation_pitch_2 _relativerotation_yaw_5))
                            (set `self.TimeSeen` 0.0)
                            (`/Engine/EditorBlueprintResources/StandardMacros.IsValid` _seenmusic
                              (:`Is Valid`
                                (`ActorComponent.K2_DestroyComponent` _seenmusic))
                              (:`Is Not Valid`
                                _))
                            (`|ExecutionSequence`
                              (:`then_0`
                                (goto _label_7 :!via `Reset`))
                              (:`then_1`
                                (goto _label_10 :!via `Reset`))))))
                      (elif (`self.Seeing Player`)
                        (set `self.Seeing Player` false)
                        (set `self.Last Player Position Seen` _impactpoint)
                        (`KismetSystemLibrary.Delay` 0.1)
                        (set `self.Can Come Back?` true)
                        (goto _label_9)
                        (elif (and (or (`self.RightTrace` _relativerotation_yaw _hitcomponent) (`self.LeftTrace` _relativerotation_yaw _hitcomponent)) (`self.Can Come Back?`))
                          (goto _label_8))))))))
            (:`then_2`
              (`/Engine/EditorBlueprintResources/StandardMacros.DoOnce` false :!label _label_10
                (:`Completed`
                  (bind (_direction_4 _lerp) (`Timeline|Timeline_2` :!via `PlayFromStart`)
                    (:`Update`
                      (`SceneComponent.K2_SetWorldRotation` (`self.CameraMesh`) (`KismetMathLibrary.RLerp` (`SceneComponent.K2_GetComponentRotation` (`self.CameraMesh`)) (`KismetMathLibrary.FindLookAtRotation` (`SceneComponent.K2_GetComponentLocation` (`self.CameraMesh`)) (`self.K2_GetActorLocation` (`GameplayStatics.GetPlayerCharacter` 0))) _lerp) false false))
                    (:`Finished`
                      (set `self.Rotated?` true)))))))
          (elif (< (`KismetMathLibrary.Vector_Distance` (`self.K2_GetActorLocation` self) (`self.K2_GetActorLocation` (`GameplayStatics.GetPlayerCharacter` 0))) 2000.0)
            (bind _outhit_2 (`KismetSystemLibrary.LineTraceSingle` _returnvalue (+ _returnvalue (* (`SceneComponent.GetForwardVector` _meshfwdvector) 1000.0)) "TraceTypeQuery1" false (`|MakeArray` (`GameplayStatics.GetPlayerCharacter` 0) :!type "Actor Object Reference") (`self.Debug Camera`)))
            (bind _output_get (set `self.StartTrace` (`.Location` (`GameplayStatics.BreakHitResult` _outhit_2))))
            (bind _outhit_3 (`KismetSystemLibrary.SphereTraceSingleForObjects` :`Start` _output_get :`End` _output_get :`Radius` 250.0 :`ObjectTypes` (`|MakeArray` "ObjectTypeQuery3" :!type "EObjectTypeQuery Enum") :`DrawDebugType` (`self.Debug Camera`)))
            (bind (_bblockinghit_2 _binitialoverlap_2 _time_2 _distance_2 _location_2 _impactpoint_2 _normal_2 _impactnormal_2 _physmat_2 _hitactor_2) (`GameplayStatics.BreakHitResult` _outhit_3))
            (if _bblockinghit_2
              (if (== _hitactor_2 (`GameplayStatics.GetPlayerCharacter` 0))
                (`/Engine/EditorBlueprintResources/StandardMacros.DoOnce` false :!label _label_11
                  (:`Completed`
                    (bind (_direction_5 _timeseen) (`Timeline|Set TimeSeen` :!via `PlayFromStart` :!label _label_12)
                      (:`Update`
                        (set `self.TimeSeen` _timeseen)))))
                (else
                  (set `self.TimeSeen` 0.0 :!label _label_13)
                  (`|ExecutionSequence`
                    (:`then_0`
                      (goto _label_12 :!via `Stop`))
                    (:`then_1`
                      (goto _label_12 :!via `Reverse`))
                    (:`then_2`
                      (goto _label_11 :!via `Reset`)))))
              (else
                (goto _label_13))))))
      (:`then_2`
        (switch `/Game/Master/Enums/CameraRot` (`self.CameraRot`)
          (:`NewEnumerator0`
            _)
          (:`NewEnumerator1`
            _)
          (:`NewEnumerator2`
            _)
          (:`NewEnumerator3`
            (goto _label_14 :!via `Reset`)))
        (`LightComponent.SetLightColor` (`self.SpotLight`) (struct :`R` 0.039546 :`G` 1.0 :`A` 1.0) true)
        (bind _returnvalue_6 (`PrimitiveComponent.CreateDynamicMaterialInstance` (`self.CameraMesh`) 0 "/Game/SplinterCellMain/Blueprints_Main/Security_Cameras/Materials/M_Security_Camera_Master.M_Security_Camera_Master" "None"))
        (`MaterialInstanceDynamic.SetVectorParameterValue` _returnvalue_6 "Lens color 1" (struct :`R` 0.039546 :`G` 1.0 :`A` 1.0))
        (`/Engine/EditorBlueprintResources/StandardMacros.DoOnce` false :!label _label_14
          (:`Completed`
            (`GameplayStatics.PlaySoundAtLocation` "/Game/Master/Audio/Electrical_Sounds/Blueprints_ComputerStatic01.Blueprints_ComputerStatic01" (`self.K2_GetActorLocation`) (struct) 1.0 0.5 0.0 "/Game/Master/Audio/Male_Voice/CameraAtt.CameraAtt" null null)))))
    (else
      (`|ExecutionSequence`
        (:`then_0`
          (goto _label_6 :!via `Stop`))
        (:`then_1`
          (goto _label_2 :!via `Stop`))
        (:`then_2`
          (goto _label_4 :!via `Stop`))
        (:`then_3`
          (goto _label_5 :!via `Reset`))))))

(fn `LeftTrace`
  (params (`Yaw Range` :type "Float (double-precision)") (`Hit Left Trace` :type "Object Object Reference"))
  (returns (ReturnValue :type Boolean))
  (bind (_relativerotation_roll _relativerotation_pitch _relativerotation_yaw) (`KismetMathLibrary.BreakRotator` (`SceneComponent.RelativeRotation` (`self.ArrowRight`))))
  (return (and (`KismetMathLibrary.InRange_FloatFloat` `Yaw Range` (- _relativerotation_yaw -0.01) (- _relativerotation_yaw -1.5)) (== (`/Game/Master/Blueprints/Player_BP.LeftTracer` (`self.Player`)) `Hit Left Trace`))))

(fn `RightTrace`
  (params (`Yaw Range` :type "Float (double-precision)") (`Hit Right Trace` :type "Object Object Reference"))
  (returns (ReturnValue :type Boolean))
  (bind (_relativerotation_roll _relativerotation_pitch _relativerotation_yaw) (`KismetMathLibrary.BreakRotator` (`SceneComponent.RelativeRotation` (`self.ArrowLeft`))))
  (return (and (`KismetMathLibrary.InRange_FloatFloat` `Yaw Range` (- _relativerotation_yaw 1.5) (- _relativerotation_yaw 0.01)) (== (`/Game/Master/Blueprints/Player_BP.RightTracer` (`self.Player`)) `Hit Right Trace`))))

(fn `UserConstructionScript`)