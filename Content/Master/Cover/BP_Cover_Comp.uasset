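; BP_Cover_Comp is an actor component, named for cover, that sets itself up only on player 0's Player_BP pawn.
; On BeginPlay it caches that player and its default capsule radius, or disables its tick on any other owner.
; A CharacterCapsule helper is meant to select player location, direction, rotation or capsule data by type.
; No tick or cover logic appears here.
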(event `self.ReceiveBeginPlay`
  (bind _returnvalue (`self.GetOwner`))
  (bind _value_x (`KismetMathLibrary.BreakVector` (`self.CharacterCapsule` "NewEnumerator5")))
  (if (== _returnvalue (`GameplayStatics.GetPlayerPawn` 0))
    (bind _ascharacter (cast `Character` _returnvalue)
      (:`then`
        (bind _asplayer_bp (cast `/Game/Master/Blueprints/Player_BP` _ascharacter)
          (:`then`
            (set `self.Player` _asplayer_bp)
            (set `self.Default Capsule Size` (`KismetMathLibrary.MakeVector2D` _value_x)))
          (:`CastFailed`
            (`self.SetComponentTickEnabled` false))))
      (:`CastFailed`
        (`self.SetComponentTickEnabled` false)))
    (else
      (`self.SetComponentTickEnabled` false))))