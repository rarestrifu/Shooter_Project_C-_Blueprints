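; Trigger volume actor that shows a one-time tutorial popup when the ALS main character overlaps it.
; On overlap it creates a Tutorial_Popup widget filled with its header, title, body text and image.
; It disables player input, switches to UI-only mode with the mouse cursor visible, plays a 2D sound and destroys itself.
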(event `self.ReceiveActorBeginOverlap`
  (params (OtherActor :type "Actor Object Reference"))
  (bind _returnvalue (`GameplayStatics.GetPlayerController` 0))
  (bind _asals_main_character (cast `/Game/SplinterCellMain/Blueprints_Main/ALS_MainCharacter` OtherActor))
  (`/Engine/EditorBlueprintResources/StandardMacros.IsValid` _asals_main_character
    (:`Is Valid`
      (`/Engine/EditorBlueprintResources/StandardMacros.DoOnce` false
        (:`Completed`
          (bind _returnvalue_2 (`|CreateWidget` "/Game/SplinterCellMain/Blueprints_Main/TutorialUI/Tutorial_Popup.Tutorial_Popup_C" _returnvalue (`self.Image`)))
          (`self.DisableInput` (`GameplayStatics.GetPlayerCharacter` 0) _returnvalue)
          (`/Game/SplinterCellMain/Blueprints_Main/TutorialUI/Tutorial_Popup.SetDisplay Header Text` _returnvalue_2 (`self.Header Text`))
          (`/Game/SplinterCellMain/Blueprints_Main/TutorialUI/Tutorial_Popup.Set Display Title Text` _returnvalue_2 (`self.Title Text`))
          (`/Game/SplinterCellMain/Blueprints_Main/TutorialUI/Tutorial_Popup.Set Display Body Text` _returnvalue_2 (`self.Body Text`))
          (`UserWidget.AddToViewport` _returnvalue_2 5)
          (`self.K2_DestroyActor`)
          (`WidgetBlueprintLibrary.SetInputMode_UIOnlyEx` _returnvalue _returnvalue_2)
          (set `PlayerController.bShowMouseCursor` true _returnvalue)
          (`GameplayStatics.SpawnSound2D` "/Game/SplinterCellMain/Audio/UI_Sounds/0065.0065" 0.35 1.0 0.0 null))))))

(fn `UserConstructionScript`)