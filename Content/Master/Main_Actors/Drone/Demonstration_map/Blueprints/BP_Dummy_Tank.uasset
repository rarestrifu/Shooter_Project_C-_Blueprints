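; Damageable dummy tank target with preset or randomized turret and gun angles and an optional overhead health bar.
; AnyDamage subtracts health and at zero spawns a destroyed-wreck actor, then removes the tank.
; Instead of Tick, a 0.025-second looping timer turns the widget toward the player, scales and hides it by distance, and colors it red at low health.
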(event `self.ReceiveHit`
  (params (MyComp :type "PrimitiveComponent Object Reference") (Other :type "Actor Object Reference") (OtherComp :type "PrimitiveComponent Object Reference") (bSelfMoved :type Boolean) (HitLocation :type "Vector Structure") (HitNormal :type "Vector Structure") (NormalImpulse :type "Vector Structure") (Hit :type "HitResult Structure (by ref)"))
  ;[0 0 0] For testing only
)

(event `self.ReceiveTick`
  (params (DeltaSeconds :type "Float (single-precision)"))
  ;[1 0 0] No tick functions :) ( Tick is disabled in blueprint if needed enable it first )
)

(event `self.ReceiveBeginPlay`
  (`|ExecutionSequence`
    (:`then_0`
      ;[1 1 1] Mpdes controling random turret and gun position
      (if (`self.bRandom_Turret_Rotation`)
        (set `self.BP_Turret_rotation` (`KismetMathLibrary.RandomFloatInRange` -180.0 180.0)))
      ;[1 1 1] Nodes controling random turret and gun position
      (if (`self.bRandom_Gun_Rotation`)
        (bind _output_get (set `self.Gun_rotation` (`KismetMathLibrary.RandomFloatInRange` -10.0 25.0)))
        (set `self.BP_Gun_rotation` _output_get)))
    (:`then_1`
      (`self.CE 3p_health_widget_rotate`))))

(event `self.ReceiveAnyDamage`
  (params (Damage :type "Float (single-precision)") (DamageType :type "DamageType Object Reference") (InstigatedBy :type "Controller Object Reference") (DamageCauser :type "Actor Object Reference"))
  (bind _dummy_tank (`self.Dummy_tank`))
  ;[1 0.8824 0] Nodes controling damage system ( how many health points is subtracted when vehicle is hit with damage )
  (if (`self.Can_be_Damaged_?`)
    (set `self.Damage` Damage)
    (set `self.Taking_damage_?` true)
    (`|ExecutionSequence`
      (:`then_0`
        (`KismetSystemLibrary.RetriggerableDelay` (`self.Health_refresh_cooldown`))
        (set `self.Taking_damage_?` false))
      (:`then_1`
        (set `self.Health_Dummy_Tank` (- (`self.Health_Dummy_Tank`) (`self.Damage`)))
        (if (<= (`self.Health_Dummy_Tank`) 0.0)
          (`/Engine/EditorBlueprintResources/StandardMacros.DoOnce` false
            (:`Completed`
              (bind _returnvalue (`|SpawnActorFromClass` "/Game/SplinterCellMain/Blueprints_Main/Drone/Demonstration_map/Blueprints/BP_Dummy_Tank_Destroyed.BP_Dummy_Tank_Destroyed_C" (`self.GetTransform`) "Undefined" "OverrideRootScale" null null))
              (set `/Game/SplinterCellMain/Blueprints_Main/Drone/Demonstration_map/Blueprints/BP_Dummy_Tank_Destroyed.Wreck_destroyed_?` true _returnvalue)
              (`/Game/SplinterCellMain/Blueprints_Main/Drone/Demonstration_map/Blueprints/BP_Dummy_Tank_Destroyed.CE_Destroy_Wreck` _returnvalue)
              (`PrimitiveComponent.SetCollisionEnabled` _dummy_tank "NoCollision")
              (`SceneComponent.SetVisibility` _dummy_tank false false)
              (`KismetSystemLibrary.Delay` 0.1)
              (`self.K2_DestroyActor`))))))))

(event `CE 3p_health_widget_rotate`
  (bind _scene (`self.Scene`))
  (bind _health_dummy_tank (`self.Health_Dummy_Tank`))
  (bind _distance_needed_t_hide_3p_widget (`self.Distance_Needed_T_Hide_3p_Widget`))
  (bind _returnvalue (`SceneComponent.K2_GetComponentLocation` _scene))
  (bind _returnvalue_2 (`self.K2_GetActorLocation` (`GameplayStatics.GetPlayerPawn` 0)))
  (bind _yaw (.yaw (`KismetMathLibrary.FindLookAtRotation` _returnvalue _returnvalue_2)))
  (bind _returnvalue_3 (`KismetMathLibrary.Abs` (/ (`KismetMathLibrary.GetPointDistanceToLine` _returnvalue_2 _returnvalue (`KismetMathLibrary.Conv_DoubleToVector` _yaw)) 100.0)))
  ;[0 0.2431 0.2471] Nodes controling T_A_Bar_3P widget and orientate it to player
  (if (not (`self.Hide_3P_Health_Widget`))
    (`/Engine/EditorBlueprintResources/StandardMacros.IsValid` (`GameplayStatics.GetPlayerPawn` 0)
      (:`Is Valid`
        (`KismetSystemLibrary.K2_SetTimerDelegate` (delegate `CE 3p_health_widget_rotate`) 0.025 true)
        (`/Engine/EditorBlueprintResources/StandardMacros.CompareFloat` _returnvalue_3 _distance_needed_t_hide_3p_widget
          (:`>`
            (`SceneComponent.SetHiddenInGame` _scene true true))
          (:`<`
            (`SceneComponent.SetHiddenInGame` _scene false true)))
        (`SceneComponent.SetWorldScale3D` _scene (`KismetMathLibrary.Conv_DoubleToVector` (`KismetMathLibrary.FClamp` (`KismetMathLibrary.NormalizeToRange` _returnvalue_3 0.0 _distance_needed_t_hide_3p_widget) 0.1 0.5)))
        (`SceneComponent.K2_SetWorldRotation` _scene (`KismetMathLibrary.MakeRotator` 0.0 0.0 _yaw) false false)
        (bind _asumg_dummy_tank_3p_health_widget (cast `/Game/SplinterCellMain/Blueprints_Main/Drone/Demonstration_map/Ui/UMG_Dummy_Tank_3P_health_Widget` (`WidgetComponent.GetUserWidgetObject` (`self.Widget_3P_Health`))))
        (bind _healthbar (`/Game/SplinterCellMain/Blueprints_Main/Drone/Demonstration_map/Ui/UMG_Dummy_Tank_3P_health_Widget.HealthBar` _asumg_dummy_tank_3p_health_widget))
        (`ProgressBar.SetPercent` _healthbar (/ _health_dummy_tank 100.0))
        (`/Engine/EditorBlueprintResources/StandardMacros.CompareFloat` _health_dummy_tank 30.0
          (:`>`
            (bind _output_get (set `/Game/SplinterCellMain/Blueprints_Main/Drone/Demonstration_map/Ui/UMG_Dummy_Tank_3P_health_Widget.HealthBar` _healthbar _asumg_dummy_tank_3p_health_widget :!label _label))
            (`ProgressBar.SetFillColorAndOpacity` _output_get (struct :`G` 1.0 :`A` 1.0)))
          (:`==`
            (goto _label))
          (:`<`
            (bind _output_get_2 (set `/Game/SplinterCellMain/Blueprints_Main/Drone/Demonstration_map/Ui/UMG_Dummy_Tank_3P_health_Widget.HealthBar` _healthbar _asumg_dummy_tank_3p_health_widget))
            (`ProgressBar.SetFillColorAndOpacity` _output_get_2 (struct :`R` 1.0 :`A` 1.0))))))))

(fn `UserConstructionScript`
  (bind _widget_3p_health (`self.Widget_3P_Health`))
  (`|ExecutionSequence`
    (:`then_0`
      (set `self.BP_Turret_rotation` (`self.Turret_rotation`))
      (set `self.BP_Gun_rotation` (`self.Gun_rotation`))
      ;[1 1 1] Hide_3P_Health_widget
      (if (`self.Hide_3P_Health_Widget`)
        (`SceneComponent.SetVisibility` _widget_3p_health false false)
        (else
          (`SceneComponent.SetVisibility` _widget_3p_health true false))))))