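; BP_Dummy_Drone_Spline moves a referenced dummy drone actor along a spline path as a moving target, apparently for the drone demonstration map.
; On Tick, when MovingTarget is set and Speed equals 1, it restarts a timeline.
; Each update scales the timeline value by HowFastTargetIsMoving to position and orient the drone by spline distance.
; The clamped magnitude of that value becomes Speed, so reaching 1 allows the next restart.
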(event `self.ReceiveTick`
  (params (DeltaSeconds :type "Float (single-precision)"))
  (bind _path (`self.Path`))
  (bind _actor_bp_dummy_drone (`self.Actor_BP_Dummy_drone`))
  ;[1 0 0] How fast is target moving
  (`/Engine/EditorBlueprintResources/StandardMacros.IsValid` (`self.Actor_BP_Dummy_drone`)
    (:`Is Valid`
      (if (and (`self.Moving target ?`) (== (`self.Speed`) 1.0))
        (bind (_direction _target_moving) (`Timeline|DRone_speed_timeline` :!via `PlayFromStart`)
          (:`Update`
            (bind _returnvalue (* _target_moving (`self.How fast target is moving ?`)))
            (set `self.Speed` (`KismetMathLibrary.FClamp` (`KismetMathLibrary.Abs` _returnvalue)))
            (`/Engine/EditorBlueprintResources/StandardMacros.IsValid` _actor_bp_dummy_drone
              (:`Is Valid`
                (bind _returnvalue_2 (* _returnvalue (`SplineComponent.GetSplineLength` _path)))
                (`self.K2_SetActorTransform` _actor_bp_dummy_drone (`KismetMathLibrary.MakeTransform` (`SplineComponent.GetLocationAtDistanceAlongSpline` _path _returnvalue_2 "World") (`SplineComponent.GetRotationAtDistanceAlongSpline` _path _returnvalue_2 "World")) false false)))))))))

(fn `UserConstructionScript`)