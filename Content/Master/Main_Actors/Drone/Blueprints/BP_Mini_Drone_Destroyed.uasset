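; Wreck actor for a destroyed mini drone that plays a one-time physics breakup with explosion effects, then removes itself.
; If WreckDestroyed is set on BeginPlay or CE_Destroy_Wreck, it wakes the body's physics and applies randomized radial force, impulse and motor-bone spin.
; It activates explosion particle and sound components, then after a delay spawns a small final explosion and destroys the actor.
; Tick is unused.
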(event `self.ReceiveTick`
  (params (DeltaSeconds :type "Float (single-precision)"))
  ;[1 0 0] No tick functions :) ( Tick is disabled in blueprint if needed enable it first )
)

(event `CE_Destroy_Wreck`
  (bind _body (`self.Body`))
  (bind _body_2 (`self.Body`))
  (bind _body_3 (`self.Body`))
  (bind _returnvalue (`SceneComponent.K2_GetComponentRotation` _body))
  ;[1 1 1] Wake rigid bodes and add some force to them
  (if (`self.Wreck_destroyed_?`) :!label _label
    (`/Engine/EditorBlueprintResources/StandardMacros.DoOnce` false
      (:`Completed`
        (`SkeletalMeshComponent.SetAllBodiesSimulatePhysics` _body_2 true)
        (`PrimitiveComponent.WakeAllRigidBodies` _body_2)
        (`PrimitiveComponent.AddRadialForce` _body (`self.K2_GetActorLocation`) 250.0 (`KismetMathLibrary.RandomFloatInRange` 30000.0 15000.0) "RIF_Constant" true)
        (`PrimitiveComponent.AddImpulse` _body_3 (* (`KismetMathLibrary.GetRightVector` _returnvalue) (`KismetMathLibrary.RandomFloatInRange` -450.0 -800.0)) "Root" true)
        (`PrimitiveComponent.AddAngularImpulseInRadians` _body_3 (* (`KismetMathLibrary.GetUpVector` _returnvalue) (`KismetMathLibrary.RandomFloatInRange` -15.0 15.0)) "Motor_RR" true)
        ;[1 1 1] Play primary PS effect, and play fire and explosion sound
        (`ActorComponent.SetActive` (`self.PS_Explosion`) true false)
        (`ActorComponent.SetActive` (`self.SC_Explosion`) true false)
        ;[1 1 1] Hide destroyed mesh, and play final PS effect
        (`KismetSystemLibrary.Delay` 5.0) ; Change this to control how long destroyed mesh will be visible in game ( Be aware that particle life is allso calculated )
        (`GameplayStatics.SpawnEmitterAtLocation` "/Game/SplinterCellMain/Blueprints_Main/Drone/Particles/PS_Generic_4x4_explosion_Small.PS_Generic_4x4_explosion_Small" (`SceneComponent.K2_GetComponentLocation` (`self.Body`)) (struct) (0.5 0.5 0.5))
        (`self.K2_DestroyActor`)))))

(event `self.ReceiveBeginPlay`
  ;[1 1 1] Wake rigid bodes and add some force to them
  (goto _label))

(fn `UserConstructionScript`)