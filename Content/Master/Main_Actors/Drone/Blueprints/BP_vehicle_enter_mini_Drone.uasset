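; Blueprint that lets the player enter and take control of a mini drone vehicle.
; Display_text shows the enter-prompt widget when the player is near an unused drone and removes it when not near.
; Enter_vehicle checks the use and proximity flags, then marks the drone in use, stores the player's character on it, possesses it and hides its third-person health widget.
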(event `Display_text`
  ;[1 1 1] Display enter text
  (if (`self.bNear_vehicle_?`)
    (if (not (`/Game/SplinterCellMain/Blueprints_Main/Drone/Blueprints/BP_Mini_Drone.Use_Mini_drone` (`self.Vehicle_P`)))
      (bind _returnvalue (`|CreateWidget` "/Game/SplinterCellMain/Blueprints_Main/Drone/UI/UMG_Mini_Drone_enter.UMG_Mini_Drone_enter_C" (`GameplayStatics.GetPlayerController` 0)))
      (`UserWidget.AddToViewport` _returnvalue 0))
    (else
      (`Widget.RemoveFromParent` _returnvalue))))

(event `Enter_vehicle`
  (bind _vehicle_p (`self.Vehicle_P`))
  ;[1 1 1] Posses vehicle
  (if (and (`self.bUse_vehicle`) (`self.bNear_vehicle_?`))
    (set `/Game/SplinterCellMain/Blueprints_Main/Drone/Blueprints/BP_Mini_Drone.Use_Mini_drone` true _vehicle_p)
    (bind _output_get (set `/Game/SplinterCellMain/Blueprints_Main/Drone/Blueprints/BP_Mini_Drone.Character` (`GameplayStatics.GetPlayerCharacter` 0) _vehicle_p))
    (`Controller.Possess` (`GameplayStatics.GetPlayerController` 0) _vehicle_p)
    (`SceneComponent.SetVisibility` (`/Game/SplinterCellMain/Blueprints_Main/Drone/Blueprints/BP_Mini_Drone.Widget_3P_Health` _vehicle_p) false false)))