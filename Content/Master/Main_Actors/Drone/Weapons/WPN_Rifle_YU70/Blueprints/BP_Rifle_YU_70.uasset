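; YU70 rifle weapon Blueprint, filed under drone weapons, that handles automatic fire, clip ammo and reload.
; Fire start runs a looping timer at the rate of fire, spending ammo to spawn 7.62mm projectiles with sound, muzzle flash and shell ejection.
; A DoOnce with a short delay throttles shell-drop audio; fire stop, empty clip and reload clear the timer, and reload instantly refills the clip.
; Construction fills the clip and creates a dynamic weapon material.
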(event `CE_Fire_STart`
  (bind _sk_weapon (`self.SK_Weapon`))
  (bind _sk_weapon_2 (`self.SK_Weapon`))
  ;[1 1 1] Nodes controling machine gun ( rate of fire, overheat sound and texture, allso checking if vehicle is empty and then to stop machine gun to fire )
  (bind _returnvalue (`KismetSystemLibrary.K2_SetTimerDelegate` (delegate `CE_Fire_STart`) (`self.YU70_Rate_OF_Fire`) true))
  (`/Engine/EditorBlueprintResources/StandardMacros.CompareInt` (`self.Clip_size`)
    (:`>`
      (`|ExecutionSequence`
        (:`then_0`
          (set `self.Clip_size` (- (`self.Clip_size`) 1))
          (`|SpawnActorFromClass` "/Game/SplinterCellMain/Blueprints_Main/Drone/Weapons/WPN_Rifle_YU70/Blueprints/BP_7_62mm_Pprojectile.BP_7_62mm_Pprojectile_C" (`SceneComponent.GetSocketTransform` (`self.Bullet_origin`) "Spring_end_point" "RTS_World") "AlwaysSpawn" "OverrideRootScale" null (`self.Instigator`)) ; Connect this if you want to spawn projectile from Micro 10
          (`GameplayStatics.SpawnSoundAttached` "/Game/SplinterCellMain/Blueprints_Main/Drone/Weapons/WPN_Rifle_YU70/Sounds/Cue/SC_Rifle_YU70_Fire.SC_Rifle_YU70_Fire" _sk_weapon_2 "Coax" (0.0 0.0 0.0) (struct) "KeepRelativeOffset" false 1.0 (`self.GetActorTimeDilation`) 0.0 null null)
          (`GameplayStatics.SpawnEmitterAttached` "/Game/SplinterCellMain/Blueprints_Main/Drone/Weapons/WPN_Rifle_YU70/Particles/PS_Rifle_Muzzle_Flash.PS_Rifle_Muzzle_Flash" _sk_weapon_2 "Fire")
          (`GameplayStatics.SpawnEmitterAttached` "/Game/SplinterCellMain/Blueprints_Main/Drone/Weapons/WPN_Rifle_YU70/Particles/PS_ejection.PS_ejection" _sk_weapon_2 "Shell")
          (`/Engine/EditorBlueprintResources/StandardMacros.DoOnce` false :!label _label
            (:`Completed`
              (`|ExecutionSequence`
                (:`then_0`
                  (`GameplayStatics.SpawnSoundAttached` "/Game/SplinterCellMain/Blueprints_Main/Drone/Weapons/WPN_Rifle_YU70/Sounds/Cue/SC_Global_Shells_Drop.SC_Global_Shells_Drop" _sk_weapon_2 "None" (0.0 0.0 0.0) (struct) "KeepRelativeOffset" false (`self.Volume_ejection_shells`) (`self.GetActorTimeDilation`) 0.0 null null)
                  (`KismetSystemLibrary.Delay` 0.1)
                  (goto _label :!via `Reset`))
                (:`then_1`
                  (`SkeletalMeshComponent.PlayAnimation` _sk_weapon "/Game/SplinterCellMain/Blueprints_Main/Drone/Weapons/WPN_Rifle_YU70/Animation/Anim_Rifle_YU70_Fire.Anim_Rifle_YU70_Fire" true))))))
        (:`then_1`
          (goto _label_3 :!via `Reset`))))
    (:`==`
      (`KismetSystemLibrary.K2_ClearAndInvalidateTimerHandle` _returnvalue :!label _label_2)
      (`/Engine/EditorBlueprintResources/StandardMacros.DoOnce` false :!label _label_3
        (:`Completed`
          (`SkeletalMeshComponent.SetPosition` _sk_weapon 0.0 true)
          (`SkeletalMeshComponent.Stop` _sk_weapon)
          (if (<= (`self.Clip_size`) 0)
            (`GameplayStatics.SpawnSoundAttached` "/Game/SplinterCellMain/Blueprints_Main/Drone/Weapons/WPN_Pistol_H9/Sounds/Cue/SC_Pistol_Empty.SC_Pistol_Empty" _sk_weapon "None" (0.0 0.0 0.0) (struct) "KeepRelativeOffset" false 2.0 (`self.GetActorTimeDilation`) 0.0 null null)))))))

(event `CE_Fire_Stop`
  ;[1 1 1] Nodes controling machine gun ( rate of fire, overheat sound and texture, allso checking if vehicle is empty and then to stop machine gun to fire )
  (goto _label_2))

(event `CE_Reload`
  (bind _clip_size_max (`self.Clip_size_MAX`))
  ;[1 1 1] Nodes controling machine gun ( rate of fire, overheat sound and texture, allso checking if vehicle is empty and then to stop machine gun to fire )
  (`|ExecutionSequence`
    (:`then_0`
      (goto _label_2))
    (:`then_1`
      (`/Engine/EditorBlueprintResources/StandardMacros.CompareInt` (`self.Clip_size`) _clip_size_max
        (:`<`
          (set `self.Clip_size` _clip_size_max))))))

(fn `UserConstructionScript`
  (set `self.Clip_size` (`self.Clip_size_MAX`))
  (bind _returnvalue (`PrimitiveComponent.CreateDynamicMaterialInstance` (`self.SK_Weapon`) 0 "/Game/SplinterCellMain/Blueprints_Main/Drone/Weapons/WPN_Rifle_YU70/Materials/M_Rifle_YU_70.M_Rifle_YU_70" "None"))
  (set `self.MI_Weapom` _returnvalue))