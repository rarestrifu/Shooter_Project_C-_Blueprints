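; H9 pistol weapon actor, filed under the drone's weapons, that handles firing, ammo and reload.
; Each fire event spends a round, spawns a 9mm projectile, muzzle flash, shell ejection and time-dilation-pitched sound, with a DoOnce throttling shell sound and fire animation.
; A second DoOnce, re-armed by each shot, plays empty animation and sound on empty-clip fire or fire stop.
; Reload instantly refills the clip; construction fills it and creates a dynamic material.
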(event `CE_Fire_STart`
  (bind _sk_weapon (`self.SK_Weapon`))
  (bind _sk_weapon_2 (`self.SK_Weapon`))
  ;[1 1 1] Nodes controling machine gun ( rate of fire, overheat sound and texture, allso checking if vehicle is empty and then to stop machine gun to fire )
  (`/Engine/EditorBlueprintResources/StandardMacros.CompareInt` (`self.Clip_size`)
    (:`>`
      (`|ExecutionSequence`
        (:`then_0`
          (set `self.Clip_size` (- (`self.Clip_size`) 1))
          (`|SpawnActorFromClass` "/Game/SplinterCellMain/Blueprints_Main/Drone/Weapons/WPN_Pistol_H9/Blueprints/BP__Pistol_9mm_Pprojectile.BP__Pistol_9mm_Pprojectile_C" (`SceneComponent.GetSocketTransform` (`self.Bullet_origin`) "Spring_end_point" "RTS_World") "AlwaysSpawn" "OverrideRootScale" null (`self.Instigator`))
          (`GameplayStatics.SpawnSoundAttached` "/Game/SplinterCellMain/Blueprints_Main/Drone/Weapons/WPN_Pistol_H9/Sounds/Cue/SC_Pistol_H9_Fire.SC_Pistol_H9_Fire" _sk_weapon_2 "Coax" (0.0 0.0 0.0) (struct) "KeepRelativeOffset" false 1.0 (`self.GetActorTimeDilation`) 0.0 null null)
          (`GameplayStatics.SpawnEmitterAttached` "/Game/SplinterCellMain/Blueprints_Main/Drone/Weapons/WPN_Pistol_H9/Particles/PS_Pistol_Muzzle_Flash.PS_Pistol_Muzzle_Flash" _sk_weapon_2 "Fire")
          (`GameplayStatics.SpawnEmitterAttached` "/Game/SplinterCellMain/Blueprints_Main/Drone/Weapons/WPN_Pistol_H9/Particles/PS_ejection_Pistol.PS_ejection_Pistol" _sk_weapon_2 "Shell")
          (`/Engine/EditorBlueprintResources/StandardMacros.DoOnce` false :!label _label
            (:`Completed`
              (`|ExecutionSequence`
                (:`then_0`
                  (`GameplayStatics.SpawnSoundAttached` "/Game/SplinterCellMain/Blueprints_Main/Drone/Weapons/WPN_Rifle_YU70/Sounds/Cue/SC_Global_Shells_Drop.SC_Global_Shells_Drop" _sk_weapon_2 "None" (0.0 0.0 0.0) (struct) "KeepRelativeOffset" false (`self.Volume_ejection_shells`) (`self.GetActorTimeDilation`) 0.0 null null)
                  (`KismetSystemLibrary.Delay` 0.1)
                  (goto _label :!via `Reset`))
                (:`then_1`
                  (`SkeletalMeshComponent.PlayAnimation` (`self.SK_Weapon`) "/Game/SplinterCellMain/Blueprints_Main/Drone/Weapons/WPN_Pistol_H9/Animation/Anim_SK_Pistol_H9_Fire_Auto.Anim_SK_Pistol_H9_Fire_Auto" false))))))
        (:`then_1`
          (goto _label_2 :!via `Reset`))))
    (:`==`
      (`/Engine/EditorBlueprintResources/StandardMacros.DoOnce` false :!label _label_2
        (:`Completed`
          (`SkeletalMeshComponent.PlayAnimation` _sk_weapon "/Game/SplinterCellMain/Blueprints_Main/Drone/Weapons/WPN_Pistol_H9/Animation/Anim_SK_Pistol_H9_Empty.Anim_SK_Pistol_H9_Empty" false)
          (`GameplayStatics.SpawnSoundAttached` "/Game/SplinterCellMain/Blueprints_Main/Drone/Weapons/WPN_Pistol_H9/Sounds/Cue/SC_Pistol_Empty.SC_Pistol_Empty" _sk_weapon "None" (0.0 0.0 0.0) (struct) "KeepRelativeOffset" false 1.0 (`self.GetActorTimeDilation`) 0.0 null null))))
    (:`<`
      (goto _label_2))))

(event `CE_Fire_Stop`
  ;[1 1 1] Nodes controling machine gun ( rate of fire, overheat sound and texture, allso checking if vehicle is empty and then to stop machine gun to fire )
  (goto _label_2))

(event `CE_Reload`
  (bind _clip_size_max (`self.Clip_size_MAX`))
  ;[1 1 1] Nodes controling machine gun ( rate of fire, overheat sound and texture, allso checking if vehicle is empty and then to stop machine gun to fire )
  (`/Engine/EditorBlueprintResources/StandardMacros.CompareInt` (`self.Clip_size`) _clip_size_max
    (:`<`
      (set `self.Clip_size` _clip_size_max))))

(fn `UserConstructionScript`
  (set `self.Clip_size` (`self.Clip_size_MAX`))
  (bind _returnvalue (`PrimitiveComponent.CreateDynamicMaterialInstance` (`self.SK_Weapon`) 0 "/Game/SplinterCellMain/Blueprints_Main/Drone/Weapons/WPN_Pistol_H9/Materials/M_Pistol_H9.M_Pistol_H9" "None"))
  (set `self.MI_Weapom` _returnvalue))