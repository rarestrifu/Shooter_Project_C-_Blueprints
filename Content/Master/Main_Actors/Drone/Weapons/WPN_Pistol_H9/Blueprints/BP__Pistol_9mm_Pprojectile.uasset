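; Projectile for the H9 9mm pistol that handles damage and impact feedback on hit.
; Tags on the hit actor select the damage class, and BP_Headshot implementers receive random damage with the bone name.
; Head and flesh hits spawn blood, while other surfaces get an impulse, sparks and an attached decal with timeline-animated emissive.
; Tagged targets show a brief screen-projected hit marker, otherwise a ricochet sound plays, then the projectile destroys itself.
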(event `self.ReceiveHit`
  (params (MyComp :type "PrimitiveComponent Object Reference") (Other :type "Actor Object Reference") (OtherComp :type "PrimitiveComponent Object Reference") (bSelfMoved :type Boolean) (HitLocation :type "Vector Structure") (HitNormal :type "Vector Structure") (NormalImpulse :type "Vector Structure") (Hit :type "HitResult Structure (by ref)"))
  (bind _returnvalue (`GameplayStatics.GetPlayerController` 0))
  (bind _returnvalue_2 (`self.GetActorTimeDilation`))
  (bind (_bblockinghit _binitialoverlap _time _distance _location _impactpoint _normal _impactnormal _physmat _hitactor _hitcomponent _hitbonename _hititem _faceindex _tracestart) (`GameplayStatics.BreakHitResult` Hit))
  (bind _returnvalue_3 (`KismetSystemLibrary.MakeLiteralName` _hitbonename))
  (bind _returnvalue_4 (`KismetMathLibrary.MakeRotFromXY` _impactnormal _impactnormal))
  (`/Engine/EditorBlueprintResources/StandardMacros.IsValid` Other
    (:`Is Valid`
      (for _array_element (`Actor.Tags` Other)
        (switch `name` _array_element
          (:`9mm_Damage_Class_5`
            (set `self.Base_Damage` (`self.9mm_Damage_Class_5`)))
          (:`9mm_Damage_Class_10`
            (set `self.Base_Damage` (`self.9mm_Damage_Class_10`)))
          (:`9mm_Damage_Class_15`
            (set `self.Base_Damage` (`self.9mm_Damage_Class_15`)))
          (:`9mm_Damage_Class_20`
            (set `self.Base_Damage` (`self.9mm_Damage_Class_20`)))
          (:`9mm_Damage_Class_25`
            (set `self.Base_Damage` (`self.9mm_Damage_Class_25`))))
        (`GameplayStatics.ApplyDamage` Other (`self.Base_Damage`) null (`self.GetInstigator`))
        (`/Engine/EditorBlueprintResources/StandardMacros.DoOnce` false :!label _label
          (:`Completed`
            (if (`KismetSystemLibrary.DoesImplementInterface` _hitactor "/Game/SplinterCellMain/Blueprints_Main/Drone/Demo/Pawn_Third_P_EA3D/Blueprints/BP_Headshot.BP_Headshot_C")
              (message `/Game/SplinterCellMain/Blueprints_Main/Drone/Demo/Pawn_Third_P_EA3D/Blueprints/BP_Headshot.Headshot` _hitactor (`KismetMathLibrary.Conv_IntToDouble` (`KismetMathLibrary.RandomIntegerInRange` 25 30)) _returnvalue_3)
              (if (== _returnvalue_3 "Head")
                (`GameplayStatics.SpawnSoundAtLocation` "/Game/SplinterCellMain/Blueprints_Main/Drone/Weapons/WPN_Rifle_YU70/Sounds/Cue/SC_Head_Shot.SC_Head_Shot" _location (struct) 1.0 1.0 0.0 null null)
                (`GameplayStatics.SpawnEmitterAtLocation` "/Game/SplinterCellMain/Blueprints_Main/Drone/Demo/Pawn_Third_P_EA3D/Particles/PS_Blood_Body_Impcat.PS_Blood_Body_Impcat" _location _returnvalue_4 (2.0 2.0 2.0))
                (if (and _bblockinghit (`KismetArrayLibrary.Array_Contains` (`self.9mm_Damage_Class_TAGS`) _array_element) (not (`self.ActorHasTag` _hitactor "NO_Damage")) (`self.ActorHasTag` _hitactor "Hit_Marker")) :!label _label_2
                  (bind _returnvalue_5 (`|CreateWidget` "/Game/SplinterCellMain/Blueprints_Main/Drone/UI/UMG_Hit_Marker.UMG_Hit_Marker_C" _returnvalue))
                  (bind _output_get (set `self.UMG_Hit_Marker` _returnvalue_5))
                  (`UserWidget.SetPositionInViewport` _output_get (`WidgetLayoutLibrary.ProjectWorldLocationToWidgetPosition` _returnvalue HitLocation) false)
                  (`UserWidget.AddToViewport` _output_get 0)
                  (`GameplayStatics.SpawnSoundAtLocation` "/Game/SplinterCellMain/Blueprints_Main/Drone/Weapons/WPN_Rifle_YU70/Sounds/Cue/SC_Body_Hit.SC_Body_Hit" _normal (struct) 1.0 _returnvalue_2 0.0 null null)
                  (`KismetSystemLibrary.Delay` 0.1)
                  (`Widget.RemoveFromParent` _output_get)
                  (else
                    (`GameplayStatics.SpawnSoundAtLocation` "/Game/SplinterCellMain/Blueprints_Main/Drone/Weapons/WPN_Rifle_YU70/Sounds/Cue/SC_Bullet_Ricochet.SC_Bullet_Ricochet" (0.0 0.0 0.0) (struct) 1.0 _returnvalue_2 0.0 null null)))
                (`ActorComponent.K2_DestroyComponent` (`self.Sphere`) :!label _label_3)
                (`ActorComponent.K2_DestroyComponent` (`self.CollisionComponent`))
                (`KismetSystemLibrary.Delay` 1.0)
                (`self.K2_DestroyActor`)
                (else
                  (if (and (> (`self.Base_Damage`) 0.0) (`KismetArrayLibrary.Array_Contains` (`self.Flesh`) (`GameplayStatics.GetObjectClass` _hitactor))) :!label _label_4
                    (`GameplayStatics.SpawnEmitterAtLocation` "/Game/SplinterCellMain/Blueprints_Main/Drone/Demo/Pawn_Third_P_EA3D/Particles/PS_Blood_Body_Impcat.PS_Blood_Body_Impcat" _location _returnvalue_4)
                    (goto _label_2)
                    (else
                      (`RadialForceComponent.FireImpulse` (`self.RadialForce1`))
                      (`GameplayStatics.SpawnEmitterAtLocation` "/Game/SplinterCellMain/Blueprints_Main/Drone/Weapons/WPN_Rifle_YU70/Particles/PS_Impact_machine_gun.PS_Impact_machine_gun" _location (`KismetMathLibrary.MakeRotator` (.x _tracestart) (.y _tracestart)))
                      (bind _returnvalue_6 (`GameplayStatics.SpawnDecalAtLocation` "/Game/SplinterCellMain/Blueprints_Main/Drone/Weapons/WPN_Rifle_YU70/Materials/M_Bullet_Iimpact_Metall_BaseColor.M_Bullet_Iimpact_Metall_BaseColor" (3.0 3.0 3.0) HitLocation (`KismetMathLibrary.MakeRotFromX` _normal) (`self.Decal_Life_Span`)))
                      (`DecalComponent.SetFadeScreenSize` _returnvalue_6 0.001)
                      (`|ExecutionSequence`
                        (:`then_0`
                          (`SceneComponent.K2_AttachToComponent` _returnvalue_6 _hitcomponent "None" "KeepWorld" "KeepWorld" "KeepWorld" true)
                          (`/Engine/EditorBlueprintResources/StandardMacros.IsValid` Other
                            (:`Is Valid`
                              (goto _label_2))
                            (:`Is Not Valid`
                              (goto _label_3))))
                        (:`then_1`
                          ;[1 1 1] Bullet hole emissive
                          (`/Engine/EditorBlueprintResources/StandardMacros.DoOnce` false
                            (:`Completed`
                              (bind _returnvalue_7 (`DecalComponent.CreateDynamicMaterialInstance` _returnvalue_6))
                              (bind (_direction _newtrack_0) (`Timeline|Timeline_Emissaive` :!via `PlayFromStart`)
                                (:`Update`
                                  (`MaterialInstanceDynamic.SetScalarParameterValue` _returnvalue_7 "Emissive_Power" (* _newtrack_0 10.0)))
                                (:`Finished`
                                  (`self.K2_DestroyActor`)))))))))))
              (else
                (goto _label_4)))))))
    (:`Is Not Valid`
      _))
  (goto _label))

(event `self.ReceiveBeginPlay`
  (`PrimitiveComponent.IgnoreActorWhenMoving` (`self.CollisionComponent`) (`self.GetInstigator`) true)
  (`PrimitiveComponent.IgnoreActorWhenMoving` (`self.Sphere`) (`self.GetInstigator`) true))

(fn `UserConstructionScript`)