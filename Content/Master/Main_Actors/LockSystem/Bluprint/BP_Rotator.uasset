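; BP_Rotator is a lock system actor that plays an endless spin-and-bob animation on its Cube once the opening action fires.
; ActiononOpening starts two Delay-driven loops through a Sequence: one flips the Switch boolean every second.
; The other runs on a short delay, stepping the Cube's yaw and moving it up or down according to Switch, without using Tick or a Timeline.
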(event `self.ReceiveBeginPlay`
  (`parent.ReceiveBeginPlay`))

(event `/Game/SplinterCellMain/Blueprints_Main/LockSystem/Bluprint/Interfase/BP_Interfase.Action on opening`
  ;[1 1 1] Play Anim
  (`|ExecutionSequence`
    (:`then_0`
      (if (`self.Switch`) :!label _label
        (set `self.Switch` false)
        (else
          (set `self.Switch` true)))
      (`KismetSystemLibrary.Delay` 1.0)
      (goto _label))
    (:`then_1`
      (`KismetSystemLibrary.Delay` 0.01 :!label _label_2)
      (`SceneComponent.K2_AddWorldRotation` (`self.Cube`) (struct :`Yaw` 1.0) false false)
      (if (`self.Switch`)
        (`SceneComponent.K2_AddWorldOffset` (`self.Cube`) (0.0 0.0 1.0) false false)
        (goto _label_2)
        (else
          (`SceneComponent.K2_AddWorldOffset` (`self.Cube`) (0.0 0.0 -1.0) false false)
          (goto _label_2))))))

(fn `UserConstructionScript`
  (`parent.UserConstructionScript`))