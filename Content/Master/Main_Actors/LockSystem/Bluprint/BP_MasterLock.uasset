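; BP_MasterLock is a base lock actor that the player can interact with, intended as a parent for specific locks.
; On BeginPlay it passes its lock settings (key, code, widget category, open state) to BPLockSystemComponent, which also handles Interact calls.
; SetLockActor updates the Open state.
; Opening, open and locked action events are empty hooks, and the widget-button and lock-component functions are stubs returning false.
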(event `self.ReceiveBeginPlay`
  ;[1 1 1] Start Game
  (`/Game/SplinterCellMain/Blueprints_Main/LockSystem/Bluprint/Component/BP_LockSystemComponent.Begin Play` (`self.BP_LockSystemComponent`) (`self.On Lock Array`) self (`self.Open?`) (`self.Length Cod`) (`self.Key`) (`self.CategoriesWidget`) (`self.Random cod?`) (`self.Cod`)))

(event `/Game/SplinterCellMain/Blueprints_Main/LockSystem/Bluprint/Interfase/BP_Interfase.Action on opening`
  ;[1 1 1] What happens when you open
)

(event `/Game/SplinterCellMain/Blueprints_Main/LockSystem/Bluprint/Interfase/BP_Interfase.Action`
  ;[1 1 1] Actions if open
)

(event `/Game/SplinterCellMain/Blueprints_Main/LockSystem/Bluprint/Interfase/BP_Interfase.Action on locked`
  ;[1 1 1] Action on locked
)

(fn `Button To Widget`
  (params (Button :type "/Game/SplinterCellMain/Blueprints_Main/LockSystem/Enumeration/E_Button Enum" :default "NewEnumerator10") (Pressed :type Boolean))
  (returns (`Success?` :type Boolean))
  (return false))

(fn `Interact`
  (params (`BP_Interact Component` :type "/Game/SplinterCellMain/Blueprints_Main/LockSystem/Bluprint/Component/BP_InteractComponent Object Reference"))
  (returns (`Success?` :type Boolean))
  ;[1 1 1] Interact
  (`/Game/SplinterCellMain/Blueprints_Main/LockSystem/Bluprint/Component/BP_LockSystemComponent.Interact` (`self.BP_LockSystemComponent`) `BP_Interact Component` (`self.Open?`) (`self.Can I open it directly?`))
  (return true))

(fn `Lock Component`
  (params (`Lock Component` :type "/Game/SplinterCellMain/Blueprints_Main/LockSystem/Bluprint/Component/BP_LockSystemComponent Object Reference"))
  (returns (`Success?` :type Boolean))
  (return false))

(fn `Set Lock Actor`
  (params (`Open?` :type Boolean))
  (returns (Open :type Boolean))
  (bind _output_get (set `self.Open?` `Open?`))
  (return _output_get))

(fn `UserConstructionScript`)