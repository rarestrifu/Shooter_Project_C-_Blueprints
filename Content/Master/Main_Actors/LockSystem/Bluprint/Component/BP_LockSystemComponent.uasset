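; Lock system component that handles key and code unlocking for a lockable actor.
; On interaction it runs the actor's action if open; otherwise, if directly accessible, it searches the interactor's inventory for the key, then shows a digital, rotational or picklock widget.
; Entered characters are checked against a fixed or random code at full length, with optional sounds.
; State changes notify the owning actor and propagate to linked locks.
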(fn `Add Char`
  (params (NewParam :type String))
  (set `self.Input Cod` (`KismetStringLibrary.Concat_StrStr` (`self.Input Cod`) NewParam))
  (`self.Update Input`)
  (return))

(fn `Begin Play`
  (params (`On Lock Array` :type "Array of /Game/SplinterCellMain/Blueprints_Main/LockSystem/Bluprint/BP_MasterLock Object Reference") (`Lock Actor` :type "/Game/SplinterCellMain/Blueprints_Main/LockSystem/Bluprint/BP_MasterLock Object Reference") (`Lock Open?` :type Boolean) (`Length Сod ` :type Integer) (Key :type "/Game/SplinterCellMain/Blueprints_Main/LockSystem/Bluprint/Key/BP_MasterKeys Class Reference") (CategoriesWidget :type "/Game/SplinterCellMain/Blueprints_Main/LockSystem/Enumeration/E_CategoriesWidget Enum" :default "NewEnumerator0") (`Random Cod?` :type Boolean) (Cod :type String))
  ;[1 1 1] Set Param
  (set `self.On Lock` `On Lock Array`)
  (set `self.A lockable object` `Lock Actor`)
  (set `self.Lock Open?` `Lock Open?`)
  (set `self.Length Сod ` `Length Сod `)
  (set `self.Key` Key)
  (set `self.CategoriesWidget` CategoriesWidget)
  (set `self.Random Cod?` `Random Cod?`)
  (set `self.Cod` Cod)
  (`self.Random Cod` (`self.Random Cod?`)))

(fn `Clear Input Cod`
  (set `self.Input Cod` ""))

(fn `Full Array Open?`
  (returns (is :type Boolean))
  (locals (`Local_Open?` :type Boolean))
  (`/Engine/EditorBlueprintResources/StandardMacros.IsValid` (`|GetArrayItem` (`self.On Lock`))
    (:`Is Valid`
      (set `local.Local_Open?` true)
      (for _array_element (`self.On Lock`)
        (if (not (`/Game/Master/Main_Actors/LockSystem/Bluprint/Component/BP_LockSystemComponent.Lock Open?` (`/Game/SplinterCellMain/Blueprints_Main/LockSystem/Bluprint/BP_MasterLock.BP_LockSystemComponent` _array_element)))
          (set `local.Local_Open?` false)
          (break)))
      (return (`local.Local_Open?`)))
    (:`Is Not Valid`
      (return false))))

(fn `Interact`
  (params (`BP_Interact Component` :type "/Game/SplinterCellMain/Blueprints_Main/LockSystem/Bluprint/Component/BP_InteractComponent Object Reference") (`Open?` :type Boolean) (`Can I open it directly?` :type Boolean))
  (bind _output_get (set `self.InteractComponent` `BP_Interact Component`))
  (set `/Game/SplinterCellMain/Blueprints_Main/LockSystem/Bluprint/Component/BP_InteractComponent.Lock SystemComponent` self _output_get)
  (bind _output_get_2 (set `self.Lock Open?` `Open?`))
  (if _output_get_2
    (message `/Game/SplinterCellMain/Blueprints_Main/LockSystem/Bluprint/Interfase/BP_Interfase.Action` (`self.A lockable object`) :!label _label)
    (return)
    (elif `Can I open it directly?`
      (`self.Used Keys`)
      (if (`self.Lock Open?`)
        (goto _label)
        (else
          (`self.Show / Hide Lock Widget` true)))
      (else
        (`KismetSystemLibrary.PrintString` "It is impossible to access directly")))))

(fn `Open`
  (params (`Play Sound?` :type Boolean))
  (if `Play Sound?`
    (`GameplayStatics.PlaySound2D` (`self.S_True`) 1.0 1.0 0.0 null null))
  (`self.Set Lock` true)
  (return))

(fn `Random Cod`
  (params (`Random?` :type Boolean))
  (if `Random?`
    (set `self.Cod` (`KismetStringLibrary.Conv_IntToString` (select `int` (`self.Length Сod `) :`0` 0 :`1` (`KismetMathLibrary.RandomIntegerInRange` 0 9) :`2` (`KismetMathLibrary.RandomIntegerInRange` 10 99) :`3` (`KismetMathLibrary.RandomIntegerInRange` 100 999) :`4` (`KismetMathLibrary.RandomIntegerInRange` 1000 9999) :`5` (`KismetMathLibrary.RandomIntegerInRange` 10000 99999) :`6` (`KismetMathLibrary.RandomIntegerInRange` 100000 999999) :`7` (`KismetMathLibrary.RandomIntegerInRange` 1000000 9999999) :`8` (`KismetMathLibrary.RandomIntegerInRange` 10000000 99999999) :`9` (`KismetMathLibrary.RandomIntegerInRange` 100000000 999999999))))))

(fn `Set Lock`
  (params (`Lock Open?` :type Boolean))
  (bind _open (message `/Game/SplinterCellMain/Blueprints_Main/LockSystem/Bluprint/Interfase/BP_Interfase.Set Lock Actor` (`self.A lockable object`) `Lock Open?`))
  (bind _output_get (set `self.Lock Open?` _open))
  (if _output_get
    (`self.Set Lock Array` true)
    (message `/Game/SplinterCellMain/Blueprints_Main/LockSystem/Bluprint/Interfase/BP_Interfase.Action on opening` (`self.A lockable object`))
    (else
      (`self.Set Lock Array` false)
      (message `/Game/SplinterCellMain/Blueprints_Main/LockSystem/Bluprint/Interfase/BP_Interfase.Action on locked` (`self.A lockable object`))))
  (return))

(fn `Set Lock Array`
  (params (`Lock Open?` :type Boolean))
  (for _array_element (`self.On Lock`)
    (`/Engine/EditorBlueprintResources/StandardMacros.IsValid` _array_element
      (:`Is Valid`
        (`self.Set Lock` (`/Game/SplinterCellMain/Blueprints_Main/LockSystem/Bluprint/BP_MasterLock.BP_LockSystemComponent` _array_element) `Lock Open?`))))
  (return))

(fn `Set Sound`
  (params (True :type "SoundBase Object Reference") (Wrong :type "SoundBase Object Reference") (`Play True Sound?` :type Boolean) (`Play Wrong Sound?` :type Boolean))
  (set `self.S_True` True)
  (set `self.S_Wrong` Wrong)
  (set `self.Play True Sound?` `Play True Sound?`)
  (set `self.Play Wrong Sound?` `Play Wrong Sound?`))

(fn `Show / Hide Lock Widget`
  (params (`Open?` :type Boolean))
  (bind _returnvalue (`GameplayStatics.GetPlayerController` 0))
  (bind _returnvalue_2 (`GameplayStatics.GetPlayerController` 0))
  (if (`self.Lock Open?`)
    ;[1 1 1] Hide
    (`self.W Lock` :!label _label
      (:`then`
        (`Widget.RemoveFromParent` (`self.W Lock`))
        (set `self.W Lock` null)
        ;[1 1 1] Set input
        (set `PlayerController.bShowMouseCursor` false _returnvalue)
        (`WidgetBlueprintLibrary.SetInputMode_GameOnly` _returnvalue))
      (:`else`))
    (elif (not `Open?`)
      (goto _label)
      (else
        ;[1 1 1] Open
        (`self.W Lock`
          (:`then`)
          (:`else`
            (bind _returnvalue_3 (`|CreateWidget` (select `/Game/SplinterCellMain/Blueprints_Main/LockSystem/Enumeration/E_CategoriesWidget` (`self.CategoriesWidget`) :`NewEnumerator0` "/Game/SplinterCellMain/Blueprints_Main/LockSystem/Widget/W_DigitalLock.W_DigitalLock_C" :`NewEnumerator1` "/Game/SplinterCellMain/Blueprints_Main/LockSystem/Widget/W_RotationalElements.W_RotationalElements_C" :`NewEnumerator2` "/Game/SplinterCellMain/Blueprints_Main/LockSystem/Widget/W_Picklock.W_Picklock_C" :!type "UserWidget Class Reference")))
            (bind _output_get (set `self.W Lock` _returnvalue_3))
            (message `/Game/SplinterCellMain/Blueprints_Main/LockSystem/Bluprint/Interfase/BP_Interfase.Lock Component` _output_get self)
            (`UserWidget.AddToViewport` _output_get 0)
            (bind _output_get_2 (set `PlayerController.bShowMouseCursor` true _returnvalue_2))
            (`WidgetBlueprintLibrary.SetInputMode_GameAndUIEx` _returnvalue_2 (`self.W Lock`) "DoNotLock" _output_get_2))))))
  (return))

(fn `Update Input`
  (if (`self.Сheck Length`)
    (if (`self.Сheck Cod`)
      (`self.Open` (`self.Play True Sound?`))
      (else
        (`self.Wrong` (`self.Play Wrong Sound?`)))))
  (return))

(fn `Used Keys`
  (locals (`Local_Open?` :type Boolean))
  (`self.Key`
    (:`then`
      (if (`KismetArrayLibrary.Array_IsValidIndex` (`/Game/SplinterCellMain/Blueprints_Main/LockSystem/Bluprint/Component/BP_InteractComponent.Inventory` (`self.InteractComponent`)))
        (for _array_element (`/Game/SplinterCellMain/Blueprints_Main/LockSystem/Bluprint/Component/BP_InteractComponent.Inventory` (`self.InteractComponent`))
          (if (`KismetSystemLibrary.IsValidClass` _array_element)
            (if (== (`self.Key`) _array_element)
              (`self.Set Lock` true)
              (break))))))
    (:`else`
      _))
  (return))

(fn `Wrong`
  (params (`Play Sound?` :type Boolean))
  (if `Play Sound?`
    (`GameplayStatics.PlaySound2D` (`self.S_Wrong`) 1.0 1.0 0.0 null null))
  (set `self.Input Cod` "")
  (return))

(fn `Сheck Cod`
  (returns (is :type Boolean))
  (return (`KismetStringLibrary.EqualEqual_StrStr` (`self.Cod`) (`self.Input Cod`))))

(fn `Сheck Length`
  (returns (`Full?` :type Boolean))
  (return (>= (`KismetStringLibrary.Len` (`self.Input Cod`)) (`self.Length Сod `))))