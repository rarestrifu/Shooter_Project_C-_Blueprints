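; BP_Lock_7 is a key-operated lock for the lockers collection, extending a parent lock and requiring key number 1.
; Key_Lock checks the player's keys while Door1 is closed, then shows the key mesh and toggles the lock.
; A timeline spins the key one full turn, reversing to relock, and hides it when finished.
; Key_Lock_info reports lock state and required key, while Interact_Lock always returns failure.
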(event `self.ReceiveBeginPlay`
  (`parent.ReceiveBeginPlay`)
  (set `self.Keys_Lock` true)
  (set `self.Need_Key_Num` 1))

(event `Key_Interact`
  (bind _returnvalue (== (`self.Need_Key_Num`) 1))
  (if (not (`self.Lock_Opened`))
    (set `self.Lock_Opened` true)
    (bind (_direction _newtrack_0) (`Timeline|Timeline_1` :!label _label)
      (:`Update`
        (`SceneComponent.K2_SetRelativeRotation` (`self.Key`) (`KismetMathLibrary.MakeRotator` 90.0 (`KismetMathLibrary.Lerp` (select `bool` _returnvalue :`true` -90.0 :!type "Float (single-precision)") (select `bool` _returnvalue :`false` -360.0 :`true` -450.0 :!type "Float (single-precision)") _newtrack_0)) false false))
      (:`Finished`
        (`SceneComponent.SetVisibility` (`self.Key`) false false)))
    (else
      (set `self.Lock_Opened` false)
      (goto _label :!via `Reverse`))))

(fn `Interact_Lock`
  (returns (Success :type Boolean) (Selected_Lock :type "/Game/SplinterCellMain/Blueprints_Main/Lockers_Collection/Blueprints/Locks/BP_Locks_Parent Object Reference"))
  (return false null))

(fn `Key_Lock`
  (returns (Success :type Boolean))
  (if (not (`self.Door_1_Open?`))
    (if (`|GetArrayItem` (`/Game/SplinterCellMain/Blueprints_Main/Lockers_Collection/DemoContent/FirstPersonBP/Blueprints/FirstPersonCharacter.Keys` (`self.Player`)) (`self.Need_Key_Num`))
      (`SceneComponent.SetVisibility` (`self.Key`) true false)
      (`self.Key_Interact`)
      (return true))))

(fn `Key_Lock_info`
  (returns (Success :type Boolean) (Lock_Opened :type Boolean) (Key :type Integer))
  (if (not (`self.Door_1_Open?`))
    (return true (`self.Lock_Opened`) (`self.Need_Key_Num`))))

(fn `UserConstructionScript`
  (`parent.UserConstructionScript`))