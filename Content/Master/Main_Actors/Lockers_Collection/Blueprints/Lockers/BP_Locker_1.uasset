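; BP_Locker_1 is a single-door locker variant that builds on a parent Blueprint and offers a choice of leg styles.
; The construction script registers its door mesh as Door1, then uses LegsType to show one of two leg sets and adjust the body height to match.
; BeginPlay runs the parent logic, then sets the door's end rotation for the inherited behavior.
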(event `self.ReceiveBeginPlay`
  (`parent.ReceiveBeginPlay`)
  (set `self.End_Rot_Door_1` -110.0))

(fn `UserConstructionScript`
  (bind _sm_locker_1_body (`self.SM_Locker_1_body`))
  (set `self.Door_1` (`self.SM_Locker_1_door`))
  (`parent.UserConstructionScript`)
  (`|ExecutionSequence`
    (:`then_0`
      (if (== (`self.Legs_Type`) 0)
        (`SceneComponent.SetVisibility` (`self.SM_Leg_1_body_1`) true true)
        (`SceneComponent.SetVisibility` (`self.SM_Leg_1_body_2`) true true)
        (`SceneComponent.SetVisibility` (`self.SM_Leg_1_body_3`) true true)
        (`SceneComponent.SetVisibility` (`self.SM_Leg_1_body_4`) true true)
        (`SceneComponent.SetVisibility` (`self.Leg_1`) false true)
        (`SceneComponent.SetVisibility` (`self.Leg_2`) false true)
        (`SceneComponent.SetVisibility` (`self.Leg_3`) false true)
        (`SceneComponent.SetVisibility` (`self.Leg_4`) false true)
        (`SceneComponent.K2_SetRelativeLocation` _sm_locker_1_body (0.0 0.0 10.043104) false true)))
    (:`then_1`
      (if (== (`self.Legs_Type`) 1)
        (`SceneComponent.SetVisibility` (`self.SM_Leg_1_body_1`) false true)
        (`SceneComponent.SetVisibility` (`self.SM_Leg_1_body_2`) false true)
        (`SceneComponent.SetVisibility` (`self.SM_Leg_1_body_3`) false true)
        (`SceneComponent.SetVisibility` (`self.SM_Leg_1_body_4`) false true)
        (`SceneComponent.SetVisibility` (`self.Leg_1`) true true)
        (`SceneComponent.SetVisibility` (`self.Leg_2`) true true)
        (`SceneComponent.SetVisibility` (`self.Leg_3`) true true)
        (`SceneComponent.SetVisibility` (`self.Leg_4`) true true)
        (`SceneComponent.K2_SetRelativeLocation` _sm_locker_1_body (0.0 0.0 5.078348) false true)))))