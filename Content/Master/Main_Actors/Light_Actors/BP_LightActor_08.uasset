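; BP_LightActor_08 is a tube light that an optional button actor switches on and off and that can be destroyed by bullets or radial damage.
; Tick polls the button to toggle light, emissive material and sound, and updates a child illumination sphere volume that shares the attenuation radius.
; Destruction plays a timeline flicker, sparks and destructible glass.
; ShotWithBullet marks the volume unlit, reports noise for AI and later disables Tick.
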(event `self.ReceiveBeginPlay`
  (bind _attenuation_radius (`self.Attenuation Radius`))
  ;[1 1 1] Begin Play
  (`|ExecutionSequence`
    (:`then_0`
      ;;[0 0 0] Set the world location for reference
      (set `self.World Location` (`SceneComponent.K2_GetComponentLocation` (`self.Light_Mesh`))))
    (:`then_1`
      ;;[0 0 0] Set associated actor as can be damaged or not
      (set `self.bCanBeDamaged` (`self.Is Destructable?`)))
    (:`then_2`
      ;;[0 0 0] Check for buttons
      (`/Engine/EditorBlueprintResources/StandardMacros.IsValid` (`self.Button Actor`)
        (:`Is Valid`
          (`LightComponent.SetIntensity` (`self.TubeLight`) (`self.New Intensity`))
          (`AudioComponent.SetVolumeMultiplier` (`self.Sound`) (`self.Sound Volume`)))
        (:`Is Not Valid`
          (set `self.Use Button?` false))))
    (:`then_3`
      ;;[0 0 0] Set reference to illumination volume child actor
      (bind _asbp_illumination_sphere_volume (cast `/Game/SplinterCellMain/Blueprints_Main/IlluminationDetection/Blueprints/IlluminationVolumes/BP_IlluminationSphereVolume` (`ChildActorComponent.ChildActor` (`self.BP_IlluminationSphereVolume`))))
      (set `self.Illumination Sphere Volume Ref` _asbp_illumination_sphere_volume))
    (:`then_4`
      ;;[0 0 0] Set matching attenuation radii
      (`LocalLightComponent.SetAttenuationRadius` (`self.TubeLight`) _attenuation_radius)
      (set `/Game/SplinterCellMain/Blueprints_Main/IlluminationDetection/Blueprints/IlluminationVolumes/BP_IlluminationVolumeMaster.AttenuationDistance` _attenuation_radius (`self.Illumination Sphere Volume Ref`)))))

(event `self.ReceiveTick`
  (params (DeltaSeconds :type "Float (single-precision)"))
  (bind _tubelight (`self.TubeLight`))
  (bind _illumination_sphere_volume_ref (`self.Illumination Sphere Volume Ref`))
  (bind _light_mesh (`self.Light_Mesh`))
  (bind _sound (`self.Sound`))
  ;[0 0 0] On TICK = Cheap
  (if (`self.Use Button?`)
    (`/Game/AdvancedLocomotionV4/Blueprints/Libraries/ALS_MacroLibrary.DoOnce Branch` (`/Game/Game/Blueprints/BP_I_Button.Is Pressed` (`self.Button Actor`))
      (:`True`
        (`SceneComponent.SetVisibility` _tubelight false false)
        (`MeshComponent.SetScalarParameterValueOnMaterials` _light_mesh "Emissive Value" 0.0)
        (`AudioComponent.Stop` _sound)
        (`/Game/SplinterCellMain/Blueprints_Main/IlluminationDetection/Blueprints/IlluminationVolumes/BP_IlluminationVolumeMaster.SetLightStatus` _illumination_sphere_volume_ref "NewEnumerator1"))
      (:`False`
        (`SceneComponent.SetVisibility` _tubelight true false)
        (`/Engine/EditorBlueprintResources/StandardMacros.IsValid` null
          (:`Is Valid`
            (`MeshComponent.SetScalarParameterValueOnMaterials` _light_mesh "Emissive Value" 15.0)
            (`AudioComponent.Play` _sound 0.0)
            (`/Game/SplinterCellMain/Blueprints_Main/IlluminationDetection/Blueprints/IlluminationVolumes/BP_IlluminationVolumeMaster.SetLightStatus` _illumination_sphere_volume_ref "NewEnumerator0")))))))

(event `self.ReceiveRadialDamage`
  (params (DamageReceived :type "Float (single-precision)") (DamageType :type "DamageType Object Reference") (Origin :type "Vector Structure") (HitInfo :type "HitResult Structure (by ref)") (InstigatedBy :type "Controller Object Reference") (DamageCauser :type "Actor Object Reference"))
  (bind _rect_lamp_glass_sm_dm (`self.Rect_Lamp_Glass_SM_DM`))
  (bind _tubelight (`self.TubeLight`))
  (bind _returnvalue (`SceneComponent.K2_GetComponentLocation` (`self.Arrow`)))
  (bind _returnvalue_2 (`SceneComponent.K2_GetComponentLocation` (`self.Arrow`)))
  ;[0 0 0] Lights out when hit by bullet
  (if (and (`self.Is Destructable?`) (not (`self.IsDead?`))) :!label _label
    (`|ExecutionSequence`
      (:`then_0`
        (set `self.IsDead?` true)
        (`/Engine/EditorBlueprintResources/StandardMacros.DoOnce` false
          (:`Completed`
            (`GameplayStatics.SpawnSoundAtLocation` "/Game/SplinterCellMain/Audio/Glass_Breaking/GLASS-SMASH_GEN-HDF-12972.GLASS-SMASH_GEN-HDF-12972" _returnvalue (struct) 1.0 1.0 0.0 null null)
            (bind (_direction _intensity_of_light) (`Timeline|Flicker`)
              (:`Update`
                (`LightComponent.SetIntensity` (`self.TubeLight`) (* _intensity_of_light 2000.0))
                (`MeshComponent.SetScalarParameterValueOnMaterials` (`self.Light_Mesh`) "Emissive Value" _intensity_of_light))
              (:`Finished`
                (`SceneComponent.SetVisibility` _tubelight false false)
                (`ActorComponent.K2_DestroyComponent` _tubelight)
                (bind _returnvalue_3 (`GameplayStatics.SpawnEmitterAtLocation` "/Game/SplinterCellMain/Particle_Effects/P_Sparks.P_Sparks" _returnvalue))
                (`AudioComponent.Stop` (`self.Sound`))
                (`MeshComponent.SetScalarParameterValueOnMaterials` (`self.Light_Mesh`) "Emissive Value" 0.0)
                (`KismetSystemLibrary.Delay` 0.5)
                (`ActorComponent.K2_DestroyComponent` _returnvalue_3)
                (`/Game/SplinterCellMain/Blueprints_Main/IlluminationDetection/Blueprints/IlluminationVolumes/BP_IlluminationVolumeMaster.SetLightStatus` (`self.Illumination Sphere Volume Ref`) "NewEnumerator1")
                ;[1 0.283 0] Report noise for AI to investigate
                (`AISense_Hearing.ReportNoiseEvent` (`self.K2_GetActorLocation`) 1.0 self 1000.0 "Shoot")
                (`KismetSystemLibrary.Delay` 5.0)
                (`self.SetActorTickEnabled` false))))))
      (:`then_1`
        (`PrimitiveComponent.AddRadialForce` _rect_lamp_glass_sm_dm _returnvalue_2 (`KismetMathLibrary.RandomFloatInRange` 0.5 1.5) (`KismetMathLibrary.RandomFloatInRange` 0.5 5.0) "RIF_Constant" false)
        (`DestructibleComponent.ApplyDamage` _rect_lamp_glass_sm_dm 10000.0 _returnvalue_2 (0.0 0.0 -1.0) 100.0)
        (`SceneComponent.SetVisibility` (`self.Rect_Lamp_Glass_SM_DM`) true false)))))

(event `/Game/AdvancedLocomotionV4/Blueprints/Interfaces/Interactive_Objects_Interface.Hit By Bullet`
  (params (`Hit Info` :type "/Game/AdvancedLocomotionV4/Data/Structs/Weapon-HitActorInfo Structure") (From :type "Character Object Reference"))
  ;[0 0 0] Lights out when hit by bullet
  (goto _label))

(fn `Get Interaction Type`
  (returns (Type :type "/Game/AdvancedLocomotionV4/Data/Enums/Interaction_Type Enum"))
  (return "NewEnumerator0"))

(fn `Get Manual Velocity`
  (returns (Velocity :type "Vector Structure"))
  (return (0.0 0.0 0.0)))

(fn `UserConstructionScript`
  (`LightComponent.SetIntensity` (`self.TubeLight`) (`self.New Intensity`))
  (`LocalLightComponent.SetAttenuationRadius` (`self.TubeLight`) (`self.Attenuation Radius`)))