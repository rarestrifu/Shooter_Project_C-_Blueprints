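; BP_LightActor_06 is a scanning spotlight that a linked button can switch off and that can optionally be destroyed.
; With UseButton set, Tick follows the button through DoOnceBranch, toggling light, emissive, sound and scan timeline.
; While unpressed, the timeline sweeps yaw between mirrored limits, smoothed by RInterpTo; without UseButton or a valid button, Tick is disabled.
; Bullet or radial damage plays a glass smash, timeline-driven flicker and sparks, then shuts it down.
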(event `self.ReceiveTick`
  (params (DeltaSeconds :type "Float (single-precision)"))
  (bind _light_mesh (`self.Light_Mesh`))
  (bind _spotlight_pitch (`self.Spotlight Pitch`))
  (bind _spotlight_max_yaw (`self.Spotlight Max Yaw`))
  (bind _sound (`self.Sound`))
  (bind _light_spotlight_0 (`self.light_spotlight_0`))
  (bind _spotlight (`self.SpotLight`))
  ;[0 0 0] On TICK = Cheap
  (`|ExecutionSequence`
    (:`then_0`
      (`/Game/AdvancedLocomotionV4/Blueprints/Libraries/ALS_MacroLibrary.DoOnce Branch` (`/Game/Game/Blueprints/BP_I_Button.Is Pressed` (`self.Button Actor`))
        (:`True`
          (`SceneComponent.SetVisibility` _spotlight false false)
          (`MeshComponent.SetScalarParameterValueOnMaterials` _light_spotlight_0 "Emissive Value" 0.0)
          (`AudioComponent.Stop` _sound)
          (bind (_direction _scan_rotation) (`Timeline|Timeline_1` :!via `Stop` :!label _label)) ; Camera animation of yaw rotation
        )
        (:`False`
          (`SceneComponent.SetVisibility` _spotlight true false)
          (`MeshComponent.SetScalarParameterValueOnMaterials` _light_spotlight_0 "Emissive Value" 10.0)
          (`AudioComponent.Play` _sound 0.0)
          (goto _label :!via `PlayFromStart`))))
    (:`then_1`
      (if (not (`/Game/Game/Blueprints/BP_I_Button.Is Pressed` (`self.Button Actor`)))
        (`SceneComponent.K2_SetRelativeRotation` _light_mesh (`KismetMathLibrary.RInterpTo` (`SceneComponent.RelativeRotation` _light_mesh) (`KismetMathLibrary.RLerp` (`KismetMathLibrary.MakeRotator` 0.0 _spotlight_pitch _spotlight_max_yaw) (`KismetMathLibrary.MakeRotator` 0.0 _spotlight_pitch (* _spotlight_max_yaw -1.0)) _scan_rotation) DeltaSeconds 0.3) false false)))))

(event `self.ReceiveBeginPlay`
  ;[0 0 0] Check for buttons
  (if (`self.Use Button?`)
    (`|ExecutionSequence`
      (:`then_0`
        (set `self.bCanBeDamaged` (`self.Is Destructable?`))
        (`/Engine/EditorBlueprintResources/StandardMacros.IsValid` (`self.Button Actor`)
          (:`Is Not Valid`
            (`self.SetActorTickEnabled` false)
            (`LightComponent.SetIntensity` (`self.SpotLight`) (`self.New Intensity`))
            (`AudioComponent.SetVolumeMultiplier` (`self.Sound`) (`self.Volume`)))))
      (:`then_1`
        (goto _label :!via `PlayFromStart`)))
    (else
      (`self.SetActorTickEnabled` false))))

(event `self.ReceiveRadialDamage`
  (params (DamageReceived :type "Float (single-precision)") (DamageType :type "DamageType Object Reference") (Origin :type "Vector Structure") (HitInfo :type "HitResult Structure (by ref)") (InstigatedBy :type "Controller Object Reference") (DamageCauser :type "Actor Object Reference"))
  (bind _returnvalue (`self.K2_GetActorLocation` self))
  ;[0 0 0] Lights out when hit by bullet
  (if (and (`self.Is Destructable?`) (not (`self.IsDead?`))) :!label _label_2
    (set `self.IsDead?` true)
    (`/Engine/EditorBlueprintResources/StandardMacros.DoOnce` false
      (:`Completed`
        (bind _returnvalue_2 (`GameplayStatics.SpawnSoundAtLocation` "/Game/SplinterCellMain/Audio/Glass_Breaking/GLASS-SMASH_GEN-HDF-12972.GLASS-SMASH_GEN-HDF-12972" _returnvalue (struct) 2.0 1.0 0.0 null null))
        (bind (_direction _intensity_of_light) (`Timeline|Timeline_0`)
          (:`Update`
            (`LightComponent.SetIntensity` (`self.SpotLight`) (* _intensity_of_light 2000.0))
            (`MeshComponent.SetScalarParameterValueOnMaterials` (`self.light_spotlight_0`) "Emissive Value" _intensity_of_light))
          (:`Finished`
            (`SceneComponent.SetVisibility` (`self.SpotLight`) false false)
            (`ActorComponent.K2_DestroyComponent` _returnvalue_2)
            (bind _returnvalue_3 (`GameplayStatics.SpawnEmitterAtLocation` "/Game/SplinterCellMain/Particle_Effects/P_Sparks.P_Sparks" _returnvalue))
            (`AudioComponent.Stop` (`self.Sound`))
            (`MeshComponent.SetScalarParameterValueOnMaterials` (`self.light_spotlight_0`) "Emissive Value" 0.0)
            (`KismetSystemLibrary.Delay` 0.5)
            (`ActorComponent.K2_DestroyComponent` _returnvalue_3)
            (`self.SetActorTickEnabled` false)))))))

(event `/Game/AdvancedLocomotionV4/Blueprints/Interfaces/Interactive_Objects_Interface.Hit By Bullet`
  (params (`Hit Info` :type "/Game/AdvancedLocomotionV4/Data/Structs/Weapon-HitActorInfo Structure") (From :type "Character Object Reference"))
  ;[0 0 0] Lights out when hit by bullet
  (goto _label_2))

(fn `Get Interaction Type`
  (returns (Type :type "/Game/AdvancedLocomotionV4/Data/Enums/Interaction_Type Enum"))
  (return "NewEnumerator0"))

(fn `Get Manual Velocity`
  (returns (Velocity :type "Vector Structure"))
  (return (0.0 0.0 0.0)))

(fn `UserConstructionScript`
  (bind _light_spotlight_0 (`self.light_spotlight_0`))
  (`LightComponent.SetIntensity` (`self.SpotLight`) (`self.New Intensity`))
  ;[1 1 1] Set pitch and yaw constraints for Spotlight
  (`SceneComponent.K2_SetRelativeRotation` _light_spotlight_0 (`KismetMathLibrary.MakeRotator` 0.0 (`self.Spotlight Pitch`)) false false)
  (set `self.Default Rotation` (`SceneComponent.K2_GetComponentRotation` _light_spotlight_0)) ; This is storing the starting rotation so we can clamp it later
)