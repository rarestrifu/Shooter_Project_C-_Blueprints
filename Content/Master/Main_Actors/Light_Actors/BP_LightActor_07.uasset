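; BP_LightActor_07 is a spotlight fixture with sound that can be switched by a linked button and optionally destroyed.
; Tick polls the button to toggle light, material, sound and a child illumination volume, whose radius matches the light's attenuation.
; Bullet hits on HitPoint or radial damage trigger timeline-driven random flicker, sparks and shattering glass via a destructible mesh.
; ShotWithBullet darkens the volume, reports noise for AI and later disables Tick.
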(event `self.ReceiveBeginPlay`
  (bind _illumination_sphere_volume_ref (`self.Illumination Sphere Volume Ref`))
  (bind _attenuation_radius (`self.Attenuation Radius`))
  ;[1 1 1] Begin Play
  (`|ExecutionSequence`
    (:`then_0`
      ;;[0 0 0] Set the world location for reference
      (set `self.World Location` (`SceneComponent.K2_GetComponentLocation` (`self.Arrow`))))
    (:`then_1`
      ;;[0 0 0] Set associated actor as can be damaged or not
      (set `self.bCanBeDamaged` (`self.Is Destructable?`)))
    (:`then_2`
      ;;[0 0 0] Check for buttons
      (`/Engine/EditorBlueprintResources/StandardMacros.IsValid` (`self.Button Actor`)
        (:`Is Valid`
          (`LightComponent.SetIntensity` (`self.SpotLight`) (`self.New Intensity`))
          (`AudioComponent.SetVolumeMultiplier` (`self.Sound`) (`self.Sound Volume`)))
        (:`Is Not Valid`
          (set `self.Use Button?` false))))
    (:`then_3`
      ;;[0 0 0] Set reference to illumination volume child actor
      (bind _asbp_illumination_sphere_volume (cast `/Game/SplinterCellMain/Blueprints_Main/IlluminationDetection/Blueprints/IlluminationVolumes/BP_IlluminationSphereVolume` (`ChildActorComponent.ChildActor` (`self.BP_IlluminationSphereVolume`))))
      (set `self.Illumination Sphere Volume Ref` _asbp_illumination_sphere_volume))
    (:`then_4`
      ;;[0 0 0] Set matching attenuation radii
      (`LocalLightComponent.SetAttenuationRadius` (`self.SpotLight`) _attenuation_radius)
      (bind _output_get (set `/Game/SplinterCellMain/Blueprints_Main/IlluminationDetection/Blueprints/IlluminationVolumes/BP_IlluminationVolumeMaster.AttenuationDistance` _attenuation_radius _illumination_sphere_volume_ref))
      (set `/Game/SplinterCellMain/Blueprints_Main/IlluminationDetection/Blueprints/IlluminationVolumes/BP_IlluminationVolumeMaster.VolumeSphereExtent` _output_get _illumination_sphere_volume_ref))))

(event `self.ReceiveTick`
  (params (DeltaSeconds :type "Float (single-precision)"))
  (bind _illumination_sphere_volume_ref (`self.Illumination Sphere Volume Ref`))
  (bind _light_mesh (`self.Light_Mesh`))
  (bind _sound (`self.Sound`))
  (bind _spotlight (`self.SpotLight`))
  ;[0 0 0] On TICK = Cheap
  (if (`self.Use Button?`)
    (`/Game/AdvancedLocomotionV4/Blueprints/Libraries/ALS_MacroLibrary.DoOnce Branch` (`/Game/Game/Blueprints/BP_I_Button.Is Pressed` (`self.Button Actor`))
      (:`True`
        (`SceneComponent.SetVisibility` _spotlight false false)
        (`MeshComponent.SetScalarParameterValueOnMaterials` _light_mesh "Use_Illum" 1.0)
        (`AudioComponent.Stop` _sound)
        (`/Game/SplinterCellMain/Blueprints_Main/IlluminationDetection/Blueprints/IlluminationVolumes/BP_IlluminationVolumeMaster.SetLightStatus` _illumination_sphere_volume_ref "NewEnumerator1"))
      (:`False`
        (`SceneComponent.SetVisibility` _spotlight true false)
        (`MeshComponent.SetScalarParameterValueOnMaterials` _light_mesh "Use_Illum" 0.0)
        (`AudioComponent.Play` _sound 0.0)
        (`/Game/SplinterCellMain/Blueprints_Main/IlluminationDetection/Blueprints/IlluminationVolumes/BP_IlluminationVolumeMaster.SetLightStatus` _illumination_sphere_volume_ref "NewEnumerator0")))))

(event `self.ReceiveRadialDamage`
  (params (DamageReceived :type "Float (single-precision)") (DamageType :type "DamageType Object Reference") (Origin :type "Vector Structure") (HitInfo :type "HitResult Structure (by ref)") (InstigatedBy :type "Controller Object Reference") (DamageCauser :type "Actor Object Reference"))
  (bind _bulb_lamp_glass_sm_dm (`self.Bulb_Lamp_Glass_SM_DM`))
  (bind _bulb_lamp_glass_sm_dm_2 (`self.Bulb_Lamp_Glass_SM_DM`))
  (bind _returnvalue (`SceneComponent.K2_GetComponentLocation` (`self.SpotLight`)))
  (bind _returnvalue_2 (`SceneComponent.K2_GetComponentLocation` (`self.Arrow`)))
  ;[0 0 0] Lights out when hit by bullet
  (if (and (`self.Is Destructable?`) (not (`self.IsDead?`))) :!label _label
    (`|ExecutionSequence`
      (:`then_0`
        (set `self.IsDead?` true)
        (`/Engine/EditorBlueprintResources/StandardMacros.DoOnce` false
          (:`Completed`
            (bind _returnvalue_3 (`GameplayStatics.SpawnSoundAtLocation` "/Game/SplinterCellMain/Audio/Glass_Breaking/GLASS-SMASH_GEN-HDF-12972.GLASS-SMASH_GEN-HDF-12972" _returnvalue_2 (struct) 2.0 1.0 0.0 null null))
            (bind (_direction _intensity_of_light) (`Timeline|Timeline_0`)
              (:`Update`
                (`LightComponent.SetIntensity` (`self.SpotLight`) (* _intensity_of_light (`KismetMathLibrary.RandomFloatInRange` 1800.0 20000.0)))
                (`MeshComponent.SetScalarParameterValueOnMaterials` (`self.Light_Mesh`) "Illum_Intensity" _intensity_of_light))
              (:`Finished`
                (`SceneComponent.SetVisibility` (`self.SpotLight`) false false)
                (`ActorComponent.K2_DestroyComponent` _returnvalue_3)
                (bind _returnvalue_4 (`GameplayStatics.SpawnEmitterAtLocation` "/Game/SplinterCellMain/Particle_Effects/P_Sparks.P_Sparks" _returnvalue_2))
                (`AudioComponent.Stop` (`self.Sound`))
                (`MeshComponent.SetScalarParameterValueOnMaterials` (`self.Light_Mesh`) "Use_Illum" 0.0)
                (`KismetSystemLibrary.Delay` 0.5)
                (`ActorComponent.K2_DestroyComponent` _returnvalue_4)
                (`/Game/SplinterCellMain/Blueprints_Main/IlluminationDetection/Blueprints/IlluminationVolumes/BP_IlluminationVolumeMaster.SetLightStatus` (`self.Illumination Sphere Volume Ref`) "NewEnumerator1")
                ;[1 0.283 0] Report noise for AI to investigate
                (`AISense_Hearing.ReportNoiseEvent` (- (`self.World Location`) (0.0 0.0 800.0)) 1.0 self 1200.0 "Shoot")
                (`KismetSystemLibrary.Delay` 1.0)
                (`self.SetActorTickEnabled` false))))))
      (:`then_1`
        (`PrimitiveComponent.AddRadialForce` _bulb_lamp_glass_sm_dm _returnvalue (`KismetMathLibrary.RandomFloatInRange` 0.1 1.0) (`KismetMathLibrary.RandomFloatInRange` 0.1 2.0) "RIF_Constant" false)
        (`DestructibleComponent.ApplyDamage` _bulb_lamp_glass_sm_dm 10000.0 _returnvalue (0.0 0.0 -1.0) 100.0)
        (`SceneComponent.SetVisibility` _bulb_lamp_glass_sm_dm_2 true false)
        (`PrimitiveComponent.SetCollisionResponseToChannel` _bulb_lamp_glass_sm_dm_2 "ECC_Pawn" "ECR_Ignore")))))

(event `/Game/AdvancedLocomotionV4/Blueprints/Interfaces/Interactive_Objects_Interface.Hit By Bullet`
  (params (`Hit Info` :type "/Game/AdvancedLocomotionV4/Data/Structs/Weapon-HitActorInfo Structure") (From :type "Character Object Reference"))
  ;[0 0 0] Lights out when hit by bullet
  (if (== `Hit Info_Component_21_DE9817A14F727A6D24C38BA42C11B98D` (`self.Hit Point`))
    (goto _label)))

(fn `Get Interaction Type`
  (returns (Type :type "/Game/AdvancedLocomotionV4/Data/Enums/Interaction_Type Enum"))
  (return "NewEnumerator0"))

(fn `Get Manual Velocity`
  (returns (Velocity :type "Vector Structure"))
  (return (0.0 0.0 0.0)))

(fn `UserConstructionScript`
  (`LightComponent.SetIntensity` (`self.SpotLight`) (`self.New Intensity`))
  (`LocalLightComponent.SetAttenuationRadius` (`self.SpotLight`) (`self.Attenuation Radius`)))