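; BP_LightActor_02 is a light fixture with looping-capable sound that can be switched by a linked button or destroyed by bullets and radial damage.
; It syncs radius and on/off status to a child BP_IlluminationSphereVolume.
; Tick polls the button, toggling light, emissive and sound, and reporting AI noise when switched off.
; Destruction, if enabled, plays glass smash, Niagara sparks and a timeline flicker; ShotWithBullet also reports noise and disables Tick.
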(event `self.ReceiveBeginPlay`
  (bind _attenuation_radius (`self.Attenuation Radius`))
  ;[1 1 1] Begin Play
  (`|ExecutionSequence`
    (:`then_0`
      ;;[0 0 0] Set the world location for reference
      (set `self.World Location` (`SceneComponent.K2_GetComponentLocation` (`self.Light_Mesh`))))
    (:`then_1`
      ;;[0 0 0] Set associated actor as can be damaged or not
      (set `self.bCanBeDamaged` (`self.Is Destructable?`)))
    (:`then_2`
      ;;[0 0 0] Check for buttons
      (`/Engine/EditorBlueprintResources/StandardMacros.IsValid` (`self.Button Actor`)
        (:`Is Not Valid`
          (set `self.Use Button?` false)
          (`self.SetActorTickEnabled` false))))
    (:`then_3`
      ;;[0 0 0] Set reference to illumination volume child actor
      (bind _asbp_illumination_sphere_volume (cast `/Game/SplinterCellMain/Blueprints_Main/IlluminationDetection/Blueprints/IlluminationVolumes/BP_IlluminationSphereVolume` (`ChildActorComponent.ChildActor` (`self.BP_IlluminationSphereVolume`))))
      (set `self.Illumination Sphere Volume Ref` _asbp_illumination_sphere_volume))
    (:`then_4`
      ;;[0 0 0] Set matching attenuation radii
      (`LocalLightComponent.SetAttenuationRadius` (`self.PointLight`) _attenuation_radius)
      (set `/Game/SplinterCellMain/Blueprints_Main/IlluminationDetection/Blueprints/IlluminationVolumes/BP_IlluminationVolumeMaster.AttenuationDistance` _attenuation_radius (`self.Illumination Sphere Volume Ref`)))
    (:`then_5`
      ;;[0 0 0] Set parameters
      (`LightComponent.SetIntensity` (`self.PointLight`) (`self.New Intensity`))
      (`AudioComponent.SetVolumeMultiplier` (`self.Sound`) (`self.Sound Volume`)))))

(event `self.ReceiveTick`
  (params (DeltaSeconds :type "Float (single-precision)"))
  (bind _button_actor (`self.Button Actor`))
  (bind _button_actor_2 (`self.Button Actor`))
  (bind _illumination_sphere_volume_ref (`self.Illumination Sphere Volume Ref`))
  (bind _sound (`self.Sound`))
  (bind _pointlight (`self.PointLight`))
  (bind _light_mesh (`self.Light_Mesh`))
  ;[0 0 0] On TICK = Cheap
  (`/Engine/EditorBlueprintResources/StandardMacros.IsValid` _button_actor
    (:`Is Valid`
      (`/Game/AdvancedLocomotionV4/Blueprints/Libraries/ALS_MacroLibrary.DoOnce Branch` (`/Game/Game/Blueprints/BP_I_Button.Is Pressed` _button_actor)
        (:`True`
          (`SceneComponent.SetVisibility` _pointlight false false)
          (`MeshComponent.SetScalarParameterValueOnMaterials` _light_mesh "Emissive Value" 0.0)
          (`AudioComponent.Stop` _sound)
          (`/Game/SplinterCellMain/Blueprints_Main/IlluminationDetection/Blueprints/IlluminationVolumes/BP_IlluminationVolumeMaster.SetLightStatus` _illumination_sphere_volume_ref "NewEnumerator1")
          ;[1 0.283 0] Report noise for AI to investigate
          (`AISense_Hearing.ReportNoiseEvent` (`/Game/Game/Blueprints/BP_I_Button.Sound Location` _button_actor_2) 1.0 _button_actor_2 1000.0 "Shoot"))
        (:`False`
          (`SceneComponent.SetVisibility` _pointlight true false)
          (`MeshComponent.SetScalarParameterValueOnMaterials` _light_mesh "Emissive Value" 15.0)
          (`AudioComponent.Play` _sound 0.0)
          (`/Game/SplinterCellMain/Blueprints_Main/IlluminationDetection/Blueprints/IlluminationVolumes/BP_IlluminationVolumeMaster.SetLightStatus` _illumination_sphere_volume_ref "NewEnumerator0"))))))

(event `self.ReceiveRadialDamage`
  (params (DamageReceived :type "Float (single-precision)") (DamageType :type "DamageType Object Reference") (Origin :type "Vector Structure") (HitInfo :type "HitResult Structure (by ref)") (InstigatedBy :type "Controller Object Reference") (DamageCauser :type "Actor Object Reference"))
  ;[0 0 0] Lights out when hit by bullet
  (if (and (`self.Is Destructable?`) (not (`self.IsDead?`))) :!label _label
    (set `self.IsDead?` true)
    (`/Engine/EditorBlueprintResources/StandardMacros.DoOnce` false
      (:`Completed`
        (`GameplayStatics.SpawnSoundAtLocation` "/Game/SplinterCellMain/Audio/Glass_Breaking/GLASS-SMASH_GEN-HDF-12972.GLASS-SMASH_GEN-HDF-12972" (`self.World Location`) (struct) 1.0 1.0 0.0 null null)
        (bind _returnvalue (`NiagaraFunctionLibrary.SpawnSystemAtLocation` (`self.Niagara Sparks`) (`SceneComponent.K2_GetComponentLocation` (`self.Arrow`))))
        (bind (_direction _intensity_of_light) (`Timeline|Timeline_0`)
          (:`Update`
            (`LightComponent.SetIntensity` (`self.PointLight`) (* _intensity_of_light (`LightComponentBase.Intensity` (`self.PointLight`))))
            (`MeshComponent.SetScalarParameterValueOnMaterials` (`self.Light_Mesh`) "Emissive Value" _intensity_of_light))
          (:`Finished`
            (`SceneComponent.SetVisibility` (`self.PointLight`) false false)
            (`/Engine/EditorBlueprintResources/StandardMacros.IsValid` _returnvalue
              (:`Is Valid`
                (`ActorComponent.K2_DestroyComponent` _returnvalue))
              (:`Is Not Valid`
                _))
            (`AudioComponent.Stop` (`self.Sound`))
            (`MeshComponent.SetScalarParameterValueOnMaterials` (`self.Light_Mesh`) "Emissive Value" 0.0)
            (`KismetSystemLibrary.Delay` 0.5)
            (`/Game/SplinterCellMain/Blueprints_Main/IlluminationDetection/Blueprints/IlluminationVolumes/BP_IlluminationVolumeMaster.SetLightStatus` (`self.Illumination Sphere Volume Ref`) "NewEnumerator1")
            ;[1 0.283 0] Report noise for AI to investigate
            (`AISense_Hearing.ReportNoiseEvent` (`self.World Location`) 1.0 self 1200.0 "Shoot")
            (`KismetSystemLibrary.Delay` 0.5)
            (`self.SetActorTickEnabled` false)))))))

(event `/Game/AdvancedLocomotionV4/Blueprints/Interfaces/Interactive_Objects_Interface.Hit By Bullet`
  (params (`Hit Info` :type "/Game/AdvancedLocomotionV4/Data/Structs/Weapon-HitActorInfo Structure") (From :type "Character Object Reference"))
  ;[0 0 0] Lights out when hit by bullet
  (goto _label))

(fn `Get Interaction Type`
  (returns (Type :type "/Game/AdvancedLocomotionV4/Data/Enums/Interaction_Type Enum"))
  (return "NewEnumerator0"))

(fn `Get Manual Velocity`
  (returns (Velocity :type "Vector Structure"))
  (return (0.0 0.0 0.0)))

(fn `UserConstructionScript`
  (`LightComponent.SetIntensity` (`self.PointLight`) (`self.New Intensity`))
  (`LocalLightComponent.SetAttenuationRadius` (`self.PointLight`) (`self.Attenuation Radius`)))