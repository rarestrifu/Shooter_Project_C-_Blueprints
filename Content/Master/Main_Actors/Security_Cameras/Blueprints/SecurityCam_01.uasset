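; SecurityCam_01 is a security camera actor that reacts to being shot.
; Its HitbyBullet event calls the parent handler, then a DoOnce toggles the PointLight's visibility and sets CameraPitch to a downward angle.
; The DoOnce is never reset, so only the first hit triggers this change.
; BeginPlay and Tick are disabled stubs, and the construction script only calls its parent.
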(event `/Game/AdvancedLocomotionV4/Blueprints/Interfaces/Interactive_Objects_Interface.Hit By Bullet`
  (params (`Hit Info` :type "/Game/AdvancedLocomotionV4/Data/Structs/Weapon-HitActorInfo Structure") (From :type "Character Object Reference"))
  (`parent.Hit By Bullet` `Hit Info` From)
  (`/Engine/EditorBlueprintResources/StandardMacros.DoOnce` false
    (:`Completed`
      (`SceneComponent.ToggleVisibility` (`self.PointLight`) false)
      (set `self.Camera Pitch` -60.0))))

(fn `UserConstructionScript`
  (`parent.UserConstructionScript`))