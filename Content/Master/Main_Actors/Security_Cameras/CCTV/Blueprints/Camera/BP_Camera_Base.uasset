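; Base security camera actor for the CCTV system, which can track an actor and be broken by damage.
; The construction script and Tick rotate the camera mesh to look at FollowActor, and both disable tick when that actor is not valid.
; When BreakWhenDamaged is set, any damage marks the camera broken and tells every BP_Monitor_Base in the level to update.
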(event `self.ReceiveTick`
  (params (DeltaSeconds :type "Float (single-precision)"))
  ;[0 0 0] Rotate camera towards actor or disable tick if not needed
  (`/Engine/EditorBlueprintResources/StandardMacros.IsValid` (`self.Follow actor`)
    (:`Is Valid`
      (`self.Rotate camera towards actor`))
    (:`Is Not Valid`
      (`self.SetActorTickEnabled` false))))

(event `self.ReceiveAnyDamage`
  (params (Damage :type "Float (single-precision)") (DamageType :type "DamageType Object Reference") (InstigatedBy :type "Controller Object Reference") (DamageCauser :type "Actor Object Reference"))
  ;[0 0 0] Camera damage
  (if (`self.Break when damaged?`)
    (set `self.Camera broken?` true)
    ;[0 0 0] Update all monitors
    (bind _outactors (`GameplayStatics.GetAllActorsOfClass` "/Game/SplinterCellMain/Blueprints_Main/Security_Cameras/CCTV/Blueprints/Screen/BP_Monitor_Base.BP_Monitor_Base_C"))
    (for _array_element _outactors
      (`/Game/SplinterCellMain/Blueprints_Main/Security_Cameras/CCTV/Blueprints/Screen/BP_Monitor_Base.Update monitor` _array_element))))

(fn `Rotate camera towards actor`
  (`SceneComponent.K2_SetWorldRotation` (`self.Camera Mesh`) (`KismetMathLibrary.FindLookAtRotation` (`SceneComponent.K2_GetComponentLocation` (`self.Camera Mesh`)) (`self.K2_GetActorLocation` (`self.Follow actor`))) false false))

(fn `UserConstructionScript`
  ;[0 0 0] Rotate camera towards actor or disable tick if not needed
  (`/Engine/EditorBlueprintResources/StandardMacros.IsValid` (`self.Follow actor`)
    (:`Is Valid`
      (`self.Rotate camera towards actor`))
    (:`Is Not Valid`
      (`self.SetActorTickEnabled` false))))