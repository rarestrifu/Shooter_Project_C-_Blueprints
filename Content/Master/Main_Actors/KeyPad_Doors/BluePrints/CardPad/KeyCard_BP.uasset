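; KeyCard_BP is a rotating key card pickup for the keypad door system, with its material set in the construction script.
; On first overlap by ALS_MainCharacter, it finds every PadData_BP actor and adds its CardName to StoredUnlocks so other Blueprints can see the pickup.
; The pickup sound and DestroyActor run inside that loop, so they depend on a PadData_BP existing in the level.
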(event `self.ReceiveTick`
  (params (DeltaSeconds :type "Float (single-precision)"))
  ;[1 1 1] RotateCard
  (`SceneComponent.K2_AddRelativeRotation` (`self.Card`) (struct :`Yaw` 1.0) false false))

(event `self.PickUpCollison.OnComponentBeginOverlap`
  (params (OverlappedComponent :type "PrimitiveComponent Object Reference") (OtherActor :type "Actor Object Reference") (OtherComp :type "PrimitiveComponent Object Reference") (OtherBodyIndex :type Integer) (bFromSweep :type Boolean) (SweepResult :type "HitResult Structure (by ref)"))
  (cast `/Game/SplinterCellMain/Blueprints_Main/ALS_MainCharacter` OtherActor)
  ;[1 1 1] Add Card Name to Array om KeyCardData Blueprint so other BP can see the card is picked Up
  (`/Engine/EditorBlueprintResources/StandardMacros.DoOnce` false
    (:`Completed`
      (bind _outactors (`GameplayStatics.GetAllActorsOfClass` "/Game/SplinterCellMain/Blueprints_Main/KeyPad_Doors/BluePrints/PadData_BP.PadData_BP_C"))
      (for _array_element _outactors
        (bind _storedunlocks (`/Game/SplinterCellMain/Blueprints_Main/KeyPad_Doors/BluePrints/PadData_BP.StoredUnlocks` _array_element))
        (`KismetArrayLibrary.Array_AddUnique` _storedunlocks (`self.CardName`))
        (set `/Game/SplinterCellMain/Blueprints_Main/KeyPad_Doors/BluePrints/PadData_BP.StoredUnlocks` _storedunlocks _array_element)
        (`GameplayStatics.PlaySound2D` "/Game/SplinterCellMain/Blueprints_Main/KeyPad_Doors/Audio/PickUp_Cue.PickUp_Cue" 1.0 1.0 0.0 null null)
        (`self.K2_DestroyActor`)))))

(fn `UserConstructionScript`
  (`PrimitiveComponent.SetMaterial` (`self.Card`) 0 (`self.CardMaterial`)))