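; Keypad lock actor that lets the player enter a four-digit code by mouse or keyboard to trigger linked Blueprints.
; Pressing F in range blends the view to the keypad and shows the cursor; Q leaves.
; Cursor hits and number keys set a HitButton for the KeyEvents macro, which animates keys and builds PassCode.
; A correct code adds BlueprintName to PadData_BP's StoredUnlocks; a wrong one briefly shows Denied.
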(event `self.CheckCollision.OnComponentBeginOverlap`
  (params (OverlappedComponent :type "PrimitiveComponent Object Reference") (OtherActor :type "Actor Object Reference") (OtherComp :type "PrimitiveComponent Object Reference") (OtherBodyIndex :type Integer) (bFromSweep :type Boolean) (SweepResult :type "HitResult Structure (by ref)"))
  ;[1 1 1] UnlockActivation Button
  (set `self.MayUse` true))

(event `SetKeyPadUnlocked`
  ;[1 1 1] Check if KeyPad is already unlocked
  (`SceneComponent.SetVisibility` (`self.*_2`) false false :!label _label)
  (`SceneComponent.SetVisibility` (`self.*_3`) false false)
  (`SceneComponent.SetVisibility` (`self.*_4`) false false)
  (`SceneComponent.SetVisibility` (`self.*_1`) false false)
  (`SceneComponent.SetVisibility` (`self.AccessText`) true false))

(event `self.ReceiveBeginPlay`
  ;[1 1 1] EnableInput
  (`self.EnableInput` (`GameplayStatics.GetPlayerController` 0))
  ;[1 1 1] Check if KeyPad is already unlocked
  (if (`self.Unlocked`)
    (goto _label)))

(event `self.CheckCollision.OnComponentEndOverlap`
  (params (OverlappedComponent :type "PrimitiveComponent Object Reference") (OtherActor :type "Actor Object Reference") (OtherComp :type "PrimitiveComponent Object Reference") (OtherBodyIndex :type Integer))
  ;[1 1 1] UnlockActivation Button
  (set `self.MayUse` false))

(event `Key|F` :consume false
  (params (Key :type "Key Structure"))
  (bind _returnvalue (`GameplayStatics.GetPlayerController` 0))
  ;[1 1 1] Activate by clicking 'F'
  ;;[1 0.255 0.255] InputKey
  (:`Pressed`
    (if (not (`self.Unlocked`))
      (set `self.MayLeaveLock` true)
      (if (`self.MayUse`)
        (`PlayerController.SetViewTargetWithBlend` _returnvalue self 0.0 "VTBlend_Linear" 0.0 true)
        (set `PlayerController.bShowMouseCursor` true _returnvalue)))))

(event `Key|Q` :consume false
  (params (Key :type "Key Structure"))
  (bind _returnvalue (`GameplayStatics.GetPlayerController` 0))
  ;[1 1 1] Leave by clicking 'Q'
  ;;[1 0.255 0.255] InputKey
  (:`Pressed`
    (if (`self.MayLeaveLock`) :!label _label_2
      (`PlayerController.SetViewTargetWithBlend` _returnvalue (`Controller.K2_GetPawn` _returnvalue) 0.0 "VTBlend_Linear" 0.0 false)
      (set `PlayerController.bShowMouseCursor` false _returnvalue)
      (set `self.MayLeaveLock` false))))

(event `DeactivateKeypad`
  ;[1 1 1] Leave by clicking 'Q'
  (goto _label_2))

(event `Key|F` :consume false
  (params (Key :type "Key Structure"))
  ;[1 0.255 0.255] InputKey
  (:`Pressed`
    ;[1 1 1] Enter Button clicks By 'F' key
    (if (`self.MayEnterCode`)
      (set `self.HitButton` (`.HitComponent` (`GameplayStatics.BreakHitResult` (`PlayerController.GetHitResultUnderCursorByChannel` (`GameplayStatics.GetPlayerController` 0) "TraceTypeQuery1" true))))
      ;[1 1 1] Apply Entry by Buttons Events
      (`|ExecutionSequence`
        (:`then_0`
          (`self.KeyEvents` (`self.Key_1`) "1" true (`self.1_Text`) :!label _label_3))
        (:`then_1`
          (`self.KeyEvents` (`self.Key_2`) "2" true (`self.2_Text`) :!label _label_4))
        (:`then_2`
          (`self.KeyEvents` (`self.Key_3`) "3" true (`self.3_Text`) :!label _label_5))
        (:`then_3`
          (`self.KeyEvents` (`self.Key_4`) "4" true (`self.4_Text`) :!label _label_6))
        (:`then_4`
          (`self.KeyEvents` (`self.Key_5`) "5" true (`self.5_Text`) :!label _label_7))
        (:`then_5`
          (`self.KeyEvents` (`self.Key_6`) "6" true (`self.6_Text`) :!label _label_8))
        (:`then_6`
          (`self.KeyEvents` (`self.Key_7`) "7" true (`self.7_Text`) :!label _label_9))
        (:`then_7`
          (`self.KeyEvents` (`self.Key_8`) "8" true (`self.8_Text`) :!label _label_10))
        (:`then_8`
          (`self.KeyEvents` (`self.Key_9`) "9" true (`self.9_Text`) :!label _label_11))
        (:`then_9`
          (`self.KeyEvents` (`self.Key_0`) "0" true (`self.0_Text`) :!label _label_12))
        (:`then_10`
          (`self.KeyEvents` (`self.Key_Correction`) "" false (`self.Correction_Text`) :!label _label_13
            (:`Out`
              (`self.ResetCode`))))
        (:`then_11`
          (`self.KeyEvents` (`self.Key_Accept`) "" false (`self.Enter_Text`) :!label _label_14
            (:`Out`
              (`self.AcceptCode`))))))))

(event `CheckLock`
  ;[1 1 1] Fill Key Entry with Button Values
  (switch `/Game/SplinterCellMain/Blueprints_Main/KeyPad_Doors/BluePrints/KeyPad/KeyEntry` (`self.KeyEntry`)
    (:`NewEnumerator0`
      (`self.KeyPadEntry` (`self.*_1`) "NewEnumerator1")
      (set `self.PassCode` (`KismetStringLibrary.Concat_StrStr` (`self.PassCode`) (`self.KeyValue`)) :!label _label_15))
    (:`NewEnumerator1`
      (`self.KeyPadEntry` (`self.*_2`) "NewEnumerator2")
      (goto _label_15))
    (:`NewEnumerator2`
      (`self.KeyPadEntry` (`self.*_3`) "NewEnumerator3")
      (goto _label_15))
    (:`NewEnumerator3`
      (`self.KeyPadEntry` (`self.*_4`) "NewEnumerator4")
      (goto _label_15))
    (:`NewEnumerator4`
      (`self.ResetKeyEntry`))))

(event `Key|One` :consume false
  (params (Key :type "Key Structure"))
  ;[1 0.39 0.39] Input By Number and Numlock Number keys
  (:`Pressed`
    (if (`self.MayEnterCode`) :!label _label_16
      (set `self.HitButton` (`self.Key_1`))
      (goto _label_3))))

(event `Key|Two` :consume false
  (params (Key :type "Key Structure"))
  ;[1 0.39 0.39] Input By Number and Numlock Number keys
  (:`Pressed`
    (if (`self.MayEnterCode`) :!label _label_17
      (set `self.HitButton` (`self.Key_2`))
      (goto _label_4))))

(event `Key|Three` :consume false
  (params (Key :type "Key Structure"))
  ;[1 0.39 0.39] Input By Number and Numlock Number keys
  (:`Pressed`
    (if (`self.MayEnterCode`) :!label _label_18
      (set `self.HitButton` (`self.Key_3`))
      (goto _label_5))))

(event `Key|Four` :consume false
  (params (Key :type "Key Structure"))
  ;[1 0.39 0.39] Input By Number and Numlock Number keys
  (:`Pressed`
    (if (`self.MayEnterCode`) :!label _label_19
      (set `self.HitButton` (`self.Key_4`))
      (goto _label_6))))

(event `Key|Five` :consume false
  (params (Key :type "Key Structure"))
  ;[1 0.39 0.39] Input By Number and Numlock Number keys
  (:`Pressed`
    (if (`self.MayEnterCode`) :!label _label_20
      (set `self.HitButton` (`self.Key_5`))
      (goto _label_7))))

(event `Key|Six` :consume false
  (params (Key :type "Key Structure"))
  ;[1 0.39 0.39] Input By Number and Numlock Number keys
  (:`Pressed`
    (if (`self.MayEnterCode`) :!label _label_21
      (set `self.HitButton` (`self.Key_6`))
      (goto _label_8))))

(event `Key|Seven` :consume false
  (params (Key :type "Key Structure"))
  ;[1 0.39 0.39] Input By Number and Numlock Number keys
  (:`Pressed`
    (if (`self.MayEnterCode`) :!label _label_22
      (set `self.HitButton` (`self.Key_7`))
      (goto _label_9))))

(event `Key|Eight` :consume false
  (params (Key :type "Key Structure"))
  ;[1 0.39 0.39] Input By Number and Numlock Number keys
  (:`Pressed`
    (if (`self.MayEnterCode`) :!label _label_23
      (set `self.HitButton` (`self.Key_8`))
      (goto _label_10))))

(event `Key|Nine` :consume false
  (params (Key :type "Key Structure"))
  ;[1 0.39 0.39] Input By Number and Numlock Number keys
  (:`Pressed`
    (if (`self.MayEnterCode`) :!label _label_24
      (set `self.HitButton` (`self.Key_9`))
      (goto _label_11))))

(event `Key|Zero` :consume false
  (params (Key :type "Key Structure"))
  ;[1 0.39 0.39] Input By Number and Numlock Number keys
  (:`Pressed`
    (if (`self.MayEnterCode`) :!label _label_25
      (set `self.HitButton` (`self.Key_0`))
      (goto _label_12))))

(event `Key|Enter` :consume false
  (params (Key :type "Key Structure"))
  ;[1 0.39 0.39] Input By Number and Numlock Number keys
  (:`Pressed`
    (if (`self.MayEnterCode`)
      (set `self.HitButton` (`self.Key_Accept`))
      (goto _label_14))))

(event `Key|C` :consume false
  (params (Key :type "Key Structure"))
  ;[1 0.39 0.39] Input By Number and Numlock Number keys
  (:`Pressed`
    (if (`self.MayEnterCode`) :!label _label_26
      (set `self.HitButton` (`self.Key_Correction`))
      (goto _label_13))))

(event `Key|NumPadOne` :consume false
  (params (Key :type "Key Structure"))
  ;[1 0.39 0.39] Input By Number and Numlock Number keys
  (:`Pressed`
    (goto _label_16)))

(event `Key|NumPadTwo` :consume false
  (params (Key :type "Key Structure"))
  ;[1 0.39 0.39] Input By Number and Numlock Number keys
  (:`Pressed`
    (goto _label_17)))

(event `Key|NumPadThree` :consume false
  (params (Key :type "Key Structure"))
  ;[1 0.39 0.39] Input By Number and Numlock Number keys
  (:`Pressed`
    (goto _label_18)))

(event `Key|NumPadFour` :consume false
  (params (Key :type "Key Structure"))
  ;[1 0.39 0.39] Input By Number and Numlock Number keys
  (:`Pressed`
    (goto _label_19)))

(event `Key|NumPadFive` :consume false
  (params (Key :type "Key Structure"))
  ;[1 0.39 0.39] Input By Number and Numlock Number keys
  (:`Pressed`
    (goto _label_20)))

(event `Key|NumPadSix` :consume false
  (params (Key :type "Key Structure"))
  ;[1 0.39 0.39] Input By Number and Numlock Number keys
  (:`Pressed`
    (goto _label_21)))

(event `Key|NumPadSeven` :consume false
  (params (Key :type "Key Structure"))
  ;[1 0.39 0.39] Input By Number and Numlock Number keys
  (:`Pressed`
    (goto _label_22)))

(event `Key|NumPadEight` :consume false
  (params (Key :type "Key Structure"))
  ;[1 0.39 0.39] Input By Number and Numlock Number keys
  (:`Pressed`
    (goto _label_23)))

(event `Key|NumPadNine` :consume false
  (params (Key :type "Key Structure"))
  ;[1 0.39 0.39] Input By Number and Numlock Number keys
  (:`Pressed`
    (goto _label_24)))

(event `Key|NumPadZero` :consume false
  (params (Key :type "Key Structure"))
  ;[1 0.39 0.39] Input By Number and Numlock Number keys
  (:`Pressed`
    (goto _label_25)))

(event `Key|Decimal` :consume false
  (params (Key :type "Key Structure"))
  ;[1 0.39 0.39] Input By Number and Numlock Number keys
  (:`Pressed`
    (goto _label_26)))

(event `Trigger keypad Linked Event`
  ;[1 0.32 0.32] Add Name of BP that must react to CardPad Event
  (bind _outactors (`GameplayStatics.GetAllActorsOfClass` "/Game/SplinterCellMain/Blueprints_Main/KeyPad_Doors/BluePrints/PadData_BP.PadData_BP_C"))
  (for _array_element _outactors
    (bind _storedunlocks (`/Game/SplinterCellMain/Blueprints_Main/KeyPad_Doors/BluePrints/PadData_BP.StoredUnlocks` _array_element))
    (`KismetArrayLibrary.Array_AddUnique` _storedunlocks (`self.BlueprintName`))
    (set `/Game/SplinterCellMain/Blueprints_Main/KeyPad_Doors/BluePrints/PadData_BP.StoredUnlocks` _storedunlocks _array_element)))

(event `AcceptCode`
  ;[1 1 1] Accept Code Button Event
  (if (`KismetStringLibrary.EqualEqual_StrStr` (`self.PassCode`) (`self.Code`))
    (set `self.Unlocked` true)
    (`GameplayStatics.PlaySound2D` "/Game/SplinterCellMain/Blueprints_Main/KeyPad_Doors/Audio/Access_Cue.Access_Cue" 1.0 1.0 0.0 null null) ; Denied Sound
    (`self.SetKeyPadUnlocked`)
    (`self.Trigger keypad Linked Event`)
    (if (`self.AutoClose`)
      (`self.DeactivateKeypad`))
    (else
      (`self.ResetKeyEntry`)
      (`self.CodeDenied` (`self.Denied Delay`)))))

(event `ResetCode`
  ;[1 1 1] Reset Code Button Event
  (`self.ResetKeyEntry`))

(fn `KeyPadEntry`
  (params (KeyPadNumber :type "TextRenderComponent Object Reference") (KeyEntry :type "/Game/SplinterCellMain/Blueprints_Main/KeyPad_Doors/BluePrints/KeyPad/KeyEntry Enum" :default "NewEnumerator0"))
  ;[1 1 1] Set KeyButton entry
  (`TextRenderComponent.K2_SetText` KeyPadNumber (`KismetTextLibrary.Conv_StringToText` (`self.KeyValue`)))
  (set `self.KeyEntry` KeyEntry)
  (return))

(fn `ResetKeyEntry`
  ;[1 1 1] Reset Key and key entry
  (set `self.KeyValue` "*")
  (`TextRenderComponent.K2_SetText` (`self.*_1`) (`KismetTextLibrary.Conv_StringToText` (`self.KeyValue`)))
  (`TextRenderComponent.K2_SetText` (`self.*_2`) (`KismetTextLibrary.Conv_StringToText` (`self.KeyValue`)))
  (`TextRenderComponent.K2_SetText` (`self.*_3`) (`KismetTextLibrary.Conv_StringToText` (`self.KeyValue`)))
  (`TextRenderComponent.K2_SetText` (`self.*_4`) (`KismetTextLibrary.Conv_StringToText` (`self.KeyValue`)))
  (set `self.KeyEntry` "NewEnumerator0")
  (set `self.PassCode` "")
  (return))

(fn `UserConstructionScript`
  (`TextRenderComponent.SetTextRenderColor` (`self.1_Text`) (`KismetMathLibrary.Conv_LinearColorToColor` (`self.InitialKeyTextColor`)))
  (`TextRenderComponent.SetTextRenderColor` (`self.2_Text`) (`KismetMathLibrary.Conv_LinearColorToColor` (`self.InitialKeyTextColor`)))
  (`TextRenderComponent.SetTextRenderColor` (`self.3_Text`) (`KismetMathLibrary.Conv_LinearColorToColor` (`self.InitialKeyTextColor`)))
  (`TextRenderComponent.SetTextRenderColor` (`self.4_Text`) (`KismetMathLibrary.Conv_LinearColorToColor` (`self.InitialKeyTextColor`)))
  (`TextRenderComponent.SetTextRenderColor` (`self.5_Text`) (`KismetMathLibrary.Conv_LinearColorToColor` (`self.InitialKeyTextColor`)))
  (`TextRenderComponent.SetTextRenderColor` (`self.6_Text`) (`KismetMathLibrary.Conv_LinearColorToColor` (`self.InitialKeyTextColor`)))
  (`TextRenderComponent.SetTextRenderColor` (`self.7_Text`) (`KismetMathLibrary.Conv_LinearColorToColor` (`self.InitialKeyTextColor`)))
  (`TextRenderComponent.SetTextRenderColor` (`self.8_Text`) (`KismetMathLibrary.Conv_LinearColorToColor` (`self.InitialKeyTextColor`)))
  (`TextRenderComponent.SetTextRenderColor` (`self.9_Text`) (`KismetMathLibrary.Conv_LinearColorToColor` (`self.InitialKeyTextColor`)))
  (`TextRenderComponent.SetTextRenderColor` (`self.0_Text`) (`KismetMathLibrary.Conv_LinearColorToColor` (`self.InitialKeyTextColor`)))
  (`TextRenderComponent.SetTextRenderColor` (`self.Correction_Text`) (`KismetMathLibrary.Conv_LinearColorToColor` (`self.InitialKeyTextColor`)))
  (`TextRenderComponent.SetTextRenderColor` (`self.Enter_Text`) (`KismetMathLibrary.Conv_LinearColorToColor` (`self.InitialKeyTextColor`))))