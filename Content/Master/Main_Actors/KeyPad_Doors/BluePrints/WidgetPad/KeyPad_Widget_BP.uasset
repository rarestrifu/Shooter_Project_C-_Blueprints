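; World keypad actor for locked doors that opens a code-entry widget when F is pressed inside its collision area.
; Overlap events toggle use and recheck the lock by searching every PadData_BP actor's StoredUnlocks for this pad's BlueprintName.
; An unlocked pad swaps several components for AccessText.
; Otherwise, F creates a KeyPadWidget, passing it the code, name, denied delay and auto-close setting.
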(event `Key|F` :consume false
  (params (Key :type "Key Structure"))
  ;[1 1 1] OpenWidget
  ;;[1 0.255 0.255] InputKey
  (:`Pressed`
    (if (`self.MayUse`)
      (`self.CheckIfLockIsUnlocked`
        (:`False`
          (bind _returnvalue (`|CreateWidget` "/Game/SplinterCellMain/Blueprints_Main/KeyPad_Doors/BluePrints/WidgetPad/KeyPadWidget.KeyPadWidget_C"))
          (set `/Game/SplinterCellMain/Blueprints_Main/KeyPad_Doors/BluePrints/WidgetPad/KeyPadWidget.DeniedDelay` (`self.DeniedDelay`) _returnvalue)
          (set `/Game/SplinterCellMain/Blueprints_Main/KeyPad_Doors/BluePrints/WidgetPad/KeyPadWidget.BlueprintName` (`self.BlueprintName`) _returnvalue)
          (set `/Game/SplinterCellMain/Blueprints_Main/KeyPad_Doors/BluePrints/WidgetPad/KeyPadWidget.Code` (`self.Code`) _returnvalue)
          (set `/Game/SplinterCellMain/Blueprints_Main/KeyPad_Doors/BluePrints/WidgetPad/KeyPadWidget.AutoClose` (`self.AutoClose`) _returnvalue)
          (`UserWidget.AddToViewport` _returnvalue 0))))))

(event `self.ReceiveBeginPlay`
  ;[1 1 1] EnableInput
  (`self.EnableInput` (`GameplayStatics.GetPlayerController` 0)))

(event `self.CheckCollision.OnComponentBeginOverlap`
  (params (OverlappedComponent :type "PrimitiveComponent Object Reference") (OtherActor :type "Actor Object Reference") (OtherComp :type "PrimitiveComponent Object Reference") (OtherBodyIndex :type Integer) (bFromSweep :type Boolean) (SweepResult :type "HitResult Structure (by ref)"))
  ;[1 1 1] UnlockActivation Button
  (set `self.MayUse` true)
  (`self.CheckIfLockIsUnlocked` :!label _label))

(event `self.CheckCollision.OnComponentEndOverlap`
  (params (OverlappedComponent :type "PrimitiveComponent Object Reference") (OtherActor :type "Actor Object Reference") (OtherComp :type "PrimitiveComponent Object Reference") (OtherBodyIndex :type Integer))
  ;[1 1 1] UnlockActivation Button
  (set `self.MayUse` false)
  (goto _label))

(fn `UserConstructionScript`)