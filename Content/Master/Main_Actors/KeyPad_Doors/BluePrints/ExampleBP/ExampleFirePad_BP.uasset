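; Example keypad-linked actor that lights a fire when the player presses F nearby and its unlock is stored.
; A collision overlap sets whether lighting is allowed, and input is enabled for the first player controller on BeginPlay.
; F searches every PadData_BP actor's StoredUnlocks for this actor's BlueprintName.
; A match activates the fire and its sound once, while each non-matching actor plays a pickup cue.
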(event `self.CheckCollision.OnComponentBeginOverlap`
  (params (OverlappedComponent :type "PrimitiveComponent Object Reference") (OtherActor :type "Actor Object Reference") (OtherComp :type "PrimitiveComponent Object Reference") (OtherBodyIndex :type Integer) (bFromSweep :type Boolean) (SweepResult :type "HitResult Structure (by ref)"))
  ;[1 1 1] Trigger event
  (set `self.MayLightFire` true))

(event `self.ReceiveBeginPlay`
  ;[1 1 1] Activate use of KeyboardKeys
  (`self.EnableInput` (`GameplayStatics.GetPlayerController` 0)))

(event `self.CheckCollision.OnComponentEndOverlap`
  (params (OverlappedComponent :type "PrimitiveComponent Object Reference") (OtherActor :type "Actor Object Reference") (OtherComp :type "PrimitiveComponent Object Reference") (OtherBodyIndex :type Integer))
  ;[1 1 1] Trigger event
  (set `self.MayLightFire` false))

(event `Key|F` :consume false
  (params (Key :type "Key Structure"))
  ;[1 1 1] Open En close Door by clicking the 'F' key
  ;;[1 0.255 0.255] InputKey
  (:`Pressed`
    (if (`self.MayLightFire`)
      (if (not (`self.IsBurning`))
        (bind _outactors (`GameplayStatics.GetAllActorsOfClass` "/Game/SplinterCellMain/Blueprints_Main/KeyPad_Doors/BluePrints/PadData_BP.PadData_BP_C"))
        (for _array_element _outactors
          (if (`KismetArrayLibrary.Array_Contains` (`/Game/SplinterCellMain/Blueprints_Main/KeyPad_Doors/BluePrints/PadData_BP.StoredUnlocks` _array_element) (`self.BlueprintName`))
            (`ActorComponent.Activate` (`self.Fire`) true)
            (`ActorComponent.Activate` (`self.FireSound`) false)
            (set `self.IsBurning` true)
            (else
              (`GameplayStatics.PlaySound2D` "/Game/SplinterCellMain/Blueprints_Main/KeyPad_Doors/Audio/PickUp_Cue.PickUp_Cue" 1.0 1.0 0.0 null null))))))))

(fn `UserConstructionScript`)