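; Locker variant 5 Blueprint, a child of a parent locker class, with two parts that open and close independently.
; It assigns the door mesh as Door1 in the construction script, and the element mesh as Door2 with both end rotations on BeginPlay.
; The Doors function matches a hit component to either part and toggles it through OpenDoor1 or OpenDoor2, with the second rotating on X.
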(event `self.ReceiveBeginPlay`
  (`parent.ReceiveBeginPlay`)
  (set `self.End_Rot_Door_1` -110.0)
  (set `self.Door_2` (`self.SM_Locker_5_element`))
  (set `self.End_Rot_Door_2_X` 80.0))

(event `self.ReceiveTick`
  (params (DeltaSeconds :type "Float (single-precision)"))
  (`parent.ReceiveTick` DeltaSeconds))

(fn `Doors`
  (params (HitComp :type "PrimitiveComponent Object Reference"))
  (returns (Success :type Boolean))
  (bind _door_2 (`self.Door_2`))
  (if (== HitComp (`self.Door_1`))
    (if (not (`self.Door_1_Opened`))
      (`self.Open_Door_1` false)
      (return true)
      (else
        (`self.Open_Door_1` true)
        (return true)))
    (else
      (`/Engine/EditorBlueprintResources/StandardMacros.IsValid` _door_2
        (:`Is Valid`
          (if (== HitComp _door_2)
            (if (not (`self.Door_2_Opened`))
              (`self.Open_Door_2` false true)
              (return true)
              (else
                (`self.Open_Door_2` true true)
                (return true)))))))))

(fn `UserConstructionScript`
  (set `self.Door_1` (`self.SM_Locker_5_door`))
  (`parent.UserConstructionScript`))