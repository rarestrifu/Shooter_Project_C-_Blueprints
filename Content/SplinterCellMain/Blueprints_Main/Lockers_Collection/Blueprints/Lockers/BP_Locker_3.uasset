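; BP_Locker_3 is a single-door locker variant in the Lockers collection that builds on a parent locker Blueprint.
; Its construction script assigns the locker door mesh to the parent's Door1 slot and, when Opened is set, yaws the door to DoorRot, otherwise resetting DoorRot to zero.
; On BeginPlay it sets its own end rotation for Door1 after calling the parent logic.
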(event `self.ReceiveBeginPlay`
  (`parent.ReceiveBeginPlay`)
  (set `self.End_Rot_Door_1` -110.0))

(event `self.ReceiveTick`
  (params (DeltaSeconds :type "Float (single-precision)"))
  (`parent.ReceiveTick` DeltaSeconds))

(fn `UserConstructionScript`
  (set `self.Door_1` (`self.SM_Locker_3_door`))
  (`parent.UserConstructionScript`)
  (`|ExecutionSequence`
    (:`then_1`
      (`|ExecutionSequence`
        (:`then_0`
          (if (`self.Opened`)
            (`SceneComponent.K2_SetRelativeRotation` (`self.SM_Locker_3_door`) (`KismetMathLibrary.MakeRotator` 0.0 0.0 (`self.Door_Rot`)) false false)
            (else
              (set `self.Door_Rot` 0.0))))))))