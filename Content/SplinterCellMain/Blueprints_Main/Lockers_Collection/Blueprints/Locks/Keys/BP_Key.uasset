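; BP_Key is a collectible key actor in the lockers collection.
; Its construction script picks one of two key meshes from the SelectedKey value.
; Interact_Key destroys the actor and returns success along with SelectedKey as the key number.
; The door and lock interaction functions are stubs that return false or empty values, and the event graph holds only disabled placeholder events.
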(fn `Doors`
  (params (HitComp :type "PrimitiveComponent Object Reference"))
  (returns (Success :type Boolean))
  (return false))

(fn `Interact_Key`
  (returns (Success :type Boolean) (Key_Num :type Integer))
  (`self.K2_DestroyActor`)
  (return true (`self.Selected_Key`)))

(fn `Interact_Lock`
  (returns (Success :type Boolean) (Selected_Lock :type "/Game/SplinterCellMain/Blueprints_Main/Lockers_Collection/Blueprints/Locks/BP_Locks_Parent Object Reference"))
  (return false null))

(fn `Key_Lock`
  (returns (Success :type Boolean))
  (return false))

(fn `Key_Lock_info`
  (returns (Success :type Boolean) (Lock_Opened :type Boolean) (Key :type Integer))
  (return false false 0))

(fn `UserConstructionScript`
  (bind _key (`self.Key`))
  (`|ExecutionSequence`
    (:`then_0`
      (if (== (`self.Selected_Key`) 0)
        (`StaticMeshComponent.SetStaticMesh` _key "/Game/SplinterCellMain/Blueprints_Main/Lockers_Collection/Meshes/SM_Key_1.SM_Key_1")))
    (:`then_1`
      (if (== (`self.Selected_Key`) 1)
        (`StaticMeshComponent.SetStaticMesh` _key "/Game/SplinterCellMain/Blueprints_Main/Lockers_Collection/Meshes/SM_Key_2.SM_Key_2")))))