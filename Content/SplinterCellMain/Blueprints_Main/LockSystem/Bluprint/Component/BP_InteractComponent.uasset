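; Interaction component for the lock system, linking the player to world objects and the lock-picking UI.
; WorldInteract line-traces forward from a camera and sends an interact message, carrying the component reference, to the hit actor.
; Hide and PressedButton relay to LockSystemComponent, closing the lock widget or forwarding button presses to it.
; Tick prints every Inventory class name as debug output; the event graph's WorldInteract and Hide calls are unwired.
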(event `self.ReceiveTick`
  (params (DeltaSeconds :type "Float (single-precision)"))
  ;[1 1 1] Inventory Display
  (for _array_element (`self.Inventory`)
    (`KismetSystemLibrary.PrintString` (`KismetSystemLibrary.GetClassDisplayName` _array_element) true true (struct :`G` 0.66 :`B` 1.0 :`A` 1.0) 0.0)))

(fn `Hide`
  (`/Game/SplinterCellMain/Blueprints_Main/LockSystem/Bluprint/Component/BP_LockSystemComponent.Show / Hide Lock Widget` (`self.Lock SystemComponent`) false))

(fn `Pressed Button`
  (params (Button :type "/Game/SplinterCellMain/Blueprints_Main/LockSystem/Enumeration/E_Button Enum" :default "NewEnumerator10") (Pressed :type Boolean))
  (bind _lock_systemcomponent (`self.Lock SystemComponent`)
    (:`then`
      (bind _w_lock (`/Game/SplinterCellMain/Blueprints_Main/LockSystem/Bluprint/Component/BP_LockSystemComponent.W Lock` _lock_systemcomponent)
        (:`then`
          (message `/Game/SplinterCellMain/Blueprints_Main/LockSystem/Bluprint/Interfase/BP_Interfase.Button To Widget` _w_lock Button Pressed))
        (:`else`)))
    (:`else`)))

(fn `World Interact`
  (params (Camera :type "CameraComponent Object Reference") (Distanse :type "Float (double-precision)") (BP_InteractComponent :type "/Game/SplinterCellMain/Blueprints_Main/LockSystem/Bluprint/Component/BP_InteractComponent Object Reference"))
  (bind _returnvalue (`SceneComponent.K2_GetComponentLocation` Camera))
  ;[1 1 1] Line Trace Interact
  (bind (_outhit _returnvalue_2) (`KismetSystemLibrary.LineTraceSingle` _returnvalue (+ _returnvalue (* (`SceneComponent.GetForwardVector` Camera) Distanse)) "TraceTypeQuery1"))
  (if _returnvalue_2
    (message `/Game/SplinterCellMain/Blueprints_Main/LockSystem/Bluprint/Interfase/BP_Interact.Interact` (`.HitActor` (`GameplayStatics.BreakHitResult` _outhit)) BP_InteractComponent)
    (return)))