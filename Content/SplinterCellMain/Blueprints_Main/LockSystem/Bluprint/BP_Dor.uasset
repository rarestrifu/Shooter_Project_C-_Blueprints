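; Door actor that swings open and closed on an Action event and displays the state of its lock.
; Action toggles the Open flag and plays or reverses the DorRotator timeline, which drives the yaw of the door mesh.
; A text render shows "Open" or "Lock" from the lock system component's LockOpen, refreshed on BeginPlay and ActiononOpening.
; Action itself does not check the lock.
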(event `/Game/SplinterCellMain/Blueprints_Main/LockSystem/Bluprint/Interfase/BP_Interfase.Action`
  ;[1 1 1] Open door
  (if (not (`self.Open? `))
    (set `self.Open? ` true)
    (bind (_direction _dorrotator) (`Timeline|DorRotator` :!label _label)
      (:`Update`
        (`SceneComponent.K2_SetRelativeRotation` (`self.SM_Door`) (`KismetMathLibrary.MakeRotator` 0.0 0.0 _dorrotator) false false)))
    (else
      (set `self.Open? ` false)
      (goto _label :!via `Reverse`))))

(event `self.ReceiveBeginPlay`
  ;[1 1 1] txt update
  (`parent.ReceiveBeginPlay`)
  (if (`/Game/SplinterCellMain/Blueprints_Main/LockSystem/Bluprint/Component/BP_LockSystemComponent.Lock Open?` (`self.BP_LockSystemComponent`)) :!label _label_2
    (`TextRenderComponent.K2_SetText` (`self.TextRender`) (`|FormatText` "Open"))
    (else
      (`TextRenderComponent.K2_SetText` (`self.TextRender`) (`|FormatText` "Lock")))))

(event `/Game/SplinterCellMain/Blueprints_Main/LockSystem/Bluprint/Interfase/BP_Interfase.Action on opening`
  ;[1 1 1] txt update
  (goto _label_2))

(fn `UserConstructionScript`
  (`parent.UserConstructionScript`))