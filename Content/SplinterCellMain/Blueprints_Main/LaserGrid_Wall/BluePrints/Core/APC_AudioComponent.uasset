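; Scene component in the laser grid wall assets that plays a start, loop and end sound sequence with volume fades.
; Init stores the cues and fade speed and spawns a persistent attached loop audio component, while start and end cues spawn as auto-destroying one-shots.
; Transition events set blend flags that Tick uses to lerp the loop volume, stopping it after fade-out.
; StopAll adds a fade multiplier and skips the end cue.
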(event `Init`
  (params (StartCue :type "SoundCue Object Reference") (EndCue :type "SoundCue Object Reference") (LoopCue :type "SoundCue Object Reference") (FadeSpeed :type "Float (double-precision)"))
  ;[1 1 1] Initialization
  (set `self.StartCue` StartCue)
  (set `self.EndCue` EndCue)
  (set `self.BlendSpeed` (`KismetMathLibrary.SelectFloat` 1.0 FadeSpeed (== FadeSpeed 0.0)))
  (bind _audiocomp (`self.Spawn` LoopCue))
  (bind _output_get (set `self.LoopAudio` _audiocomp))
  (`/Engine/EditorBlueprintResources/StandardMacros.IsValid` _output_get
    (:`Is Valid`
      (`self.SetActive` _output_get false true))))

(event `StartToLoop`
  (bind _loopaudio (`self.LoopAudio`))
  ;[1 1 1] FadeIn from Start to Loop sample
  (set `self.StopMultiplier` 1.0)
  (bind _audiocomp (`self.Spawn` (`self.StartCue`) true))
  (bind _output_get (set `self.StartAudio` _audiocomp))
  (`/Engine/EditorBlueprintResources/StandardMacros.IsValid` _output_get
    (:`Is Valid`
      (`AudioComponent.Play` _output_get 0.0))
    (:`Is Not Valid`
      _))
  (`/Engine/EditorBlueprintResources/StandardMacros.IsValid` _loopaudio
    (:`Is Valid`
      (`AudioComponent.SetVolumeMultiplier` _loopaudio 0.0)
      (`self.SetActive` _loopaudio true true)
      (`AudioComponent.Play` _loopaudio 0.0)
      (set `self.BlendTime` 0.0)
      (set `self.VolumeMultiplier` 0.0)
      (set `self.StartLoopSound` true)
      (set `self.WantBlend` true)
      (set `self.WantStopAll` false))))

(event `StopAll`
  ;[1 1 1] FadeOut from Loop to End sample
  (set `self.WantStopAll` true)
  (set `self.StopBlendTime` 0.0)
  (`/Engine/EditorBlueprintResources/StandardMacros.IsValid` (`self.LoopAudio`) :!label _label
    (:`Is Valid`
      (set `self.BlendTime` 0.0)
      (set `self.VolumeMultiplier` 1.0)
      (set `self.StartLoopSound` false)
      (set `self.WantBlend` true))))

(event `LoopToEnd`
  ;[1 1 1] FadeOut from Loop to End sample
  (set `self.StopMultiplier` 1.0)
  (set `self.WantStopAll` false)
  (bind _audiocomp (`self.Spawn` (`self.EndCue`) true))
  (`/Engine/EditorBlueprintResources/StandardMacros.IsValid` _audiocomp
    (:`Is Valid`
      (`AudioComponent.Play` _audiocomp 0.0)
      (goto _label))
    (:`Is Not Valid`
      (goto _label))))

(event `LoopOnly`
  (bind _loopaudio (`self.LoopAudio`))
  (set `self.StopMultiplier` 1.0)
  (set `self.WantStopAll` false)
  (set `self.BlendTime` 0.0)
  (set `self.VolumeMultiplier` 0.0)
  (set `self.StartLoopSound` true)
  (set `self.WantBlend` true)
  (set `self.StopMultiplier` 1.0)
  (`/Engine/EditorBlueprintResources/StandardMacros.IsValid` _loopaudio
    (:`Is Valid`
      (`AudioComponent.Play` _loopaudio 0.0))))

(event `StopStartSound`
  (bind _startaudio (`self.StartAudio`))
  (`/Engine/EditorBlueprintResources/StandardMacros.IsValid` _startaudio
    (:`Is Valid`
      (`AudioComponent.Stop` _startaudio))))

(event `self.ReceiveTick`
  (params (DeltaSeconds :type "Float (single-precision)"))
  (bind _returnvalue (+ (`self.BlendTime`) (* DeltaSeconds (`self.BlendSpeed`))))
  (bind _returnvalue_2 (`KismetMathLibrary.FClamp` _returnvalue))
  (bind _returnvalue_3 (`KismetMathLibrary.FClamp` (+ (`self.StopBlendTime`) (* DeltaSeconds (`self.BlendSpeed`)))))
  ;[1 1 1] Blend Volume Multiplier for Loop sample
  (`|ExecutionSequence`
    (:`then_0`
      (if (`self.WantStopAll`)
        (set `self.StopBlendTime` _returnvalue_3)
        (set `self.StopMultiplier` (`KismetMathLibrary.Lerp` 1.0 0.0 _returnvalue_3))
        (if (>= (`self.StopBlendTime`) 1.0)
          (set `self.WantStopAll` false))))
    (:`then_1`
      (if (`self.WantBlend`)
        (set `self.BlendTime` _returnvalue)
        (`AudioComponent.SetVolumeMultiplier` (`self.LoopAudio`) (* (`self.VolumeMultiplier`) (`self.StopMultiplier`)))
        (set `self.VolumeMultiplier` (`KismetMathLibrary.SelectFloat` (`KismetMathLibrary.Lerp` 0.0 1.0 _returnvalue_2) (`KismetMathLibrary.Lerp` 1.0 0.0 _returnvalue_2) (`self.StartLoopSound`)))
        (if (> (`self.BlendTime`) 1.0)
          (set `self.WantBlend` false)
          (if (not (`self.StartLoopSound`))
            (`AudioComponent.Stop` (`self.LoopAudio`))))))))

(fn `GetLoopAudioComponent`
  (returns (LoopAudioComp :type "AudioComponent Object Reference"))
  ;[1 1 1] Return Loop Audio component
  (return (`self.LoopAudio`)))

(fn `Spawn`
  (params (Cue :type "SoundCue Object Reference") (Autodestroy :type Boolean))
  (returns (AudioComp :type "AudioComponent Object Reference"))
  ;[1 1 1] Spawn Audio component for Loop sample attached
  (`/Engine/EditorBlueprintResources/StandardMacros.IsValid` Cue
    (:`Is Valid`
      (bind _returnvalue (`GameplayStatics.SpawnSoundAttached` Cue self "None" (0.0 0.0 0.0) (struct) "KeepRelativeOffset" true 1.0 1.0 0.0 null null Autodestroy))
      (return _returnvalue))
    (:`Is Not Valid`
      (return null))))