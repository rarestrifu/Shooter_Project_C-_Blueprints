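; AC_CallAction is an actor component that lets its owning character target and trigger interactable objects.
; CallAction line-traces forward from a third-person view point, toggles custom depth on targets carrying a Virtual_AC_RunAction component and shows a W_ActionHotkey widget.
; The PreAction flag selects between sending that component a preview message or an action message with the character, the latter also hiding the widget.
; A missed trace clears the last target's highlight and the widget.
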(event `CallAction`
  (params (PreAction :type Boolean))
  (bind _lastactor (`self.LastActor`))
  (bind _transformcomponent (`PlayerCameraManager.TransformComponent` (`PlayerController.PlayerCameraManager` (`GameplayStatics.GetPlayerController` 0))))
  (bind (_start _end) (`/Game/SplinterCellMain/Blueprints_Main/Lift_Actors/ScissorsLift/Blueprints/Data/ML_Ob_MacroLibrary.CalcTrace` (`SceneComponent.K2_GetComponentLocation` _transformcomponent) (`SceneComponent.GetForwardVector` _transformcomponent) 600.0))
  (bind (_outhit _returnvalue) (`KismetSystemLibrary.LineTraceSingle` :`Start` _start :`End` _end :`TraceChannel` (enumliteral `ETraceTypeQuery` "TraceTypeQuery11") :`DrawDebugType` "ForOneFrame"))
  (if _returnvalue
    (bind (_bblockinghit _binitialoverlap _time _distance _location _impactpoint _normal _impactnormal _physmat _hitactor) (`GameplayStatics.BreakHitResult` _outhit))
    (bind _returnvalue_2 (`Actor.GetComponentByClass` _hitactor "/Game/SplinterCellMain/Blueprints_Main/Lift_Actors/ScissorsLift/Blueprints/Data/Virtual_AC_RunAction.Virtual_AC_RunAction_C"))
    (if (and (!= (`self.LastActor`) _hitactor) (`KismetSystemLibrary.IsValid` _returnvalue_2))
      (`/Game/SplinterCellMain/Blueprints_Main/Lift_Actors/ScissorsLift/Blueprints/Data/BP_FunctionLibrary.On\\Off_CustomDepth` _hitactor true))
    (set `self.LastActor` _hitactor)
    (`self.WidgetOn`)
    (if PreAction
      (message `/Game/SplinterCellMain/Blueprints_Main/Lift_Actors/ScissorsLift/Blueprints/Data/BPI_GamePlay.PreAction` _returnvalue_2)
      (else
        (message `/Game/SplinterCellMain/Blueprints_Main/Lift_Actors/ScissorsLift/Blueprints/Data/BPI_GamePlay.Action` _returnvalue_2 (cast `Character` (`self.GetOwner`) :!pure true))
        (`Widget.RemoveFromParent` (`self.UI`))))
    (else
      (`/Engine/EditorBlueprintResources/StandardMacros.IsValid` _lastactor
        (:`Is Valid`
          (`/Game/SplinterCellMain/Blueprints_Main/Lift_Actors/ScissorsLift/Blueprints/Data/BP_FunctionLibrary.On\\Off_CustomDepth` _lastactor)
          (set `self.LastActor` null)
          (`Widget.RemoveFromParent` (`self.UI`)))))))

(fn `WidgetOn`
  (bind _ui (`self.UI`))
  (`/Engine/EditorBlueprintResources/StandardMacros.IsValid` _ui
    (:`Is Valid`
      (if (not (`Widget.IsInViewport` _ui))
        (`UserWidget.AddToViewport` _ui 0)))
    (:`Is Not Valid`
      (bind _returnvalue (`|CreateWidget` "/Game/SplinterCellMain/Blueprints_Main/Lift_Actors/ScissorsLift/Blueprints/UI/W_ActionHotkey.W_ActionHotkey_C"))
      (bind _output_get (set `self.UI` _returnvalue))
      (`UserWidget.AddToViewport` _output_get 0))))