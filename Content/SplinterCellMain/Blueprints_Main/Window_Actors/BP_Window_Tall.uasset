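; Tall window actor whose glass shatters when a bullet hits its hit box or it takes radial damage.
; Breaking plays a sound, swaps the glass for a runtime-added destructible mesh with force and damage, removes the hit box and reports a "Shoot" noise for AI to investigate.
; BreakTheGlass is a gentler variant that keeps the hit box and reports no noise.
; Interaction type and manual velocity functions return fixed values.
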(event `self.ReceiveBeginPlay`
  (set `self.World Location` (`SceneComponent.K2_GetComponentLocation` (`self.Window_Frame_Square`))))

(event `/Game/AdvancedLocomotionV4/Blueprints/Interfaces/Interactive_Objects_Interface.Hit By Bullet`
  (params (`Hit Info` :type "/Game/AdvancedLocomotionV4/Data/Structs/Weapon-HitActorInfo Structure") (From :type "Character Object Reference"))
  (bind _glass_tall (`self.Glass_Tall`))
  (bind _returnvalue (`SceneComponent.K2_GetComponentLocation` (`self.Hit_Box_Tall`)))
  ;[0 0 0] Check make sure it is glass
  (if (== `Hit Info_Component_21_DE9817A14F727A6D24C38BA42C11B98D` (`self.Hit_Box_Tall`))
    (`/Engine/EditorBlueprintResources/StandardMacros.IsValid` (`self.Glass_Tall`) :!label _label
      (:`Is Valid`
        ;[1 1 1] Get sound to play smashing sound
        (`GameplayStatics.PlaySoundAtLocation` (`self.Sound`) _returnvalue (struct) (`self.Volume Multiplier`) 1.0 0.0 null null null)
        ;[1 1 1] Swap out for destructible mesh, destroy original mesh apply damage and impulse
        (bind _returnvalue_2 (`AddComponent|NODE_AddDestructibleComponent-2` :`bManualAttachment` true))
        (`SceneComponent.K2_SetWorldTransform` _returnvalue_2 (`SceneComponent.K2_GetComponentToWorld` _glass_tall) false true)
        (`DestructibleComponent.SetDestructibleMesh` _returnvalue_2 (`self.DestructibleMeshTall`))
        (`PrimitiveComponent.AddRadialForce` _returnvalue_2 _returnvalue 100.0 250.0 "RIF_Constant" false)
        (`DestructibleComponent.ApplyDamage` _returnvalue_2 10000.0 _returnvalue (0.0 0.0 -1.0) 250.0)
        (`ActorComponent.K2_DestroyComponent` _glass_tall)
        (`ActorComponent.K2_DestroyComponent` (`self.Hit_Box_Tall`))
        ;[1 0.283 0] Report noise for AI to investigate
        (`AISense_Hearing.ReportNoiseEvent` (`self.World Location`) 1.0 self 1200.0 "Shoot")))))

(event `self.ReceiveRadialDamage`
  (params (DamageReceived :type "Float (single-precision)") (DamageType :type "DamageType Object Reference") (Origin :type "Vector Structure") (HitInfo :type "HitResult Structure (by ref)") (InstigatedBy :type "Controller Object Reference") (DamageCauser :type "Actor Object Reference"))
  (goto _label))

(fn `Break The Glass`
  (bind _glass_tall (`self.Glass_Tall`))
  (bind _returnvalue (`SceneComponent.K2_GetComponentLocation` (`self.Hit_Box_Tall`)))
  ;[1 1 1] Get sound to play smashing sound
  (`GameplayStatics.PlaySoundAtLocation` (`self.Sound`) _returnvalue (struct) (`self.Volume Multiplier`) 1.0 0.0 null null null)
  ;[1 1 1] Swap out for destructible mesh, destroy original mesh apply damage and impulse
  (bind _returnvalue_2 (`AddComponent|NODE_AddDestructibleComponent-1` :`bManualAttachment` true))
  (`SceneComponent.K2_SetWorldTransform` _returnvalue_2 (`SceneComponent.K2_GetComponentToWorld` _glass_tall) false true)
  (`DestructibleComponent.SetDestructibleMesh` _returnvalue_2 (`self.DestructibleMeshTall`))
  (`PrimitiveComponent.AddRadialForce` _returnvalue_2 _returnvalue 50.0 100.0 "RIF_Constant" false)
  (`DestructibleComponent.ApplyDamage` _returnvalue_2 10000.0 _returnvalue (0.0 0.0 -1.0) 100.0)
  (`ActorComponent.K2_DestroyComponent` _glass_tall))

(fn `Get Interaction Type`
  (returns (Type :type "/Game/AdvancedLocomotionV4/Data/Enums/Interaction_Type Enum"))
  (return "NewEnumerator0"))

(fn `Get Manual Velocity`
  (returns (Velocity :type "Vector Structure"))
  (return (0.0 0.0 0.0)))

(fn `UserConstructionScript`)