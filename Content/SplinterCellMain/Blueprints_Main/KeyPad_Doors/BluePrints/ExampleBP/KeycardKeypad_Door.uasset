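; Example door that opens and closes on the Interaction input once a keypad or keycard pad has unlocked it.
; A collision overlap enables player input, and a timeline swings the door 90 degrees in yaw.
; While locked, pressing searches every PadData_BP's StoredUnlocks for BlueprintName, then opens or plays a locked sound; IsOpen toggles either way.
; The construction script sets the door's text label and color.
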(event `self.CheckCollision.OnComponentBeginOverlap`
  (params (OverlappedComponent :type "PrimitiveComponent Object Reference") (OtherActor :type "Actor Object Reference") (OtherComp :type "PrimitiveComponent Object Reference") (OtherBodyIndex :type Integer) (bFromSweep :type Boolean) (SweepResult :type "HitResult Structure (by ref)"))
  ;[1 1 1] Trigger event
  (if (== OtherActor (`GameplayStatics.GetPlayerPawn` 0))
    (set `self.MayOpenDoor` true)
    ;;[0 0 0] Enable input only on overlap?
    (`self.EnableInput` (`GameplayStatics.GetPlayerController` 0))))

(event `self.CheckCollision.OnComponentEndOverlap`
  (params (OverlappedComponent :type "PrimitiveComponent Object Reference") (OtherActor :type "Actor Object Reference") (OtherComp :type "PrimitiveComponent Object Reference") (OtherBodyIndex :type Integer))
  ;[1 1 1] Trigger event
  (set `self.MayOpenDoor` false)
  ;;[0 0 0] Enable input only on overlap?
  (`self.DisableInput` (`GameplayStatics.GetPlayerController` 0)))

(event `OpenDoor`
  ;[1 1 1] Open and close door sequence
  (if (`self.CheckDoorUnlocked`)
    (bind (_direction _opendoor) (`Timeline|openDoorAnimation` :!label _label)
      (:`Update`
        (`SceneComponent.K2_SetRelativeRotation` (`self.Door`) (`KismetMathLibrary.MakeRotator` 0.0 0.0 (* _opendoor 90.0)) false false)))))

(event `CloseDoor`
  ;[1 1 1] Open and close door sequence
  (if (`self.CheckDoorUnlocked`)
    (goto _label :!via `Reverse`)))

(event `InputAction|Interaction` :consume false
  (params (Key :type "Key Structure"))
  ;[1 1 1] Open En close Door by clicking the
  ;;[1 0.255 0.255] InputKey
  (:`Pressed`
    (if (`self.MayOpenDoor`)
      (if (`self.Is Open`)
        (`self.CloseDoor`)
        (set `self.Is Open` false)
        (else
          (`self.OpenDoor`)
          (set `self.Is Open` true)))
      ;[1 1 1] Check If Door is unlocked by Pad
      (if (`self.CheckDoorUnlocked`)
        (`GameplayStatics.PlaySound2D` "/Game/SplinterCellMain/Blueprints_Main/KeyPad_Doors/Audio/DoorOpen_Cue.DoorOpen_Cue" 1.0 1.0 0.0 null null)
        (else
          (bind _outactors (`GameplayStatics.GetAllActorsOfClass` "/Game/SplinterCellMain/Blueprints_Main/KeyPad_Doors/BluePrints/PadData_BP.PadData_BP_C"))
          (for _array_element _outactors
            (bind _output_get (set `self.CheckDoorUnlocked` (`KismetArrayLibrary.Array_Contains` (`/Game/SplinterCellMain/Blueprints_Main/KeyPad_Doors/BluePrints/PadData_BP.StoredUnlocks` _array_element) (`self.BlueprintName`))))
            (if _output_get
              (`self.OpenDoor`)
              (`GameplayStatics.PlaySound2D` "/Game/SplinterCellMain/Blueprints_Main/KeyPad_Doors/Audio/DoorOpen_Cue.DoorOpen_Cue" 1.0 1.0 0.0 null null)
              (else
                (`GameplayStatics.PlaySound2D` "/Game/SplinterCellMain/Blueprints_Main/KeyPad_Doors/Audio/DoorLocked_Cue.DoorLocked_Cue" 1.0 1.0 0.0 null null)))))))))

(fn `UserConstructionScript`
  (bind _doortext (`self.DoorText`))
  (`TextRenderComponent.K2_SetText` _doortext (`self.Text`))
  (`TextRenderComponent.SetTextRenderColor` _doortext (`KismetMathLibrary.Conv_LinearColorToColor` (`self.TextColor`))))