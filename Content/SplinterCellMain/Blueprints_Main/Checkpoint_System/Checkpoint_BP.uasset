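; Checkpoint trigger actor with a configurable platform mesh that autosaves a respawn transform when the player overlaps it, then destroys itself.
; Update Saved Checkpoint writes the actor's transform, raised slightly, to a Checkpoint_SaveGame slot, creating the save if none exists.
; A first save plays sound and particles and shows a "Checkpoint Saved" popup, while overwriting an existing save shows "Checkpoint Updated".
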(event `self.ReceiveBeginPlay`
  (if (`self.Disable Mesh Collision?`)
    (`PrimitiveComponent.SetCollisionEnabled` (`self.platform_mesh`) "NoCollision")
    (set `self.As Player Character` (`GameplayStatics.GetPlayerPawn` 0))))

(event `self.Checkpoint_Overlap.OnComponentBeginOverlap`
  (params (OverlappedComponent :type "PrimitiveComponent Object Reference") (OtherActor :type "Actor Object Reference") (OtherComp :type "PrimitiveComponent Object Reference") (OtherBodyIndex :type Integer) (bFromSweep :type Boolean) (SweepResult :type "HitResult Structure (by ref)"))
  (bind _returnvalue (`GameplayStatics.GetPlayerController` 0))
  (bind (_returnvalue_location _returnvalue_rotation) (`KismetMathLibrary.BreakTransform` (`self.GetTransform`)))
  (bind _returnvalue_2 (`KismetMathLibrary.MakeTransform` (+ _returnvalue_location (0.0 0.0 100.0)) _returnvalue_rotation))
  (if (== OtherActor (`GameplayStatics.GetPlayerPawn` 0))
    (`/Engine/EditorBlueprintResources/StandardMacros.DoOnce` false
      (:`Completed`
        (bind _returnvalue_3 (`GameplayStatics.DoesSaveGameExist` (`self.Checkpoint Save Name`)))
        (if _returnvalue_3
          (bind _returnvalue_4 (`GameplayStatics.LoadGameFromSlot` (`self.Checkpoint Save Name`)))
          (bind _ascheckpoint_save_game (cast `/Game/SplinterCellMain/Blueprints_Main/Checkpoint_System/Checkpoint_SaveGame` _returnvalue_4))
          (set `self.Checkpoint Save Game Ref` _ascheckpoint_save_game)
          (bind _output_get (set `/Game/SplinterCellMain/Blueprints_Main/Checkpoint_System/Checkpoint_SaveGame.Checkpoint` _returnvalue_2 (`self.Checkpoint Save Game Ref`)))
          (`GameplayStatics.SaveGameToSlot` (`self.Checkpoint Save Game Ref`) (`self.Checkpoint Save Name`))
          (`KismetSystemLibrary.PrintString` (`KismetStringLibrary.Concat_StrStr` "Reset Location:  " (`KismetStringLibrary.Conv_VectorToString` (.location _output_get))) true true (struct :`R` 0.758248 :`G` 1.0 :`A` 1.0) 10.0)
          (bind _returnvalue_5 (`|CreateWidget` "/Game/SplinterCellMain/Blueprints_Main/Checkpoint_System/AutoSave_Popup.AutoSave_Popup_C" _returnvalue))
          (`/Game/SplinterCellMain/Blueprints_Main/Checkpoint_System/AutoSave_Popup.Display_AutoSave_Popup` _returnvalue_5 "Checkpoint Updated")
          (`UserWidget.AddToViewport` _returnvalue_5 0)
          (else
            (bind _returnvalue_6 (`GameplayStatics.CreateSaveGameObject` "/Game/SplinterCellMain/Blueprints_Main/Checkpoint_System/Checkpoint_SaveGame.Checkpoint_SaveGame_C"))
            (set `self.Checkpoint Save Game Ref` _returnvalue_6)
            (`GameplayStatics.PlaySound2D` (`self.Sound to Play`) 1.0 1.0 0.0 null null)
            (`GameplayStatics.SpawnEmitterAtLocation` (`self.Particle To Play`) _returnvalue_location)
            (`KismetSystemLibrary.PrintString` "Checkpoint Saved!" true true (struct :`R` 1.0 :`G` 0.870238 :`A` 1.0) 5.0)
            (bind _output_get_2 (set `/Game/SplinterCellMain/Blueprints_Main/Checkpoint_System/Checkpoint_SaveGame.Checkpoint` _returnvalue_2 (`self.Checkpoint Save Game Ref`)))
            (`GameplayStatics.SaveGameToSlot` (`self.Checkpoint Save Game Ref`) (`self.Checkpoint Save Name`))
            (`KismetSystemLibrary.PrintString` (`KismetStringLibrary.Concat_StrStr` "New Location:  " (`KismetStringLibrary.Conv_VectorToString` (.location _output_get_2))) true true (struct :`R` 1.0 :`G` 0.501495 :`A` 1.0) 10.0)
            (bind _returnvalue_7 (`|CreateWidget` "/Game/SplinterCellMain/Blueprints_Main/Checkpoint_System/AutoSave_Popup.AutoSave_Popup_C" _returnvalue))
            (`/Game/SplinterCellMain/Blueprints_Main/Checkpoint_System/AutoSave_Popup.Display_AutoSave_Popup` _returnvalue_7 "Checkpoint Saved")
            (`UserWidget.AddToViewport` _returnvalue_7 0)))
        (`self.K2_DestroyActor`)))))

(event `self.Checkpoint_Overlap.OnComponentEndOverlap`
  (params (OverlappedComponent :type "PrimitiveComponent Object Reference") (OtherActor :type "Actor Object Reference") (OtherComp :type "PrimitiveComponent Object Reference") (OtherBodyIndex :type Integer))
  (if (== OtherActor (`GameplayStatics.GetPlayerPawn` 0))
    (`self.K2_DestroyActor`)))

(fn `UserConstructionScript`
  (bind _platform_mesh (`self.platform_mesh`))
  (`StaticMeshComponent.SetStaticMesh` _platform_mesh (`self.New Mesh`))
  (`SceneComponent.SetHiddenInGame` _platform_mesh (`self.Hide Mesh inGame?`) false))