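; Blueprint function library that combines readings from an array of light probes for the illumination detection system.
; CheckOverallIllumination sums each probe's illumination, weighted by its MaxOverallIllumination, clamping the running total between zero and one.
; CheckOverallColor averages the probes' ColorMix RGB channels into a single opaque color, with no guard for an empty array.
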(fn `CheckOverallColor`
  (params (IlluminationProbes :type "Array of /Game/SplinterCellMain/Blueprints_Main/IlluminationDetection/Blueprints/IlluminationComponents/BP_IlluminationProbe Object Reference"))
  (returns (LinearColor :type "LinearColor Structure"))
  (locals (TempR :type "Float (double-precision)") (TempG :type "Float (double-precision)") (TempB :type "Float (double-precision)"))
  (bind _returnvalue (`KismetMathLibrary.Conv_IntToDouble` (`KismetArrayLibrary.Array_Length` IlluminationProbes)))
  ;[1 1 1] ResetTempValues
  (set `local.TempR` 0.0)
  (set `local.TempG` 0.0)
  (set `local.TempB` 0.0)
  ;[1 1 1] Get total RGB
  (for _array_element IlluminationProbes
    (bind (_r _g _b) (break `LinearColor` (`/Game/SplinterCellMain/Blueprints_Main/IlluminationDetection/Blueprints/IlluminationComponents/BP_IlluminationProbe.ColorMix` _array_element)))
    (set `local.TempR` (+ _r (`local.TempR`)))
    (set `local.TempG` (+ _g (`local.TempG`)))
    (set `local.TempB` (+ _b (`local.TempB`))))
  ;[1 1 1] Sample RGB/number of colors sampled
  (set `local.TempR` (/ (`local.TempR`) _returnvalue))
  (set `local.TempG` (/ (`local.TempG`) _returnvalue))
  (set `local.TempB` (/ (`local.TempB`) _returnvalue))
  ;[1 1 1] Store result to ColorMix
  (return (make `LinearColor` (`local.TempR`) (`local.TempG`) (`local.TempB`) 1.0)))

(fn `CheckOverallIllumination`
  (params (IlluminationProbes :type "Array of /Game/SplinterCellMain/Blueprints_Main/IlluminationDetection/Blueprints/IlluminationComponents/BP_IlluminationProbe Object Reference"))
  (returns (OverallIllumination :type "Float (double-precision)"))
  (locals (TempIlluminationVal :type "Float (double-precision)"))
  ;[1 1 1] Compares illumination value of all light probes in an array & provides an overall illumination value across the board
  (set `local.TempIlluminationVal` 0.0)
  (for _array_element IlluminationProbes
    (set `local.TempIlluminationVal` (`KismetMathLibrary.FClamp` (+ (`local.TempIlluminationVal`) (* (`/Game/SplinterCellMain/Blueprints_Main/IlluminationDetection/Blueprints/IlluminationComponents/BP_IlluminationProbe.MaxOverallIllumination` _array_element) (`/Game/SplinterCellMain/Blueprints_Main/IlluminationDetection/Blueprints/IlluminationComponents/BP_IlluminationProbe.ProbeIllumination` _array_element))))))
  (return (`local.TempIlluminationVal`)))