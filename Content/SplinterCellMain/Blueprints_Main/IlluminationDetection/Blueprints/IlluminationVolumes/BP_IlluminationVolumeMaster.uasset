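; Master illumination volume for the light detection system, marking a light's area of influence and exposing its source location, color, attenuation distance and status to probes.
; Construction snaps it to a referenced spot or point light, copying color and radius, and aligning rotation for spotlights.
; A referenced actor without either component makes it a manual boundary, with attenuation from the largest box or sphere extent.
; An invalid reference only changes light status.
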(event `UpdateBoundsVisibility`
  (params (`HiddenInGame?` :type Boolean)))

(event `SetLightStatus`
  (params (Status :type "/Game/SplinterCellMain/Blueprints_Main/IlluminationDetection/Blueprints/IlluminationVolumes/EN_LightStatus Enum" :default "NewEnumerator0"))
  (set `self.LightStatus` Status))

(fn `GetAttenuationDistanceFromAllExtentAxes`
  (returns (Return :type Boolean))
  (locals (TempMaxDist :type "Float (double-precision)") (Extents :type "Array of Float (double-precision)") (CurrentHighestInstance :type Integer :default -1))
  (bind (_volumeboxextent_x _volumeboxextent_y _volumeboxextent_z) (`KismetMathLibrary.BreakVector` (`self.VolumeBoxExtent`)))
  ;[1 1 1] Measures extent values of all box axes/sphere radius, compares floats per axis to determine which kind of boundary subclass is being used, and what size/scale boundaries it has using a float comparison script
  (set `local.TempMaxDist` 0.0)
  (set `local.CurrentHighestInstance` -1)
  (bind _output_get (set `local.Extents` (`|MakeArray` _volumeboxextent_x _volumeboxextent_y _volumeboxextent_z (`self.VolumeSphereExtent`))))
  (for (_array_element _array_index) _output_get
    (if (> _array_element (`local.TempMaxDist`))
      (set `local.TempMaxDist` _array_element)
      (set `local.CurrentHighestInstance` _array_index)))
  (if (>= (`local.CurrentHighestInstance`) 0)
    (set `self.AttenuationDistance` (`|GetArrayItem` (`local.Extents`) (`local.CurrentHighestInstance`)))
    (return true)
    (else
      (return false))))

(fn `GetWorldspaceSourceLocation`
  (returns (ReturnValue :type "Vector Structure"))
  ;[1 1 1] Transforms source location (relative) to worldspace coordinates for other actors to reference
  (return (`KismetMathLibrary.TransformLocation` (`self.GetTransform`) (`self.SourceLocation`))))

(fn `Initialize`
  (returns (`Success?` :type Boolean))
  (bind _pl_ref (`self.PL_Ref`))
  (bind _sl_ref (`self.SL_Ref`))
  (`self.LightActorRef`
    (:`then`
      ;[1 1 1] Checks to see if a light component ref has been set, if not then the volume is treated as a manual boundary, presumably for special use cases/LPV emission injections
      (if (or (`KismetSystemLibrary.IsValid` (`self.GetComponentByClass` (`self.LightActorRef`) "/Script/Engine.PointLightComponent")) (`KismetSystemLibrary.IsValid` (`self.GetComponentByClass` (`self.LightActorRef`) "/Script/Engine.SpotLightComponent")))
        ;[1 1 1] Light ref has been detected; is it a spot light(t) or a point light(f)?
        (bind _output_get (set `self.IsSpotLight?` (`KismetSystemLibrary.IsValid` (`self.GetComponentByClass` (`self.LightActorRef`) "/Script/Engine.SpotLightComponent"))))
        (if _output_get
          ;[1 1 1] Spot light has been detected; gets light attenuation radius to use as overlap boundary extent,  and actor forward vector to orient boundary to match spotlight rot. Also sets Illumination Component Color
          (set `self.SL_Ref` (`self.GetComponentByClass` (`self.LightActorRef`) "/Script/Engine.SpotLightComponent"))
          (set `self.VolumeSphereExtent` (`LocalLightComponent.AttenuationRadius` (`self.SL_Ref`)))
          (`self.K2_SetActorLocationAndRotation` (`SceneComponent.K2_GetComponentLocation` _sl_ref) (`KismetMathLibrary.Conv_VectorToRotator` (`SceneComponent.GetForwardVector` _sl_ref)))
          (set `/Game/SplinterCellMain/Blueprints_Main/IlluminationDetection/Blueprints/IlluminationComponents/BP_LightIlluminationProperties.LightSourceColor` (`LightComponentBase.GetLightColor` (`self.SL_Ref`)) (`self.BP_LightIlluminationProperties`))
          (else
            ;[1 1 1] Point light has been detected; gets light attenuation radius to use as overlap boundary extent. Also sets illumination component color
            (set `self.PL_Ref` (`self.GetComponentByClass` (`self.LightActorRef`) "/Script/Engine.PointLightComponent"))
            (set `self.VolumeSphereExtent` (`LocalLightComponent.AttenuationRadius` _pl_ref))
            (`self.K2_SetActorLocation` (`SceneComponent.K2_GetComponentLocation` _pl_ref))
            (set `/Game/SplinterCellMain/Blueprints_Main/IlluminationDetection/Blueprints/IlluminationComponents/BP_LightIlluminationProperties.LightSourceColor` (`LightComponentBase.GetLightColor` (`self.PL_Ref`)) (`self.BP_LightIlluminationProperties`))))
        ;[1 1 1] Attenuation Radius used by Probe to scale illumination over distance, uses auto-scaled Sphere Extent as basis
        (set `self.AttenuationDistance` (`self.VolumeSphereExtent`))
        (`self.SetLightStatus` "NewEnumerator0")
        (return true)
        (else
          ;[1 1 1] Measures extent values of all box axes/sphere radius to determine which kind of boundary subclass is being used, and what size boundaries it has
          (`self.GetAttenuationDistanceFromAllExtentAxes`)
          (`self.SetLightStatus` "NewEnumerator0")
          (return true))))
    (:`else`
      (`self.SetLightStatus` "NewEnumerator1")
      (return false))))

(fn `UserConstructionScript`
  (`self.Initialize`))