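; BP_LockpickBox is a pickup that gives the player lockpicks when interacted with.
; Its construction script can randomize the box's count within a range.
; LockPickInteract checks that BP_LockPickingComponent on the player pawn is below MaxLockpicks, then adds the full count once, without clamping.
; It then shows an animated singular or plural notification on UI_LockpickingHUD, plays a sound and destroys itself.
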(event `/Game/SplinterCellMain/Blueprints_Main/LockPicking/Blueprints/Core/BPI_LockPick.LockPick_Interact`
  (bind _lockpicksinbox (`self.LockpicksInBox`))
  (bind _returnvalue (`self.GetComponentByClass` (`GameplayStatics.GetPlayerPawn` 0) "/Game/SplinterCellMain/Blueprints_Main/LockPicking/Blueprints/BP_LockPickingComponent.BP_LockPickingComponent_C"))
  ;[0.02315 0.2918 0.0137] Check if lockpicks are full
  (if (< (`/Game/SplinterCellMain/Blueprints_Main/LockPicking/Blueprints/BP_LockPickingComponent.LockPicks` _returnvalue) (`/Game/SplinterCellMain/Blueprints_Main/LockPicking/Blueprints/BP_LockPickingComponent.MaxLockpicks` _returnvalue))
    ;[0.02315 0.2918 0.0137] Add amount of lockpicks, then destroy box
    (`/Engine/EditorBlueprintResources/StandardMacros.DoOnce` false
      (:`Completed`
        (set `/Game/SplinterCellMain/Blueprints_Main/LockPicking/Blueprints/BP_LockPickingComponent.LockPicks` (+ (`/Game/SplinterCellMain/Blueprints_Main/LockPicking/Blueprints/BP_LockPickingComponent.LockPicks` _returnvalue) (`self.LockpicksInBox`)) _returnvalue)
        (bind _foundwidgets (`WidgetBlueprintLibrary.GetAllWidgetsOfClass` "/Game/SplinterCellMain/Blueprints_Main/LockPicking/UserInterface/UI_LockpickingHUD.UI_LockpickingHUD_C"))
        (bind _output (`|GetArrayItem` _foundwidgets))
        (`TextBlock.SetText` (`/Game/SplinterCellMain/Blueprints_Main/LockPicking/UserInterface/UI_LockpickingHUD.NotificationText` _output) (`KismetTextLibrary.Conv_StringToText` (`KismetStringLibrary.Concat_StrStr` (`.OutKey` (`KismetTextLibrary.StringTableIdAndKeyFromText` "Collected")) " " (`KismetStringLibrary.Conv_IntToString` _lockpicksinbox) (select `bool` (> _lockpicksinbox 1) :`false` (`.OutKey` (`KismetTextLibrary.StringTableIdAndKeyFromText` "Lockpick")) :`true` (`.OutKey` (`KismetTextLibrary.StringTableIdAndKeyFromText` "Lockpicks"))) ".")))
        (`UserWidget.PlayAnimation` _output (`/Game/SplinterCellMain/Blueprints_Main/LockPicking/UserInterface/UI_LockpickingHUD.Notification` _output) 0.0 1 "Forward" 1.0 false)
        (`GameplayStatics.PlaySound2D` "/Game/SplinterCellMain/Blueprints_Main/LockPicking/Sound/Cues/SC_TakeLockpicks.SC_TakeLockpicks" 1.0 1.0 0.0 null null)
        (`self.K2_DestroyActor`)))))

(fn `UserConstructionScript`
  (if (`self.RandomInRange?`)
    (set `self.LockpicksInBox` (`KismetMathLibrary.RandomIntegerInRange` (`self.RangeMin`) (`self.RangeMax`)))))