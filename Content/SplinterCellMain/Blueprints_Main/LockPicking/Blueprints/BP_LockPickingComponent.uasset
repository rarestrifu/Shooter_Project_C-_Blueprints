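; BP_LockPickingComponent lets the player detect and pick locks on nearby objects.
; A looping timer sphere-traces ahead of the character, normally only when still, caching any BP_LockComponent and updating the lockpicking HUD, which also recognizes "LockpickBox"-tagged actors.
; CheckForLock reports unlocked objects or calls PickLock for locked ones.
; With picks available, PickLock disables input and spawns a BP_Lockpicking actor before the camera; otherwise it shows a notification.
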(event `self.ReceiveBeginPlay`
  ;[0.02315 0.2918 0.0137] Begin Play - Create HUD and Set Instance
  (bind _returnvalue (`|CreateWidget` "/Game/SplinterCellMain/Blueprints_Main/LockPicking/UserInterface/UI_LockpickingHUD.UI_LockpickingHUD_C"))
  (bind _output_get (set `self.LockInfoHUD` _returnvalue))
  (`UserWidget.AddToViewport` _output_get 0)
  (`KismetSystemLibrary.K2_SetTimerDelegate` (delegate `TraceForLock`) (`.TraceInterval_8_3019EE3249C2B2498BDADDBD4955AB28` (break `/Game/SplinterCellMain/Blueprints_Main/LockPicking/Blueprints/Core/Lockpicking_Settings` (`self.Settings`))) true))

(event `TraceForLock`
  (bind _returnvalue (`GameplayStatics.GetPlayerCharacter` 0))
  (bind _lockinfohud (`self.LockInfoHUD`))
  (bind _lockinfohud_2 (`self.LockInfoHUD`))
  (bind _returnvalue_2 (`Actor.K2_GetActorLocation` _returnvalue))
  ;[0.02315 0.2918 0.0137] Trace for a locked object
  (if (and (or (`KismetMathLibrary.NearlyEqual_FloatFloat` (`KismetMathLibrary.VSize` (`Actor.GetVelocity` (`self.GetOwner`))) 0.0 1.0) (`.TraceWhileMoving_5_6BC6CD0140C89C0A35B0A4B74214AD26` (break `/Game/SplinterCellMain/Blueprints_Main/LockPicking/Blueprints/Core/Lockpicking_Settings` (`self.Settings`)))) (not (`self.Busy`)))
    (`/Engine/EditorBlueprintResources/StandardMacros.IsValid` _returnvalue
      (:`Is Valid`
        (bind (_outhit _returnvalue_3) (`KismetSystemLibrary.SphereTraceSingle` _returnvalue_2 (+ _returnvalue_2 (* (`Actor.GetActorForwardVector` _returnvalue) 40.0)) 40.0 "TraceTypeQuery1" false (`|MakeArray` (`GameplayStatics.GetPlayerPawn` 0) :!type "Actor Object Reference")))
        (if _returnvalue_3
          (bind (_bblockinghit _binitialoverlap _time _distance _location _impactpoint _normal _impactnormal _physmat _hitactor) (`GameplayStatics.BreakHitResult` _outhit))
          (`/Engine/EditorBlueprintResources/StandardMacros.IsValid` _hitactor
            (:`Is Valid`
              (set `self.FocusedActor` _hitactor)
              (bind _returnvalue_4 (`Actor.GetComponentByClass` _hitactor "/Game/SplinterCellMain/Blueprints_Main/LockPicking/Blueprints/BP_LockComponent.BP_LockComponent_C"))
              (`/Engine/EditorBlueprintResources/StandardMacros.IsValid` _returnvalue_4
                (:`Is Valid`
                  (bind _output_get (set `self.Lock` _returnvalue_4))
                  (`/Game/SplinterCellMain/Blueprints_Main/LockPicking/Blueprints/BP_LockComponent.SetHUDInfo` _output_get (`self.LockInfoHUD`))
                  (set `/Game/SplinterCellMain/Blueprints_Main/LockPicking/UserInterface/UI_LockpickingHUD.Lockpicks` (`KismetTextLibrary.Conv_IntToText` (`self.LockPicks`)) _lockinfohud_2)
                  (set `/Game/SplinterCellMain/Blueprints_Main/LockPicking/UserInterface/UI_LockpickingHUD.InfoBoxVisible?` true _lockinfohud_2))
                (:`Is Not Valid`
                  (if (`Actor.ActorHasTag` _hitactor "LockpickBox")
                    (set `/Game/SplinterCellMain/Blueprints_Main/LockPicking/UserInterface/UI_LockpickingHUD.IsLocked?` false _lockinfohud)
                    (set `/Game/SplinterCellMain/Blueprints_Main/LockPicking/UserInterface/UI_LockpickingHUD.ObjectNameText` "LockpickBox" _lockinfohud)
                    (set `/Game/SplinterCellMain/Blueprints_Main/LockPicking/UserInterface/UI_LockpickingHUD.InfoBoxVisible?` true _lockinfohud)
                    (else
                      (set `self.Lock` null :!label _label)
                      (set `/Game/SplinterCellMain/Blueprints_Main/LockPicking/UserInterface/UI_LockpickingHUD.InfoBoxVisible?` false (`self.LockInfoHUD`)))))))
            (:`Is Not Valid`
              (set `self.FocusedActor` null :!label _label_2)
              (goto _label)))
          (else
            (goto _label_2)))))
    (else
      (goto _label_2))))

(event `PickLock`
  (bind _returnvalue (`GameplayStatics.GetPlayerCameraManager` 0))
  (bind _lockinfohud (`self.LockInfoHUD`))
  (bind _lock (`self.Lock`))
  ;[0.02315 0.2918 0.0137] Pick Lock
  ;[0.02315 0.2918 0.0137] Has enough lockpicks?
  (if (>= (`self.LockPicks`) 1)
    ;[0.02315 0.2918 0.0137] Disable Input and wait until player stands still
    (`Actor.DisableInput` (`Actor.GetInstigator` (`GameplayStatics.GetPlayerPawn` 0)) (`GameplayStatics.GetPlayerController` 0))
    (`KismetSystemLibrary.Delay` 0.5) ; Make sure Character is not moving anymore
    ;[0.02315 0.2918 0.0137] Spawn Lock in front of Character, set difficulty and object information
    (bind _returnvalue_2 (`|SpawnActorFromClass` "/Game/SplinterCellMain/Blueprints_Main/LockPicking/Blueprints/Core/BP_Lockpicking.BP_Lockpicking_C" (`KismetMathLibrary.MakeTransform` (+ (`PlayerCameraManager.GetCameraLocation` _returnvalue) (* (`Actor.GetActorForwardVector` _returnvalue) 40.0)) (`PlayerCameraManager.GetCameraRotation` _returnvalue)) "AlwaysSpawn" "OverrideRootScale" null null))
    (set `/Game/SplinterCellMain/Blueprints_Main/LockPicking/Blueprints/Core/BP_Lockpicking.LockPickingComponent` self _returnvalue_2)
    (set `/Game/SplinterCellMain/Blueprints_Main/LockPicking/Blueprints/Core/BP_Lockpicking.LockedObject` _lock _returnvalue_2)
    (`/Game/SplinterCellMain/Blueprints_Main/LockPicking/Blueprints/Core/BP_Lockpicking.LockSetup` _returnvalue_2 (`/Game/SplinterCellMain/Blueprints_Main/LockPicking/Blueprints/BP_LockComponent.LockDifficulty` _lock))
    (set `self.Busy` true)
    (else
      ;[0.02315 0.2918 0.0137] Show no lockpicks notification
      (`TextBlock.SetText` (`/Game/SplinterCellMain/Blueprints_Main/LockPicking/UserInterface/UI_LockpickingHUD.NotificationText` (`self.LockInfoHUD`)) "You don't have lockpicks left.")
      (`UserWidget.PlayAnimation` _lockinfohud (`/Game/SplinterCellMain/Blueprints_Main/LockPicking/UserInterface/UI_LockpickingHUD.Notification` _lockinfohud) 0.0 1 "Forward" 1.0 false))))

(fn `CheckForLock`
  (returns (Unlocked :type Boolean) (LockedActor :type "Actor Object Reference"))
  (bind _lock (`self.Lock`))
  (`self.Lock`
    (:`then`
      (if (`/Game/SplinterCellMain/Blueprints_Main/LockPicking/Blueprints/BP_LockComponent.Locked?` _lock)
        (`self.PickLock`)
        (return false null)
        (else
          (return true (`self.GetOwner` _lock)))))
    (:`else`
      (return false null))))