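; Drone landing pad actor with blinking side lights.
; On BeginPlay a timeline plays from the start and outputs an Emissive value on each update.
; That one value drives both the mesh material's side-light emissive parameter and the intensity of five point lights, keeping glow and lighting in sync.
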(event `self.ReceiveBeginPlay`
  (bind (_direction _emissive) (`Timeline|Timeline_blinking_lights` :!via `PlayFromStart`)
    (:`Update`
      (`MeshComponent.SetScalarParameterValueOnMaterials` (`self.StaticMesh`) "Emissive_Side_lights" (* _emissive 1.0))
      (`LightComponent.SetIntensity` (`self.PointLight1`) (* _emissive 1.0))
      (`LightComponent.SetIntensity` (`self.PointLight2`) (* _emissive 1.0))
      (`LightComponent.SetIntensity` (`self.PointLight3`) (* _emissive 1.0))
      (`LightComponent.SetIntensity` (`self.PointLight`) (* _emissive 1.0))
      (`LightComponent.SetIntensity` (`self.PointLight4`) (* _emissive 1.0)))))

(fn `UserConstructionScript`)