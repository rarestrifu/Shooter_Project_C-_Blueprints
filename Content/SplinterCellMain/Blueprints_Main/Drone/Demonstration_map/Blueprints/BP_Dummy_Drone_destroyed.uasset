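; Destroyed drone wreck actor that plays a physics-driven explosion and burn-out, then removes itself.
; BeginPlay and CE_Destroy_Wreck share a one-shot sequence, gated by WreckDestroyed.
; It spawns explosion effects, wakes the skeletal body's physics with randomized radial force, impulse and per-wing spin, and activates fire particles and sound.
; Timed delays fade the fire, then hide the mesh, spawn a final explosion and destroy the actor.
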(event `self.ReceiveTick`
  (params (DeltaSeconds :type "Float (single-precision)"))
  ;[1 0 0] No tick functions :) ( Tick is disabled in blueprint if needed enable it first )
)

(event `CE_Destroy_Wreck`
  (bind _body (`self.Body`))
  (bind _body_2 (`self.Body`))
  (bind _body_3 (`self.Body`))
  (bind _body_4 (`self.Body`))
  (bind _body_5 (`self.Body`))
  (bind _cs_fire_burning (`self.CS_Fire_burning`))
  (bind _returnvalue (`SceneComponent.K2_GetComponentRotation` _body_3))
  (bind _returnvalue_2 (* (`KismetMathLibrary.GetUpVector` _returnvalue) (`KismetMathLibrary.RandomFloatInRange` -5.0 5.0)))
  ;[1 1 1] Wake rigid bodes and add some force to them
  (if (`self.Wreck_destroyed_?`) :!label _label
    (`/Engine/EditorBlueprintResources/StandardMacros.DoOnce` false
      (:`Completed`
        (`GameplayStatics.SpawnEmitterAttached` "/Game/SplinterCellMain/Blueprints_Main/Drone/Particles/PS_Generic_4x4_explosion_Small.PS_Generic_4x4_explosion_Small" _body_4 "SK_Dummy_Drone_Destroyed")
        (`GameplayStatics.SpawnSoundAtLocation` null (`SceneComponent.K2_GetComponentLocation` _body_4) (struct) 1.0 1.0 0.0 null null)
        (`SkeletalMeshComponent.SetAllBodiesSimulatePhysics` _body_2 true)
        (`PrimitiveComponent.WakeAllRigidBodies` _body_2)
        (`PrimitiveComponent.AddRadialForce` _body_3 (`self.K2_GetActorLocation`) 250.0 (`KismetMathLibrary.RandomFloatInRange` 30000.0 15000.0) "RIF_Constant" true)
        (`PrimitiveComponent.AddImpulse` (`self.Body`) (* (`KismetMathLibrary.GetForwardVector` _returnvalue) (`KismetMathLibrary.RandomFloatInRange` 2000.0 3000.0)) "None" true)
        (`PrimitiveComponent.AddAngularImpulseInRadians` _body _returnvalue_2 "Wing_R" true)
        (`PrimitiveComponent.AddAngularImpulseInRadians` _body _returnvalue_2 "Wing_L" true)
        ;[1 1 1] Play primary PS effect, and play fire and explosion sound
        (`ActorComponent.SetActive` _cs_fire_burning true false)
        (`ActorComponent.SetActive` (`self.PS_Fire_Wing_R`) true false)
        (`ActorComponent.SetActive` (`self.PS_Fire_Rear`) true false)
        (`ActorComponent.SetActive` (`self.PS_Fire_Wing_L`) true false)
        (`KismetSystemLibrary.Delay` 2.0) ; Change this to control how long PS effect will be played
        (`AudioComponent.FadeOut` _cs_fire_burning 2.0 0.0 "Linear")
        (`ActorComponent.SetActive` (`self.PS_Fire_Wing_L`) false false)
        (`ActorComponent.SetActive` (`self.PS_Fire_Rear`) false false)
        (`ActorComponent.SetActive` (`self.PS_Fire_Wing_R`) false false)
        ;[1 1 1] Hide destroyed mesh, and play final PS effect
        (`KismetSystemLibrary.Delay` 2.0) ; Change this to control how long destroyed mesh will be visible in game ( Be aware that particle life is allso calculated )
        (`SceneComponent.SetVisibility` _body_5 false false)
        (`GameplayStatics.SpawnEmitterAtLocation` "/Game/SplinterCellMain/Blueprints_Main/Drone/Particles/PS_ExplosionEnd.PS_ExplosionEnd" (`SceneComponent.K2_GetComponentLocation` _body_5))
        (`self.K2_DestroyActor`)))))

(event `self.ReceiveBeginPlay`
  ;[1 1 1] Wake rigid bodes and add some force to them
  (goto _label))

(fn `UserConstructionScript`)