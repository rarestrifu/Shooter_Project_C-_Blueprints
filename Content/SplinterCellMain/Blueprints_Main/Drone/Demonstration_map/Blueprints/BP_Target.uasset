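; BP_Target is a shooting target in the drone demonstration map that tips over when hit and can optionally stand back up and move along a spline.
; A hit, gated by DoOnce, plays a metal impact sound and a timeline pitches the target horizontal.
; After a delay, an optional reset timeline raises it and re-arms the gate.
; When movement is enabled, Tick restarts a spline-position timeline whenever the clamped Speed value equals 1.
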(event `self.SM_Target.OnComponentHit`
  (params (HitComponent :type "PrimitiveComponent Object Reference") (OtherActor :type "Actor Object Reference") (OtherComp :type "PrimitiveComponent Object Reference") (NormalImpulse :type "Vector Structure") (Hit :type "HitResult Structure (by ref)"))
  ;[1 1 1] Event when target is hit, and when to reset target
  (`/Engine/EditorBlueprintResources/StandardMacros.DoOnce` false :!label _label
    (:`Completed`
      (`GameplayStatics.PlaySoundAtLocation` "/Game/SplinterCellMain/Blueprints_Main/Drone/Demonstration_map/Sounds/Cues/SC_impact_metal_Cue.SC_impact_metal_Cue" (`SceneComponent.K2_GetComponentLocation` (`self.SM_Target_Base`)) (struct) 1.0 1.0 0.0 "/Game/SplinterCellMain/Blueprints_Main/Drone/Sounds/ATT_Engine.ATT_Engine" null null)
      (bind (_direction _target) (`Timeline|Timeline if target is hit set it to horizontal position` :!via `PlayFromStart`)
        (:`Update`
          (`SceneComponent.K2_SetRelativeRotation` (`self.SM_Target`) (`KismetMathLibrary.MakeRotator` 0.0 _target) false false)
          (set `self.Target_hit` true)
          (`KismetSystemLibrary.Delay` (`self.Delay to reset target`))
          (if (`self.Target ressets ?`)
            (bind (_direction_2 _target_2) (`Timeline|Timeline reset target set it to vertical position` :!via `PlayFromStart`)
              (:`Update`
                (`SceneComponent.K2_SetRelativeRotation` (`self.SM_Target`) (`KismetMathLibrary.MakeRotator` 0.0 _target_2) false false)
                (set `self.Target_hit` false))
              (:`Finished`
                (goto _label :!via `Reset`)))))))))

(event `self.ReceiveTick`
  (params (DeltaSeconds :type "Float (single-precision)"))
  (bind _sm_target_base (`self.SM_Target_Base`))
  (bind _spline (`self.Spline`))
  ;[1 0 0] How fast is target moving
  (if (and (`self.Moving target ?`) (== (`self.Speed`) 1.0))
    (bind (_direction _target_moving) (`Timeline|Timelin how fast target is moving multiply by float` :!via `PlayFromStart`)
      (:`Update`
        (bind _returnvalue (* _target_moving (`self.How fast target is moving ?`)))
        (set `self.Speed` (`KismetMathLibrary.FClamp` (`KismetMathLibrary.Abs` _returnvalue)))
        (`SceneComponent.K2_SetWorldTransform` _sm_target_base (`KismetMathLibrary.MakeTransform` (`SplineComponent.GetLocationAtDistanceAlongSpline` _spline (* _returnvalue (`SplineComponent.GetSplineLength` _spline)) "World") (`SceneComponent.K2_GetComponentRotation` _sm_target_base)) false false)))))

(fn `UserConstructionScript`)