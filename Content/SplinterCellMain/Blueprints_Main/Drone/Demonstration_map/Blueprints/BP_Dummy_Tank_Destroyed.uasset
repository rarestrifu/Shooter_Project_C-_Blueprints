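; Destroyed wreck of a dummy tank that explodes on BeginPlay or CE_Destroy_Wreck, if WreckDestroyed is set, then cleans itself up.
; A one-shot explosion wakes body physics and randomly either launches the skeletal Turret bone or hides it and throws the separate SMTurret mesh.
; The matching hull or turret effect plays with burning audio on timed delays, then the meshes hide, end effects spawn and the actor is destroyed.
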(event `self.ReceiveTick`
  (params (DeltaSeconds :type "Float (single-precision)"))
  ;[1 0 0] No tick functions :) ( Tick is disabled in blueprint if needed enable it first )
)

(event `CE_Destroy_Wreck`
  (bind _body (`self.Body`))
  (bind _body_2 (`self.Body`))
  (bind _body_3 (`self.Body`))
  (bind _body_4 (`self.Body`))
  (bind _cs_fire_burning (`self.CS_Fire_burning`))
  (bind _sm_turret (`self.SM_Turret`))
  (bind _body_5 (`self.Body`))
  (bind _returnvalue (* (`KismetMathLibrary.GetRightVector` (`SceneComponent.K2_GetComponentRotation` (`self.Body`))) (`KismetMathLibrary.RandomFloatInRange` 5.0 15.0)))
  ;[1 1 1] Wake rigid bodes and add some force to them
  (if (`self.Wreck_destroyed_?`) :!label _label
    (`/Engine/EditorBlueprintResources/StandardMacros.DoOnce` false
      (:`Completed`
        (`GameplayStatics.SpawnEmitterAttached` "/Game/SplinterCellMain/Blueprints_Main/Drone/Particles/PS_Generic_4x4_explosion_Small.PS_Generic_4x4_explosion_Small" _body_3 "Root")
        (`GameplayStatics.SpawnSoundAtLocation` null (`SceneComponent.K2_GetComponentLocation` _body_3) (struct) 1.0 1.0 0.0 null null)
        (`SkeletalMeshComponent.SetAllBodiesSimulatePhysics` _body_2 true)
        (`PrimitiveComponent.WakeAllRigidBodies` _body_2)
        (if (`KismetMathLibrary.RandomBool`)
          ;[1 1 1] Nodes controling adding impulse to turret bone
          (`PrimitiveComponent.AddImpulse` _body (+ (* (`KismetMathLibrary.Normal` (`self.GetActorForwardVector`)) (800.0 800.0 0.0)) (* (`KismetMathLibrary.Normal` (`self.GetActorUpVector`)) (0.0 0.0 1200.0))) "Turret" true)
          (`PrimitiveComponent.AddAngularImpulseInRadians` _body _returnvalue "Turret" true)
          (`SkinnedMeshComponent.HideBoneByName` _body "Hatch" "PBO_None")
          (`ActorComponent.SetActive` (`self.PS_Turret`) true false)
          ;[1 1 1] Play primary PS effect, and play fire and explosion sound
          (`ActorComponent.SetActive` _cs_fire_burning true false :!label _label_2)
          (`KismetSystemLibrary.Delay` 19.0) ; Change this to control how long PS effect will be played
          (`AudioComponent.FadeOut` _cs_fire_burning 2.0 0.0 "Linear")
          (`ActorComponent.SetActive` (`self.PS_Hull`) false false)
          (`ActorComponent.SetActive` null false false)
          (`ActorComponent.SetActive` (`self.PS_Turret`) false false)
          ;[1 1 1] Hide destroyed mesh, and play final PS effect
          (`KismetSystemLibrary.Delay` 10.0) ; Change this to control how long destroyed mesh will be visible in game ( Be aware that particle life is allso calculated )
          (`SceneComponent.SetVisibility` _body_4 false false)
          (`SceneComponent.SetVisibility` (`self.SM_Turret`) false false)
          (`GameplayStatics.SpawnEmitterAtLocation` "/Game/SplinterCellMain/Blueprints_Main/Drone/Particles/PS_ExplosionEnd.PS_ExplosionEnd" (`SceneComponent.K2_GetComponentLocation` _body_4))
          (if (`self.bSM_Turret_Visible`)
            (`GameplayStatics.SpawnEmitterAtLocation` "/Game/SplinterCellMain/Blueprints_Main/Drone/Particles/PS_ExplosionEnd.PS_ExplosionEnd" (`SceneComponent.K2_GetComponentLocation` (`self.SM_Turret`))))
          (`self.K2_DestroyActor`)
          (else
            ;[1 1 1] Nodes controling turret decapitation
            (`PrimitiveComponent.SetCollisionEnabled` _sm_turret "QueryAndPhysics")
            (`PrimitiveComponent.SetSimulatePhysics` _sm_turret true)
            (`PrimitiveComponent.AddImpulse` _sm_turret (+ (* (`KismetMathLibrary.Normal` (`self.GetActorForwardVector`)) (800.0 800.0 0.0)) (* (`KismetMathLibrary.Normal` (`self.GetActorUpVector`)) (0.0 0.0 1200.0))) "None" true)
            (`PrimitiveComponent.AddAngularImpulseInRadians` _sm_turret _returnvalue "None" true)
            (`SceneComponent.SetVisibility` _sm_turret true false)
            (`SkinnedMeshComponent.HideBoneByName` _body_5 "Turret" "PBO_None")
            (`SkinnedMeshComponent.HideBoneByName` _body_5 "Gun" "PBO_None")
            (`ActorComponent.SetActive` (`self.PS_Hull`) true false)
            (`|ExecutionSequence`
              (:`then_0`
                (set `self.bSM_Turret_Visible` true)
                (goto _label_2))
              (:`then_1`
                (`KismetSystemLibrary.Delay` 1.0)
                (`PrimitiveComponent.SetCollisionResponseToAllChannels` (`self.SM_Turret`) "ECR_Block")))))))))

(event `self.ReceiveBeginPlay`
  ;[1 1 1] Wake rigid bodes and add some force to them
  (goto _label))

(fn `UserConstructionScript`)