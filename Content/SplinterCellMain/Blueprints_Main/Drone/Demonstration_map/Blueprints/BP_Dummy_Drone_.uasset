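; BP_Dummy_Drone is a damageable demonstration target drone that spawns its own BP_Dummy_Drone_Spline and hands it a reference and movement speed.
; Timelines drive engine rotation, optional sensor pitch, and red/green lights.
; A looping timer, used instead of Tick, rotates the 3P health widget toward the player, scales and hides it by distance, and updates its bar.
; Damage lowers health, triggers smoke when low, and swaps in a wreck actor at zero.
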(event `CE 3p_health_widget_rotate`
  (bind _scene (`self.Scene`))
  (bind _distance_needed_t_hide_3p_widget (`self.Distance_Needed_T_Hide_3p_Widget`))
  (bind _health_dummy_drone (`self.Health_Dummy_Drone`))
  (bind _returnvalue (`SceneComponent.K2_GetComponentLocation` _scene))
  (bind _returnvalue_2 (`self.K2_GetActorLocation` (`GameplayStatics.GetPlayerPawn` 0)))
  (bind _yaw (.yaw (`KismetMathLibrary.FindLookAtRotation` _returnvalue _returnvalue_2)))
  (bind _returnvalue_3 (`KismetMathLibrary.Abs` (/ (`KismetMathLibrary.GetPointDistanceToLine` _returnvalue_2 _returnvalue (`KismetMathLibrary.Conv_DoubleToVector` _yaw)) 100.0)))
  ;[0 0.2431 0.2471] Nodes controling T_A_Bar_3P widget and orientate it to player
  (if (not (`self.Hide_3P_Health_Widget`))
    (`/Engine/EditorBlueprintResources/StandardMacros.IsValid` (`GameplayStatics.GetPlayerPawn` 0)
      (:`Is Valid`
        (`KismetSystemLibrary.K2_SetTimerDelegate` (delegate `CE 3p_health_widget_rotate`) 0.025 true)
        (`/Engine/EditorBlueprintResources/StandardMacros.CompareFloat` _returnvalue_3 _distance_needed_t_hide_3p_widget
          (:`>`
            (`SceneComponent.SetHiddenInGame` _scene true true))
          (:`<`
            (`SceneComponent.SetHiddenInGame` _scene false true)))
        (`SceneComponent.SetWorldScale3D` _scene (`KismetMathLibrary.Conv_DoubleToVector` (`KismetMathLibrary.FClamp` (`KismetMathLibrary.NormalizeToRange` _returnvalue_3 0.0 _distance_needed_t_hide_3p_widget) 0.5 2.0)))
        (`SceneComponent.K2_SetWorldRotation` _scene (`KismetMathLibrary.MakeRotator` 0.0 0.0 _yaw) false false)
        (bind _asumg_dummy_drone_3p_health_widget (cast `/Game/SplinterCellMain/Blueprints_Main/Drone/Demonstration_map/Ui/UMG_Dummy_Drone_3P_health_Widget` (`WidgetComponent.GetUserWidgetObject` (`self.Widget_3P_Health`))))
        (bind _healthbar (`/Game/SplinterCellMain/Blueprints_Main/Drone/Demonstration_map/Ui/UMG_Dummy_Drone_3P_health_Widget.HealthBar` _asumg_dummy_drone_3p_health_widget))
        (`ProgressBar.SetPercent` _healthbar (/ _health_dummy_drone 100.0))
        (`/Engine/EditorBlueprintResources/StandardMacros.CompareFloat` _health_dummy_drone 30.0
          (:`>`
            (bind _output_get (set `/Game/SplinterCellMain/Blueprints_Main/Drone/Demonstration_map/Ui/UMG_Dummy_Drone_3P_health_Widget.HealthBar` _healthbar _asumg_dummy_drone_3p_health_widget :!label _label))
            (`ProgressBar.SetFillColorAndOpacity` _output_get (struct :`G` 1.0 :`A` 1.0)))
          (:`==`
            (goto _label))
          (:`<`
            (bind _output_get_2 (set `/Game/SplinterCellMain/Blueprints_Main/Drone/Demonstration_map/Ui/UMG_Dummy_Drone_3P_health_Widget.HealthBar` _healthbar _asumg_dummy_drone_3p_health_widget))
            (`ProgressBar.SetFillColorAndOpacity` _output_get_2 (struct :`R` 1.0 :`A` 1.0))))))))

(event `self.ReceiveBeginPlay`
  (bind _emissive (`self.Emissive`))
  (bind _skeletalmesh (`self.SkeletalMesh`))
  (`|ExecutionSequence`
    (:`then_0`
      ;[1 1 1] Sensors and engine rotation
      (bind (_direction _engine) (`Timeline|Timeline_engine_rotation` :!via `PlayFromStart`)
        (:`Update`
          (set `self.Engine_BP` _engine))))
    (:`then_1`
      ;[1 1 1] Lights
      (bind (_direction_2 _emissive_red _light_red) (`Timeline|Timeline_RED_Lights` :!via `PlayFromStart`)
        (:`Update`
          (`MaterialInstanceDynamic.SetScalarParameterValue` _emissive "Emissive_power_RED" _emissive_red)
          (`LightComponent.SetIntensity` (`self.Pintlight_RED`) _light_red)
          (`LightComponent.SetIntensity` (`self.PointLight_Tail_L`) _light_red)
          (`LightComponent.SetIntensity` (`self.PointLight_Tail_R`) _light_red)
          (`LightComponent.SetIntensity` (`self.PointLight_Wing_R`) _light_red)
          (`LightComponent.SetIntensity` (`self.PointLight_Wing_L`) _light_red)
          (`LightComponent.SetIntensity` (`self.PointLight_Tail_Botom`) _light_red)
          (`MaterialInstanceDynamic.SetScalarParameterValue` _emissive "Emissive_power_GREEN" (/ _emissive_red 2.0)))))
    (:`then_2`
      (if (`self.Use_moving_sensors_?`)
        (bind (_direction_3 _sensors_pitch) (`Timeline|Sensors` :!via `PlayFromStart`)
          (:`Update`
            (set `self.Sensors_pitch_BP` _sensors_pitch)))))
    (:`then_3`
      ;[1 1 1] Add spline
      (`/Engine/EditorBlueprintResources/StandardMacros.IsValid` _skeletalmesh
        (:`Is Valid`
          (bind _returnvalue (`|SpawnActorFromClass` "/Game/SplinterCellMain/Blueprints_Main/Drone/Demonstration_map/Blueprints/BP_Dummy_Drone_Spline.BP_Dummy_Drone_Spline_C" (`SceneComponent.K2_GetComponentToWorld` _skeletalmesh) "Undefined" "OverrideRootScale" null null))
          (bind _output_get (set `/Game/SplinterCellMain/Blueprints_Main/Drone/Demonstration_map/Blueprints/BP_Dummy_Drone_Spline.Actor_BP_Dummy_drone` self _returnvalue))
          (set `/Game/SplinterCellMain/Blueprints_Main/Drone/Demonstration_map/Blueprints/BP_Dummy_Drone_Spline.How fast target is moving ?` (`self.How fast target is moving ?`) _returnvalue))))
    (:`then_4`
      (`self.CE 3p_health_widget_rotate`))))

(event `self.ReceiveTick`
  (params (DeltaSeconds :type "Float (single-precision)"))
  ;[1 0 0] No tick functions :) ( Tick is disabled in blueprint if needed enable it first )
)

(event `self.ReceiveAnyDamage`
  (params (Damage :type "Float (single-precision)") (DamageType :type "DamageType Object Reference") (InstigatedBy :type "Controller Object Reference") (DamageCauser :type "Actor Object Reference"))
  (bind _skeletalmesh (`self.SkeletalMesh`))
  (bind _ps_missle_smoke (`self.PS_Missle_Smoke`))
  ;[1 0.8824 0] Nodes controling damage system ( how many health points is subtracted when vehicle is hit with damage )
  (if (`self.Can_be_Damaged_?`)
    (set `self.Damage` Damage)
    (set `self.Taking_damage_?` true)
    (`|ExecutionSequence`
      (:`then_0`
        (`KismetSystemLibrary.RetriggerableDelay` (`self.Health_refresh_cooldown`))
        (set `self.Taking_damage_?` false))
      (:`then_1`
        (set `self.Health_Dummy_Drone` (- (`self.Health_Dummy_Drone`) (`self.Damage`)))
        (`ActorComponent.Deactivate` _ps_missle_smoke)
        (if (<= (`self.Health_Dummy_Drone`) 0.0)
          (`/Engine/EditorBlueprintResources/StandardMacros.DoOnce` false
            (:`Completed`
              (bind _returnvalue (`|SpawnActorFromClass` "/Game/SplinterCellMain/Blueprints_Main/Drone/Demonstration_map/Blueprints/BP_Dummy_Drone_destroyed.BP_Dummy_Drone_destroyed_C" (`self.GetTransform`) "Undefined" "OverrideRootScale" null null))
              (`/Game/SplinterCellMain/Blueprints_Main/Drone/Demonstration_map/Blueprints/BP_Dummy_Drone_destroyed.CE_Destroy_Wreck` _returnvalue)
              (set `/Game/SplinterCellMain/Blueprints_Main/Drone/Demonstration_map/Blueprints/BP_Dummy_Drone_destroyed.Wreck_destroyed_?` true _returnvalue)
              (`PrimitiveComponent.SetCollisionResponseToAllChannels` _skeletalmesh "ECR_Ignore")
              (`PrimitiveComponent.SetCollisionEnabled` _skeletalmesh "PhysicsOnly")
              (`PrimitiveComponent.SetSimulatePhysics` _skeletalmesh false)
              (`SceneComponent.SetVisibility` _skeletalmesh false false)
              (`KismetSystemLibrary.Delay` 0.1)
              (`self.K2_DestroyActor` (stale `self.ReceiveBeginPlay` _output_get))
              (`self.K2_DestroyActor`)))))
      (:`then_2`
        (`/Engine/EditorBlueprintResources/StandardMacros.CompareFloat` (`self.Health_Dummy_Drone`) 40.0
          (:`<`
            (`/Engine/EditorBlueprintResources/StandardMacros.DoOnce` false
              (:`Completed`
                (`ActorComponent.Activate` _ps_missle_smoke false)))))))))

(fn `UserConstructionScript`
  (bind _widget_3p_health (`self.Widget_3P_Health`))
  (`|ExecutionSequence`
    (:`then_0`
      (bind _returnvalue (`PrimitiveComponent.CreateDynamicMaterialInstance` (`self.SkeletalMesh`) 0 null "None"))
      (set `self.Emissive` _returnvalue))
    (:`then_1`
      ;[1 1 1] Hide_3P_Health_widget
      (if (`self.Hide_3P_Health_Widget`)
        (`SceneComponent.SetVisibility` _widget_3p_health false false)
        (else
          (`SceneComponent.SetVisibility` _widget_3p_health true false))))))