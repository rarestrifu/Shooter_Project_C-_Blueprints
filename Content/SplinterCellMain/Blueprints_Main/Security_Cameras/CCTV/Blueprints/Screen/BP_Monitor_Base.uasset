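; BP_Monitor_Base is a CCTV monitor actor that shows the live view of an assigned security camera.
; Construction creates a render target and dynamic screen material, applies look settings like grayscale, scanlines, overlay and noise, then feeds the camera's SceneCapture2D into it.
; Updatemonitor shows the broken effect and destroys the capture component when that camera is broken.
; A removable debug toggle enables Tick to draw a line to the linked camera.
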(event `Toggle debug`
  ;[0.9798 0.02567 1] Debug (Can be deleted)
  (bind _output_get (set `self.Debug on?` (not (`self.Debug on?`))))
  (`self.SetActorTickEnabled` _output_get))

(event `self.ReceiveTick`
  (params (DeltaSeconds :type "Float (single-precision)"))
  ;[0.9798 0.02567 1] Debug (Can be deleted)
  (`KismetSystemLibrary.DrawDebugLine` (`self.K2_GetActorLocation`) (`self.K2_GetActorLocation` (`self.Camera to display`)) (struct :`R` 1.0 :`G` 1.0 :`B` 1.0 :`A` 1.0) 0.0 1.0))

(event `Update monitor`
  (bind _camera_to_display (`self.Camera to display`))
  ;[0 0 0] Display noise when camera is broken
  (`/Engine/EditorBlueprintResources/StandardMacros.IsValid` _camera_to_display
    (:`Is Valid`
      (if (`/Game/SplinterCellMain/Blueprints_Main/Security_Cameras/CCTV/Blueprints/Camera/BP_Camera_Base.Camera broken?` _camera_to_display)
        (`MaterialInstanceDynamic.SetScalarParameterValue` (`self.Screen Material`) "Broken Amount" 1.0)
        (`ActorComponent.K2_DestroyComponent` (`/Game/SplinterCellMain/Blueprints_Main/Security_Cameras/CCTV/Blueprints/Camera/BP_Camera_Base.SceneCaptureComponent2D` _camera_to_display))))))

(fn `UserConstructionScript`
  (bind _screen_material (`self.Screen Material`))
  (bind (_resx _resy) (break `CaptureResolution` (`self.Resolution`)))
  (bind _scenecapturecomponent2d (`/Game/SplinterCellMain/Blueprints_Main/Security_Cameras/CCTV/Blueprints/Camera/BP_Camera_Base.SceneCaptureComponent2D` (`self.Camera to display`)))
  (bind _returnvalue (`KismetRenderingLibrary.CreateRenderTarget2D` _resx _resy))
  (set `self.Screen Texture` _returnvalue)
  (bind _returnvalue_2 (`KismetMaterialLibrary.CreateDynamicMaterialInstance` "/Game/SplinterCellMain/Blueprints_Main/Security_Cameras/CCTV/Demo/Materials/Screen/M_Screen.M_Screen"))
  (bind _output_get (set `self.Screen Material` _returnvalue_2))
  (`PrimitiveComponent.SetMaterial` (`self.Screen mesh`) (`self.Screen Material Index`) _output_get)
  (`MaterialInstanceDynamic.SetTextureParameterValue` (`self.Screen Material`) "CameraView" (`self.Screen Texture`))
  (`MaterialInstanceDynamic.SetScalarParameterValue` _screen_material "Grayscale" (`KismetMathLibrary.SelectFloat` 0.0 1.0 (`self.Colors?`)))
  (`MaterialInstanceDynamic.SetScalarParameterValue` _screen_material "Scanlines amount" (`self.Scanlines Opacity`))
  (`MaterialInstanceDynamic.SetScalarParameterValue` _screen_material "Overlay amount" (`self.Overlay Opacity`))
  (`MaterialInstanceDynamic.SetScalarParameterValue` _screen_material "Zoom" (`self.Noise amount`))
  (`MaterialInstanceDynamic.SetScalarParameterValue` _screen_material "Noise" (`self.Noise amount`))
  (`MaterialInstanceDynamic.SetTextureParameterValue` (`self.Screen Material`) "Overlay" (`self.Texture overlay`))
  (set `SceneCaptureComponent2D.FOVAngle` (`self.FOV`) _scenecapturecomponent2d)
  (set `SceneCaptureComponent2D.TextureTarget` (`self.Screen Texture`) _scenecapturecomponent2d))