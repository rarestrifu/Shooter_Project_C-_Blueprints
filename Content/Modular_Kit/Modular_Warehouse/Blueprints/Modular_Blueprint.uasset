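; Modular warehouse builder Blueprint that assembles a run of walls, windows and door frames, one piece per event.
; AddMesh places each piece at the previous "End" socket, records type and transforms in StaticMeshArrays, and spawns door actors at "Door" sockets.
; The construction script rebuilds components from that array, applies the warehouse material and reattaches doors.
; DeleteLastComponent removes the newest piece and any door it has.
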(event `Wall Side Inside`
  ;[1 0.8556 0.2125] Wall Sides
  (`self.AddMesh` "NewEnumerator8"))

(event `Wall Large`
  ;[0.2125 0.5081 1] Walls
  (`self.AddMesh` "NewEnumerator0"))

(event `Door`
  ;[0.2125 1 0.6325] Doors
  (`self.AddMesh` "NewEnumerator4"))

(event `Wall Side outside`
  ;[1 0.8556 0.2125] Wall Sides
  (`self.AddMesh` "NewEnumerator9"))

(event `Door Garage`
  ;[0.2125 1 0.6325] Doors
  (`self.AddMesh` "NewEnumerator5"))

(event `Wall Medium`
  ;[0.2125 0.5081 1] Walls
  (`self.AddMesh` "NewEnumerator1"))

(event `Door Double`
  ;[0.2125 1 0.6325] Doors
  (`self.AddMesh` "NewEnumerator10"))

(event `Wall Small`
  ;[0.2125 0.5081 1] Walls
  (`self.AddMesh` "NewEnumerator2"))

(event `Window`
  ;[1 0.2125 0.2518] Wall Sides
  (`self.AddMesh` "NewEnumerator6"))

(event `Wall Small Extra`
  ;[0.2125 0.5081 1] Walls
  (`self.AddMesh` "NewEnumerator3"))

(event `Window Small`
  ;[1 0.2125 0.2518] Wall Sides
  (`self.AddMesh` "NewEnumerator7"))

(event `Delete Last`
  ;[0.2125 1 0.6325] Doors
  (`self.Delete_Last_Component`))

(event `Wall Small Extra 2`
  ;[0.2125 0.5081 1] Walls
  (`self.AddMesh` "NewEnumerator11"))

(fn `AddMesh`
  (params (Mesh :type "/Game/Modular_Kit/Modular_Warehouse/Blueprints/Data/MeshType Enum" :default "NewEnumerator0"))
  (bind (_static_mesh _door) (`self.Get_StaticMesh` Mesh))
  (bind _static_mesh_arrays (`self.Static_Mesh_Arrays`))
  (bind _returnvalue (`KismetSystemLibrary.IsValidClass` _door))
  (bind (_output_previoustransform _output_type _output_myendpoint) (break `/Game/Modular_Kit/Modular_Warehouse/Blueprints/Data/StaticMesh_Struct` (`|GetArrayItem` _static_mesh_arrays (`KismetArrayLibrary.Array_LastIndex` _static_mesh_arrays))))
  (bind _returnvalue_2 (select `bool` (> (`KismetArrayLibrary.Array_Length` (`self.Static_Mesh_Arrays`)) 0) :`true` _output_myendpoint))
  (bind _returnvalue_3 (`AddComponent|NODE_AddStaticMeshComponent-0` :`RelativeTransform` _returnvalue_2))
  (`StaticMeshComponent.SetStaticMesh` _returnvalue_3 _static_mesh)
  (`KismetArrayLibrary.Array_Add` (`self.Static Meshes`) _returnvalue_3)
  (`KismetArrayLibrary.Array_Add` (`self.Static_Mesh_Arrays`) (make `/Game/Modular_Kit/Modular_Warehouse/Blueprints/Data/StaticMesh_Struct` _returnvalue_2 Mesh (`SceneComponent.GetSocketTransform` _returnvalue_3 "End" "RTS_Actor") _returnvalue))
  (if _returnvalue
    (bind _returnvalue_4 (`|SpawnActorFromClass` _door (`SceneComponent.GetSocketTransform` _returnvalue_3 "Door" "RTS_World") "Undefined" "OverrideRootScale" null null))
    (`KismetArrayLibrary.Array_Add` (`self.Doors_Array`) _returnvalue_4)))

(fn `Delete_Last_Component`
  (bind _static_mesh_arrays (`self.Static_Mesh_Arrays`))
  (bind _static_meshes (`self.Static Meshes`))
  (bind _static_mesh_arrays_2 (`self.Static_Mesh_Arrays`))
  (bind _doors_array (`self.Doors_Array`))
  (bind _returnvalue (`KismetArrayLibrary.Array_LastIndex` _static_meshes))
  (bind _returnvalue_2 (`KismetArrayLibrary.Array_LastIndex` _doors_array))
  (if (> (`KismetArrayLibrary.Array_Length` (`self.Static_Mesh_Arrays`)) 0)
    (if (`.HasDoor?_7_F1A150C945196248DD90FDAB1317C3BA` (break `/Game/Modular_Kit/Modular_Warehouse/Blueprints/Data/StaticMesh_Struct` (`|GetArrayItem` _static_mesh_arrays (`KismetArrayLibrary.Array_LastIndex` _static_mesh_arrays))))
      (`self.K2_DestroyActor` (`|GetArrayItem` _doors_array _returnvalue_2))
      (`KismetArrayLibrary.Array_Remove` _doors_array _returnvalue_2))
    (`ActorComponent.K2_DestroyComponent` (`|GetArrayItem` _static_meshes _returnvalue))
    (`KismetArrayLibrary.Array_Remove` _static_meshes _returnvalue)
    (`KismetArrayLibrary.Array_Remove` _static_mesh_arrays_2 (`KismetArrayLibrary.Array_LastIndex` _static_mesh_arrays_2))
    (else
      (`KismetSystemLibrary.PrintString` "No elements to delete"))))

(fn `Get_StaticMesh`
  (params (Type :type "/Game/Modular_Kit/Modular_Warehouse/Blueprints/Data/MeshType Enum" :default "NewEnumerator0"))
  (returns (`Static mesh` :type "StaticMesh Object Reference") (Door :type "Actor Class Reference"))
  (switch `/Game/Modular_Kit/Modular_Warehouse/Blueprints/Data/MeshType` Type
    (:`NewEnumerator0`
      (return "/Game/Modular_Kit/Modular_Warehouse/Meshes/Modulars/SM_LargelWall.SM_LargelWall" null))
    (:`NewEnumerator1`
      (return "/Game/Modular_Kit/Modular_Warehouse/Meshes/Modulars/SM_MediumWall.SM_MediumWall" null))
    (:`NewEnumerator2`
      (return "/Game/Modular_Kit/Modular_Warehouse/Meshes/Modulars/SM_SmallWall.SM_SmallWall" null))
    (:`NewEnumerator3`
      (return "/Game/Modular_Kit/Modular_Warehouse/Meshes/Modulars/SM_Extra_SmallWall.SM_Extra_SmallWall" null))
    (:`NewEnumerator4`
      (return "/Game/Modular_Kit/Modular_Warehouse/Meshes/Modulars/SM_Door_Frame.SM_Door_Frame" "/Game/Modular_Kit/Modular_Warehouse/Blueprints/Door_BP/SingleDoor.SingleDoor_C"))
    (:`NewEnumerator5`
      (return "/Game/Modular_Kit/Modular_Warehouse/Meshes/Modulars/SM_GarageDoor_Frame.SM_GarageDoor_Frame" "/Game/Modular_Kit/Modular_Warehouse/Blueprints/Door_BP/GarageDoor.GarageDoor_C"))
    (:`NewEnumerator6`
      (return "/Game/Modular_Kit/Modular_Warehouse/Meshes/Modulars/SM_Window.SM_Window" null))
    (:`NewEnumerator7`
      (return "/Game/Modular_Kit/Modular_Warehouse/Meshes/Modulars/SM_SmallWindow.SM_SmallWindow" null))
    (:`NewEnumerator8`
      (return "/Game/Modular_Kit/Modular_Warehouse/Meshes/Modulars/SM_SideWall.SM_SideWall" null))
    (:`NewEnumerator9`
      (return "/Game/Modular_Kit/Modular_Warehouse/Meshes/Modulars/SM_SideWall_01.SM_SideWall_01" null))
    (:`NewEnumerator10`
      (return "/Game/Modular_Kit/Modular_Warehouse/Meshes/Modulars/SM_DoubleDoor_Frame.SM_DoubleDoor_Frame" "/Game/Modular_Kit/Modular_Warehouse/Blueprints/Door_BP/DoubleDoor.DoubleDoor_C"))
    (:`NewEnumerator11`
      (return "/Game/Modular_Kit/Modular_Warehouse/Meshes/Modulars/SM_Extra_SmallWall1.SM_Extra_SmallWall1" null))))

(fn `UserConstructionScript`
  (set `self.Current_DoorIndex` 0)
  (for _array_element (`self.Static_Mesh_Arrays`)
    (bind (_previoustransform _type _myendpoint _hasdoor_) (break `/Game/Modular_Kit/Modular_Warehouse/Blueprints/Data/StaticMesh_Struct` _array_element))
    (bind _returnvalue (`AddComponent|NODE_AddStaticMeshComponent-1` :`RelativeTransform` _previoustransform))
    (`StaticMeshComponent.SetStaticMesh` _returnvalue (`self.Get_StaticMesh` _type))
    (`PrimitiveComponent.SetMaterial` _returnvalue 0 (`self.Warehouse_Material`))
    (if _hasdoor_
      (`self.K2_AttachToComponent` (`|GetArrayItem` (`self.Doors_Array`) (`self.Current_DoorIndex`)) _returnvalue "Door" "SnapToTarget" "SnapToTarget" "SnapToTarget" true)
      (`/Engine/EditorBlueprintResources/StandardMacros.IncrementInt` (`self.Current_DoorIndex`)
        (:`  `
          _)))
    (if (`self.Refresh`)
      (set `self.Refresh` false))))