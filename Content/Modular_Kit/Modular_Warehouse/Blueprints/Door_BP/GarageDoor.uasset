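; Garage door Blueprint for a modular warehouse kit that the player opens and closes with the E key.
; Front and rear trigger boxes enable input for the player when that side has buttons, and any end overlap disables it.
; E alternately plays and reverses a Timeline rotating the door mesh's roll, with a DoOnce reset by a delay after updates.
; The Construction Script applies the material and adds the optional button meshes.
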(event `self.Collision_Box_F.OnComponentBeginOverlap`
  (params (OverlappedComponent :type "PrimitiveComponent Object Reference") (OtherActor :type "Actor Object Reference") (OtherComp :type "PrimitiveComponent Object Reference") (OtherBodyIndex :type Integer) (bFromSweep :type Boolean) (SweepResult :type "HitResult Structure (by ref)"))
  ;[1 0.3229 0.3229] Trigger_can_openDoor
  (if (== OtherActor (`GameplayStatics.GetPlayerCharacter` 0))
    (if (`self.Buttons Outside?`)
      (`self.EnableInput` (`GameplayStatics.GetPlayerController` 0)))))

(event `self.Collision_Box_F.OnComponentEndOverlap`
  (params (OverlappedComponent :type "PrimitiveComponent Object Reference") (OtherActor :type "Actor Object Reference") (OtherComp :type "PrimitiveComponent Object Reference") (OtherBodyIndex :type Integer))
  ;[1 0.3229 0.3229] Trigger_can_openDoor
  (`self.DisableInput` (`GameplayStatics.GetPlayerController` 0)))

(event `Key|E`
  (params (Key :type "Key Structure"))
  ;[1 1 1] Door Rotation
  (:`Pressed`
    (`/Engine/EditorBlueprintResources/StandardMacros.DoOnce` false :!label _label
      (:`Completed`
        (`/Engine/EditorBlueprintResources/StandardMacros.FlipFlop`
          (:`A`
            (bind (_direction _rotation) (`Timeline|DoorRotation` :!label _label_2)
              (:`Update`
                (`SceneComponent.K2_SetRelativeRotation` (`self.Door_Mesh`) (`KismetMathLibrary.MakeRotator` _rotation) false false)
                (`KismetSystemLibrary.Delay` 1.5)
                (goto _label :!via `Reset`))))
          (:`B`
            (goto _label_2 :!via `Reverse`)))))))

(event `self.Collision_Box_R.OnComponentBeginOverlap`
  (params (OverlappedComponent :type "PrimitiveComponent Object Reference") (OtherActor :type "Actor Object Reference") (OtherComp :type "PrimitiveComponent Object Reference") (OtherBodyIndex :type Integer) (bFromSweep :type Boolean) (SweepResult :type "HitResult Structure (by ref)"))
  ;[1 0.3229 0.3229] Trigger_can_openDoor
  (if (== OtherActor (`GameplayStatics.GetPlayerCharacter` 0))
    (if (`self.Buttons Inside?`)
      (`self.EnableInput` (`GameplayStatics.GetPlayerController` 0)))))

(event `self.Collision_Box_R.OnComponentEndOverlap`
  (params (OverlappedComponent :type "PrimitiveComponent Object Reference") (OtherActor :type "Actor Object Reference") (OtherComp :type "PrimitiveComponent Object Reference") (OtherBodyIndex :type Integer))
  ;[1 0.3229 0.3229] Trigger_can_openDoor
  (`self.DisableInput` (`GameplayStatics.GetPlayerController` 0)))

(fn `UserConstructionScript`
  (`PrimitiveComponent.SetMaterial` (`self.Door_Mesh`) 0 (`self.Material`))
  (if (`self.Buttons Outside?`)
    (`AddComponent|NODE_AddStaticMeshComponent-0` :`RelativeTransform` (`SceneComponent.GetRelativeTransform` (`self.Front_Buttons`))))
  (if (`self.Buttons Inside?`)
    (`AddComponent|NODE_AddStaticMeshComponent-1` :`RelativeTransform` (`SceneComponent.GetRelativeTransform` (`self.Rear_Buttons`)))))