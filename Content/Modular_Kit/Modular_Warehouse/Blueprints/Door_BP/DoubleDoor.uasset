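; Interactive double door that the player opens and closes with the E key while inside one of its front or rear trigger boxes.
; Overlaps enable or disable input and set side flags; the rear flag decides the swing direction.
; The DoorRotation timeline drives both leaves with mirrored yaw, keeping the current sign once moving, and reverses to close.
; The construction script applies the chosen material to both leaves.
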(event `self.Collision_Box_F1.OnComponentBeginOverlap`
  (params (OverlappedComponent :type "PrimitiveComponent Object Reference") (OtherActor :type "Actor Object Reference") (OtherComp :type "PrimitiveComponent Object Reference") (OtherBodyIndex :type Integer) (bFromSweep :type Boolean) (SweepResult :type "HitResult Structure (by ref)"))
  ;[1 0.3229 0.3229] Trigger_can_openDoor
  (if (== (stale `self.Collision_Box_F.OnComponentBeginOverlap` OtherActor) (`GameplayStatics.GetPlayerCharacter` 0)) :!label _label
    (set `self.Can Open F` true)
    (`self.EnableInput` (`GameplayStatics.GetPlayerController` 0))))

(event `self.Collision_Box_F.OnComponentBeginOverlap`
  (params (OverlappedComponent :type "PrimitiveComponent Object Reference") (OtherActor :type "Actor Object Reference") (OtherComp :type "PrimitiveComponent Object Reference") (OtherBodyIndex :type Integer) (bFromSweep :type Boolean) (SweepResult :type "HitResult Structure (by ref)"))
  ;[1 0.3229 0.3229] Trigger_can_openDoor
  (goto _label))

(event `self.Collision_Box_F1.OnComponentEndOverlap`
  (params (OverlappedComponent :type "PrimitiveComponent Object Reference") (OtherActor :type "Actor Object Reference") (OtherComp :type "PrimitiveComponent Object Reference") (OtherBodyIndex :type Integer))
  ;[1 0.3229 0.3229] Trigger_can_openDoor
  (set `self.Can Open F` false :!label _label_2)
  (`self.DisableInput` (`GameplayStatics.GetPlayerController` 0)))

(event `self.Collision_Box_F.OnComponentEndOverlap`
  (params (OverlappedComponent :type "PrimitiveComponent Object Reference") (OtherActor :type "Actor Object Reference") (OtherComp :type "PrimitiveComponent Object Reference") (OtherBodyIndex :type Integer))
  ;[1 0.3229 0.3229] Trigger_can_openDoor
  (goto _label_2))

(event `Key|E`
  (params (Key :type "Key Structure"))
  (bind (_relativerotation_roll _relativerotation_pitch _relativerotation_yaw) (`KismetMathLibrary.BreakRotator` (`SceneComponent.RelativeRotation` (`self.Door_L`))))
  (bind (_relativerotation_roll_2 _relativerotation_pitch_2 _relativerotation_yaw_2) (`KismetMathLibrary.BreakRotator` (`SceneComponent.RelativeRotation` (`self.Door_L`))))
  (bind _returnvalue (== _relativerotation_yaw_2 0.0))
  ;[1 1 1] Door Rotation
  (:`Pressed`
    (if _returnvalue
      (bind (_direction _rotation) (`Timeline|DoorRotation` :!label _label_3)
        (:`Update`
          (bind _returnvalue_2 (* -1 _rotation))
          (bind _returnvalue_3 (select `bool` _returnvalue :`false` (select `bool` (> _relativerotation_yaw 0.0) :`false` _returnvalue_2 :`true` _rotation) :`true` (select `bool` (`self.Can Open R`) :`false` _returnvalue_2 :`true` _rotation)))
          (`SceneComponent.K2_SetRelativeRotation` (`self.Door_L`) (`KismetMathLibrary.MakeRotator` 0.0 0.0 _returnvalue_3) false false)
          (`SceneComponent.K2_SetRelativeRotation` (`self.Door_R`) (`KismetMathLibrary.MakeRotator` 0.0 0.0 (- 180.0 _returnvalue_3)) false false)))
      (else
        (goto _label_3 :!via `Reverse`)))))

(event `self.Collision_BoxR1.OnComponentBeginOverlap`
  (params (OverlappedComponent :type "PrimitiveComponent Object Reference") (OtherActor :type "Actor Object Reference") (OtherComp :type "PrimitiveComponent Object Reference") (OtherBodyIndex :type Integer) (bFromSweep :type Boolean) (SweepResult :type "HitResult Structure (by ref)"))
  ;[1 0.3229 0.3229] Trigger_can_openDoor
  (if (== (stale `self.Collision_BoxR.OnComponentBeginOverlap` OtherActor) (`GameplayStatics.GetPlayerCharacter` 0)) :!label _label_4
    (set `self.Can Open R` true)
    (`self.EnableInput` (`GameplayStatics.GetPlayerController` 0))))

(event `self.Collision_BoxR.OnComponentBeginOverlap`
  (params (OverlappedComponent :type "PrimitiveComponent Object Reference") (OtherActor :type "Actor Object Reference") (OtherComp :type "PrimitiveComponent Object Reference") (OtherBodyIndex :type Integer) (bFromSweep :type Boolean) (SweepResult :type "HitResult Structure (by ref)"))
  ;[1 0.3229 0.3229] Trigger_can_openDoor
  (goto _label_4))

(event `self.Collision_BoxR1.OnComponentEndOverlap`
  (params (OverlappedComponent :type "PrimitiveComponent Object Reference") (OtherActor :type "Actor Object Reference") (OtherComp :type "PrimitiveComponent Object Reference") (OtherBodyIndex :type Integer))
  ;[1 0.3229 0.3229] Trigger_can_openDoor
  (set `self.Can Open R` false :!label _label_5)
  (`self.DisableInput` (`GameplayStatics.GetPlayerController` 0)))

(event `self.Collision_BoxR.OnComponentEndOverlap`
  (params (OverlappedComponent :type "PrimitiveComponent Object Reference") (OtherActor :type "Actor Object Reference") (OtherComp :type "PrimitiveComponent Object Reference") (OtherBodyIndex :type Integer))
  ;[1 0.3229 0.3229] Trigger_can_openDoor
  (goto _label_5))

(fn `UserConstructionScript`
  (`PrimitiveComponent.SetMaterial` (`self.Door_L`) 0 (`self.Material`))
  (`PrimitiveComponent.SetMaterial` (`self.Door_R`) 0 (`self.Material`)))