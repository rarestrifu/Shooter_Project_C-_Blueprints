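; Modular water pipe builder that assembles a pipe run from long, medium, short, left and right static mesh pieces.
; Events append a piece at the previous one's "End" socket transform or delete the last piece.
; Each piece's type and start/end transforms are stored in PipeStruct, from which the Construction Script rebuilds the run.
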(event `Delete Last`
  ;[0.2125 1 0.6325] Doors
  (`self.Delete_Last_Component`))

(event `Long Pipe`
  ;[0.2125 0.5081 1] Walls
  (`self.Add_Pipe` "NewEnumerator0"))

(event `Medium Pipe`
  ;[0.2125 0.5081 1] Walls
  (`self.Add_Pipe` "NewEnumerator1"))

(event `Short Pipe`
  ;[0.2125 0.5081 1] Walls
  (`self.Add_Pipe` "NewEnumerator2"))

(event `Right`
  ;[0.2125 0.5081 1] Walls
  (`self.Add_Pipe` "NewEnumerator3"))

(event `Left`
  ;[0.2125 0.5081 1] Walls
  (`self.Add_Pipe` "NewEnumerator4"))

(fn `Add_Pipe`
  (params (Mesh :type "/Game/Modular_Kit/Modular_Warehouse/Blueprints/Data/PipeType Enum" :default "NewEnumerator0"))
  (bind _pipestruct (`self.PipeStruct`))
  (bind (_output_pervious_pipe _output_myend_pipe) (break `/Game/Modular_Kit/Modular_Warehouse/Blueprints/Data/Pipe_Struct` (`|GetArrayItem` _pipestruct (`KismetArrayLibrary.Array_LastIndex` _pipestruct))))
  (bind _returnvalue (select `bool` (> (`KismetArrayLibrary.Array_Length` (`self.PipeStruct`)) 0) :`true` _output_myend_pipe))
  (bind _returnvalue_2 (`AddComponent|NODE_AddStaticMeshComponent-0` :`RelativeTransform` _returnvalue))
  (`StaticMeshComponent.SetStaticMesh` _returnvalue_2 (`self.Get_StaticMesh` Mesh))
  (`KismetArrayLibrary.Array_Add` (`self.Pipes_Array`) _returnvalue_2)
  (`KismetArrayLibrary.Array_Add` (`self.PipeStruct`) (make `/Game/Modular_Kit/Modular_Warehouse/Blueprints/Data/Pipe_Struct` _returnvalue (`SceneComponent.GetSocketTransform` _returnvalue_2 "End" "RTS_Actor") Mesh))
  (`SceneComponent.SetVisibility` (`self.Arrow`) false false))

(fn `Delete_Last_Component`
  (bind _pipes_array (`self.Pipes_Array`))
  (bind _pipestruct (`self.PipeStruct`))
  (bind _returnvalue (`KismetArrayLibrary.Array_LastIndex` _pipes_array))
  (if (> (`KismetArrayLibrary.Array_Length` (`self.PipeStruct`)) 0)
    (`ActorComponent.K2_DestroyComponent` (`|GetArrayItem` _pipes_array _returnvalue))
    (`KismetArrayLibrary.Array_Remove` _pipes_array _returnvalue)
    (`KismetArrayLibrary.Array_Remove` _pipestruct (`KismetArrayLibrary.Array_LastIndex` _pipestruct))
    (else
      (`KismetSystemLibrary.PrintString` "No elements to delete"))))

(fn `Get_StaticMesh`
  (params (Type :type "/Game/Modular_Kit/Modular_Warehouse/Blueprints/Data/PipeType Enum" :default "NewEnumerator0"))
  (returns (`Static mesh` :type "StaticMesh Object Reference"))
  (switch `/Game/Modular_Kit/Modular_Warehouse/Blueprints/Data/PipeType` Type
    (:`NewEnumerator0`
      (return "/Game/Modular_Kit/Modular_Warehouse/Meshes/Props/Water_Pipe_Long.Water_Pipe_Long"))
    (:`NewEnumerator1`
      (return "/Game/Modular_Kit/Modular_Warehouse/Meshes/Props/Water_Pipe_Medium.Water_Pipe_Medium"))
    (:`NewEnumerator2`
      (return "/Game/Modular_Kit/Modular_Warehouse/Meshes/Props/Water_Pipe_Small.Water_Pipe_Small"))
    (:`NewEnumerator3`
      (return "/Game/Modular_Kit/Modular_Warehouse/Meshes/Props/Water_Pipe_right.Water_Pipe_right"))
    (:`NewEnumerator4`
      (return "/Game/Modular_Kit/Modular_Warehouse/Meshes/Props/Water_Pipe_left.Water_Pipe_left"))))

(fn `UserConstructionScript`
  (for _array_element (`self.PipeStruct`)
    (bind (_pervious_pipe _myend_pipe _pipetype) (break `/Game/Modular_Kit/Modular_Warehouse/Blueprints/Data/Pipe_Struct` _array_element))
    (bind _returnvalue (`AddComponent|NODE_AddStaticMeshComponent-1` :`RelativeTransform` _pervious_pipe))
    (`StaticMeshComponent.SetStaticMesh` _returnvalue (`self.Get_StaticMesh` _pipetype))
    (if (`self.Refresh`)
      (set `self.Refresh` false))))