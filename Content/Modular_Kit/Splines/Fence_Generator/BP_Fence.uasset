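; Spline-driven fence generator that builds poles, bars and optional traverses as HISM instances in the construction script.
; Each straight segment between spline points gets poles at PoleSpacing, bars at BarSpacing and traverses scaled along their forward axis to span pole gaps.
; Segments in OpenSegments get only a start pole, and poles too close to a segment end are dropped.
; A seeded random stream jitters pole and bar transforms and omits some bars.
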(fn `AddCornerPole`
  (params (`Spline Segment Index` :type Integer))
  (bind (_segment_start _segment_end) (`self.GetSplineSegment` `Spline Segment Index`))
  (bind (_returnvalue_roll _returnvalue_pitch _returnvalue_yaw) (`KismetMathLibrary.BreakRotator` (`KismetMathLibrary.FindLookAtRotation` _segment_start _segment_end)))
  (`InstancedStaticMeshComponent.AddInstanceWorldSpace` (`self.Poles_HISM`) (`KismetMathLibrary.MakeTransform` _segment_start (`KismetMathLibrary.MakeRotator` 0.0 0.0 _returnvalue_yaw))))

(fn `Get2DDirectionVector`
  (params (From :type "Vector Structure") (To :type "Vector Structure"))
  (returns (ReturnValue :type "Vector Structure"))
  (bind _ztozero (`self.ZToZero`))
  (return (`KismetMathLibrary.GetDirectionUnitVector` (* From _ztozero) (* To _ztozero))))

(fn `GetBarCount`
  (params (`Pole Segment Index` :type Integer))
  (returns (ReturnValue :type Integer))
  (bind _returnvalue_location (`KismetMathLibrary.BreakTransform` (`self.GetPoleTransform` `Pole Segment Index`)))
  (bind _splinesegmentindex (`self.SplineSegmentIndex`))
  (bind _returnvalue_location_2 (`KismetMathLibrary.BreakTransform` (`self.GetPoleTransform` (+ `Pole Segment Index` 1))))
  (return (- (`KismetMathLibrary.Round` (/ (`KismetMathLibrary.Vector_Distance2D` _returnvalue_location (`KismetMathLibrary.SelectVector` _returnvalue_location_2 (`.Segment End` (`self.GetSplineSegment` _splinesegmentindex)) (not (== `Pole Segment Index` (`self.GetPoleCount` _splinesegmentindex))))) (`self.BarSpacing`))) (`KismetMathLibrary.SelectInt` 1 2 (`self.bPoleExcluded`)))))

(fn `GetBarTransform`
  (params (BarIndex :type Integer))
  (returns (ReturnValue :type "Transform Structure"))
  (bind _polesegmentindex (`self.PoleSegmentIndex`))
  (bind _returnvalue_location (`KismetMathLibrary.BreakTransform` (`self.GetPoleTransform` _polesegmentindex)))
  (bind _returnvalue_location_2 (`KismetMathLibrary.BreakTransform` (`self.GetPoleTransform` (+ _polesegmentindex -1))))
  (bind _returnvalue_location_3 (`KismetMathLibrary.BreakTransform` (`self.GetPoleTransform` (+ _polesegmentindex 1))))
  (bind _returnvalue (`self.Get2DDirectionVector` _returnvalue_location _returnvalue_location_3))
  (bind (_returnvalue_x _returnvalue_y) (`KismetMathLibrary.BreakVector` (+ _returnvalue_location (* (* _returnvalue (`self.BarSpacing`)) (+ BarIndex (`KismetMathLibrary.SelectInt` 0 1 (`self.bPoleExcluded`)))))))
  (return (`self.RandomizeBarTransform` (`KismetMathLibrary.MakeTransform` (`KismetMathLibrary.MakeVector` _returnvalue_x _returnvalue_y (`KismetMathLibrary.FMin` (.z (`KismetMathLibrary.SelectVector` _returnvalue_location_2 _returnvalue_location (`self.bPoleExcluded`))) (.z _returnvalue_location_3))) (`KismetMathLibrary.MakeRotFromX` _returnvalue)))))

(fn `GetPoleCount`
  (params (`Spline Segment Index` :type Integer))
  (returns (ReturnValue :type Integer))
  (return (`KismetMathLibrary.FTrunc` (/ (`.Segment Length` (`self.GetSplineSegment` `Spline Segment Index`)) (`self.PoleSpacing`)))))

(fn `GetPoleTransform`
  (params (PoleSegmentIndex :type Integer))
  (returns (ReturnValue :type "Transform Structure"))
  (bind (_segment_start _segment_end _segment_length) (`self.GetSplineSegment` (`self.SplineSegmentIndex`)))
  (bind (_returnvalue_roll _returnvalue_pitch _returnvalue_yaw) (`KismetMathLibrary.BreakRotator` (`KismetMathLibrary.FindLookAtRotation` _segment_start _segment_end)))
  (bind (_returnvalue_x _returnvalue_y _returnvalue_z) (`KismetMathLibrary.BreakVector` (`KismetMathLibrary.GetDirectionUnitVector` _segment_start _segment_end)))
  (bind (_returnvalue_x_2 _returnvalue_y_2) (`KismetMathLibrary.BreakVector` (`self.Get2DDirectionVector` _segment_start _segment_end)))
  (return (`self.RandomizePoleTransform` (`KismetMathLibrary.MakeTransform` (+ _segment_start (* (* (`KismetMathLibrary.MakeVector` _returnvalue_x_2 _returnvalue_y_2 _returnvalue_z) (* (`self.PoleSpacing`) (/ (`KismetMathLibrary.FMax` _segment_length 1.0) (`KismetMathLibrary.FMax` (`KismetMathLibrary.Vector_Distance2D` _segment_start _segment_end) 1.0)))) PoleSegmentIndex)) (`KismetMathLibrary.MakeRotator` 0.0 0.0 _returnvalue_yaw)))))

(fn `GetSplineSegment`
  (params (`Spline Segment Index` :type Integer))
  (returns (`Segment Start` :type "Vector Structure") (`Segment End` :type "Vector Structure") (`Segment Length` :type "Float (double-precision)"))
  (bind _spline (`self.Spline`))
  (bind _returnvalue (`SplineComponent.GetLocationAtSplinePoint` _spline (+ `Spline Segment Index` 1) "World"))
  (bind _returnvalue_2 (`SplineComponent.GetLocationAtSplinePoint` _spline `Spline Segment Index` "World"))
  (return _returnvalue_2 _returnvalue (`KismetMathLibrary.Vector_Distance2D` _returnvalue_2 _returnvalue)))

(fn `GetSplineSegmentCount`
  (returns (SplineSegmentCount :type Integer))
  (return (- (`SplineComponent.GetNumberOfSplinePoints` (`self.Spline`)) 1)))

(fn `GetTraverseTransform`
  (params (SegmentPoleIndex :type Integer))
  (returns (ReturnValue :type "Transform Structure"))
  (bind _returnvalue_location (`KismetMathLibrary.BreakTransform` (`self.GetPoleTransform` SegmentPoleIndex)))
  (bind _splinesegmentindex (`self.SplineSegmentIndex`))
  (bind _returnvalue_location_2 (`KismetMathLibrary.BreakTransform` (`self.GetPoleTransform` (- SegmentPoleIndex 1))))
  (bind _returnvalue_location_3 (`KismetMathLibrary.BreakTransform` (`self.GetPoleTransform` (+ SegmentPoleIndex 1))))
  (bind (_returnvalue_roll _returnvalue_pitch _returnvalue_yaw) (`KismetMathLibrary.BreakRotator` (`KismetMathLibrary.FindLookAtRotation` _returnvalue_location _returnvalue_location_3)))
  (bind _returnvalue (`StaticMesh.GetBounds` (`StaticMeshComponent.StaticMesh` (`self.Traverses_HISM`))))
  (bind _returnvalue_2 (* (.y (`.BoxExtent` (`KismetMathLibrary.BreakBoxSphereBounds` _returnvalue))) 2.0))
  (bind _returnvalue_3 (* (.x (`.BoxExtent` (`KismetMathLibrary.BreakBoxSphereBounds` _returnvalue))) 2.0))
  (bind _returnvalue_4 (/ (`KismetMathLibrary.Vector_Distance2D` _returnvalue_location (`KismetMathLibrary.SelectVector` _returnvalue_location_3 (`.Segment End` (`self.GetSplineSegment` _splinesegmentindex)) (not (== SegmentPoleIndex (`self.GetPoleCount` _splinesegmentindex))))) (select `/Game/Modular_Kit/Splines/Fence_Generator/Enums/TraverseAxis` (`self.TraverseForwardAxis`) :`NewEnumerator0` _returnvalue_3 :`NewEnumerator1` _returnvalue_3 :`NewEnumerator2` _returnvalue_2 :`NewEnumerator3` _returnvalue_2)))
  (bind _returnvalue_5 (`KismetMathLibrary.MakeVector` _returnvalue_4 1.0 1.0))
  (bind _returnvalue_6 (`KismetMathLibrary.MakeVector` 1.0 _returnvalue_4 1.0))
  (return (`KismetMathLibrary.MakeTransform` (`KismetMathLibrary.MakeVector` (.x _returnvalue_location) (.y _returnvalue_location) (`KismetMathLibrary.FMin` (.z (`KismetMathLibrary.SelectVector` _returnvalue_location_2 _returnvalue_location (`self.bPoleExcluded`))) (.z _returnvalue_location_3))) (`KismetMathLibrary.MakeRotator` 0.0 0.0 (select `/Game/Modular_Kit/Splines/Fence_Generator/Enums/TraverseAxis` (`self.TraverseForwardAxis`) :`NewEnumerator0` _returnvalue_yaw :`NewEnumerator1` (+ _returnvalue_yaw 180.0) :`NewEnumerator2` (+ _returnvalue_yaw -90.0) :`NewEnumerator3` (+ _returnvalue_yaw 90.0))) (select `/Game/Modular_Kit/Splines/Fence_Generator/Enums/TraverseAxis` (`self.TraverseForwardAxis`) :`NewEnumerator0` _returnvalue_5 :`NewEnumerator1` _returnvalue_5 :`NewEnumerator2` _returnvalue_6 :`NewEnumerator3` _returnvalue_6))))

(fn `IsBarNotMissing`
  (returns (BarNotMissing :type Boolean))
  (return (> (`KismetMathLibrary.RandomFloatInRangeFromStream` 0.0 100.0 (`self.RandomStream`)) (`self.BarsMissing (%)`))))

(fn `IsPoleNotExcluded`
  (params (SegmentPoleTransform :type "Transform Structure (by ref)"))
  (returns (NotExcluded :type Boolean))
  (bind _splinesegmentindex (`self.SplineSegmentIndex`))
  (bind _returnvalue (and (== (.location SegmentPoleTransform) (`.Segment End` (`self.GetSplineSegment` _splinesegmentindex)) :`ErrorTolerance` (`self.PoleSpacingMin`)) (!= (`self.PoleSegmentIndex`) 0)))
  (return (not (select `bool` (`self.bPlaceLastPole`) :`false` (or _returnvalue (== _splinesegmentindex (`self.GetSplineSegmentCount`))) :`true` _returnvalue))))

(fn `IsSegmentNotExcluded`
  (params (SplineSegmentIndex :type "Integer (by ref)"))
  (returns (SegmentNotExcluded :type Boolean))
  (return (== (`KismetArrayLibrary.Array_Find` (`self.OpenSegments`) SplineSegmentIndex) -1)))

(fn `RandomizeBarTransform`
  (params (BarTransform :type "Transform Structure"))
  (returns (RandomBarTransform :type "Transform Structure"))
  (bind (_minbarlocation_x _minbarlocation_y _minbarlocation_z) (`KismetMathLibrary.BreakVector` (`self.MinBarLocation`)))
  (bind (_maxbarlocation_x _maxbarlocation_y _maxbarlocation_z) (`KismetMathLibrary.BreakVector` (`self.MaxBarLocation`)))
  (bind (_minbarrotation_roll _minbarrotation_pitch _minbarrotation_yaw) (`KismetMathLibrary.BreakRotator` (`self.MinBarRotation`)))
  (bind (_maxbarrotation_roll _maxbarrotation_pitch _maxbarrotation_yaw) (`KismetMathLibrary.BreakRotator` (`self.MaxBarRotation`)))
  (bind _randomstream (`self.RandomStream`))
  (bind _returnvalue (`KismetMathLibrary.RandomFloatInRangeFromStream` (`self.MinBarScale`) (`self.MaxBarScale`) _randomstream))
  (return (`KismetMathLibrary.MakeTransform` (+ BarTransform_Location (`KismetMathLibrary.MakeVector` (`KismetMathLibrary.RandomFloatInRangeFromStream` _minbarlocation_x _maxbarlocation_x _randomstream) (`KismetMathLibrary.RandomFloatInRangeFromStream` _minbarlocation_y _maxbarlocation_y _randomstream) (`KismetMathLibrary.RandomFloatInRangeFromStream` _minbarlocation_z _maxbarlocation_z _randomstream))) (`KismetMathLibrary.ComposeRotators` BarTransform_Rotation (`KismetMathLibrary.MakeRotator` (`KismetMathLibrary.RandomFloatInRangeFromStream` _minbarrotation_roll _maxbarrotation_roll _randomstream) (`KismetMathLibrary.RandomFloatInRangeFromStream` _minbarrotation_pitch _maxbarrotation_pitch _randomstream) (`KismetMathLibrary.RandomFloatInRangeFromStream` _minbarrotation_yaw _maxbarrotation_yaw _randomstream))) (`KismetMathLibrary.MakeVector` _returnvalue _returnvalue _returnvalue))))

(fn `RandomizePoleTransform`
  (params (PoleTransform :type "Transform Structure"))
  (returns (RandomPoleTransform :type "Transform Structure"))
  (bind (_maxpolerotation_roll _maxpolerotation_pitch _maxpolerotation_yaw) (`KismetMathLibrary.BreakRotator` (`self.MaxPoleRotation`)))
  (bind _randomstream (`self.RandomStream`))
  (bind (_minpolelocation_x _minpolelocation_y _minpolelocation_z) (`KismetMathLibrary.BreakVector` (`self.MinPoleLocation`)))
  (bind (_maxpolelocation_x _maxpolelocation_y _maxpolelocation_z) (`KismetMathLibrary.BreakVector` (`self.MaxPoleLocation`)))
  (bind (_minpolerotation_roll _minpolerotation_pitch _minpolerotation_yaw) (`KismetMathLibrary.BreakRotator` (`self.MinPoleRotation`)))
  (bind _returnvalue (`KismetMathLibrary.RandomFloatInRangeFromStream` (`self.MinPoleScale`) (`self.MaxPoleScale`) _randomstream))
  (return (`KismetMathLibrary.MakeTransform` (+ PoleTransform_Location (`KismetMathLibrary.MakeVector` (`KismetMathLibrary.RandomFloatInRangeFromStream` _minpolelocation_x _maxpolelocation_x _randomstream) (`KismetMathLibrary.RandomFloatInRangeFromStream` _minpolelocation_y _maxpolelocation_y _randomstream) (`KismetMathLibrary.RandomFloatInRangeFromStream` _minpolelocation_z _maxpolelocation_z _randomstream))) (`KismetMathLibrary.ComposeRotators` PoleTransform_Rotation (`KismetMathLibrary.MakeRotator` (`KismetMathLibrary.RandomFloatInRangeFromStream` _minpolerotation_roll _maxpolerotation_roll _randomstream) (`KismetMathLibrary.RandomFloatInRangeFromStream` _minpolerotation_pitch _maxpolerotation_pitch _randomstream) (`KismetMathLibrary.RandomFloatInRangeFromStream` _minpolerotation_yaw _maxpolerotation_yaw _randomstream))) (`KismetMathLibrary.MakeVector` _returnvalue _returnvalue _returnvalue))))

(fn `SetupData`
  (set `self.RandomStream` (`KismetMathLibrary.MakeRandomStream` 0))
  (`StaticMeshComponent.SetStaticMesh` (`self.Poles_HISM`) (`self.PoleMesh`))
  (`StaticMeshComponent.SetStaticMesh` (`self.Bars_HISM`) (`self.BarMesh`))
  (`StaticMeshComponent.SetStaticMesh` (`self.Traverses_HISM`) (`self.TraverseMesh`)))

(fn `UserConstructionScript`
  (bind _traverses_hism (`self.Traverses_HISM`))
  (bind _splinesegmentindex (`self.SplineSegmentIndex`))
  (bind _returnvalue (`self.GetPoleTransform` (`self.PoleSegmentIndex`)))
  (`|ExecutionSequence`
    (:`then_0`
      (`self.SetupData`) ; Assign user selected meshes to the HISM components
    )
    (:`then_1`
      (for _index (range (+ (`self.GetSplineSegmentCount`) 1))
        (bind _output_get (set `self.SplineSegmentIndex` _index)) ; Store segment index for later use
        (if (`self.IsSegmentNotExcluded` _output_get)
          (for _index_2 (range (+ (`self.GetPoleCount` _splinesegmentindex) 1))
            (set `self.PoleSegmentIndex` _index_2) ; Store segment index for later use
            (`|ExecutionSequence`
              (:`then_0`
                ;[1 1 1] Place poles along each spline segment using Pole Spacing. Swap pole for a bar if excluded by Pole Spacing Min parameter.
                (if (`self.IsPoleNotExcluded` _returnvalue)
                  (`InstancedStaticMeshComponent.AddInstanceWorldSpace` (`self.Poles_HISM`) _returnvalue)
                  (set `self.bPoleExcluded` false)
                  (else
                    (set `self.bPoleExcluded` true))))
              (:`then_1`
                ;[1 1 1] Place bars between the poles
                (for _index_3 (range (+ (`self.GetBarCount` (`self.PoleSegmentIndex`)) 1))
                  (if (`self.IsBarNotMissing`)
                    (`InstancedStaticMeshComponent.AddInstanceWorldSpace` (`self.Bars_HISM`) (`self.GetBarTransform` _index_3)))))
              (:`then_2`
                ;[1 1 1] Place traverses between the poles
                (if (`KismetSystemLibrary.IsValid` (`StaticMeshComponent.StaticMesh` _traverses_hism))
                  (`InstancedStaticMeshComponent.AddInstanceWorldSpace` _traverses_hism (`self.GetTraverseTransform` (`self.PoleSegmentIndex`)))))))
          (else
            (`self.AddCornerPole` _splinesegmentindex) ; Add start pole if we skip the segment
          ))))))