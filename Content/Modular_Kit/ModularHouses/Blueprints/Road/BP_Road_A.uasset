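; BP_Road_A is a modular road segment for the modular houses kit that builds its meshes in the construction script.
; With RoadEnd set, it adds one end-cap mesh picked by RoadMesh.
; Otherwise it adds separate left and right meshes, picked independently by Side1 and Side2 from plain road and driveway variants.
; The event graph holds no gameplay logic.
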(fn `UserConstructionScript`
  (if (`self.Road End`)
    (bind _output_get (set `self.Array` (`|MakeArray` "/Game/Modular_Kit/ModularHouses/Meshes/Road/SM_Road_03_End.SM_Road_03_End" "/Game/Modular_Kit/ModularHouses/Meshes/Road/SM_Road_02_End.SM_Road_02_End" :!type "StaticMesh Object Reference")))
    (bind _returnvalue (`AddComponent|NODE_AddStaticMeshComponent-3`))
    (`StaticMeshComponent.SetStaticMesh` _returnvalue (`|GetArrayItem` _output_get (`self.Road Mesh`)))
    (else
      (bind _output_get_2 (set `self.Array` (`|MakeArray` "/Game/Modular_Kit/ModularHouses/Meshes/Road/SM_Road_01_Left.SM_Road_01_Left" "/Game/Modular_Kit/ModularHouses/Meshes/Road/SM_Road_Driveway_04_Left.SM_Road_Driveway_04_Left" "/Game/Modular_Kit/ModularHouses/Meshes/Road/SM_Road_Driveway_05_Left.SM_Road_Driveway_05_Left" "/Game/Modular_Kit/ModularHouses/Meshes/Road/SM_Road_Driveway_06_Left.SM_Road_Driveway_06_Left" "/Game/Modular_Kit/ModularHouses/Meshes/Road/SM_Road_Driveway_01_Left.SM_Road_Driveway_01_Left" "/Game/Modular_Kit/ModularHouses/Meshes/Road/SM_Road_Driveway_02_Left.SM_Road_Driveway_02_Left" "/Game/Modular_Kit/ModularHouses/Meshes/Road/SM_Road_Driveway_03_Left.SM_Road_Driveway_03_Left" :!type "StaticMesh Object Reference")))
      (bind _returnvalue_2 (`AddComponent|NODE_AddStaticMeshComponent-0`))
      (`StaticMeshComponent.SetStaticMesh` _returnvalue_2 (`|GetArrayItem` _output_get_2 (`self.Side_1`)))
      (bind _output_get_3 (set `self.Array_2` (`|MakeArray` "/Game/Modular_Kit/ModularHouses/Meshes/Road/SM_Road_01_Right.SM_Road_01_Right" "/Game/Modular_Kit/ModularHouses/Meshes/Road/SM_Road_Driveway_04_Right.SM_Road_Driveway_04_Right" "/Game/Modular_Kit/ModularHouses/Meshes/Road/SM_Road_Driveway_05_Right.SM_Road_Driveway_05_Right" "/Game/Modular_Kit/ModularHouses/Meshes/Road/SM_Road_Driveway_06_Right.SM_Road_Driveway_06_Right" "/Game/Modular_Kit/ModularHouses/Meshes/Road/SM_Road_Driveway_01_Right.SM_Road_Driveway_01_Right" "/Game/Modular_Kit/ModularHouses/Meshes/Road/SM_Road_Driveway_02_Right.SM_Road_Driveway_02_Right" "/Game/Modular_Kit/ModularHouses/Meshes/Road/SM_Road_Driveway_03_Right.SM_Road_Driveway_03_Right" :!type "StaticMesh Object Reference")))
      (bind _returnvalue_3 (`AddComponent|NODE_AddStaticMeshComponent-1`))
      (`StaticMeshComponent.SetStaticMesh` _returnvalue_3 (`|GetArrayItem` _output_get_3 (`self.Side_2`))))))