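; Modular CityPark construction-script Blueprint that builds a chain of deformed spline meshes along its Spline, using a chosen mesh and two materials.
; SplineMeshVar selects the layout: one mesh per spline point pair, or repeated segments at fixed Spacing along the spline length.
; Point mode copies the spline's own tangents, while spacing mode scales direction vectors by Spacing plus TangentScaleAdd.
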(fn `UserConstructionScript`
  (bind _conponent_1 (`self.Conponent 1`))
  (bind _spline (`self.Spline`))
  (bind _spline_2 (`self.Spline`))
  (bind _points (`self.Points`))
  (bind _spacing (`self.Spacing`))
  (bind (_location _tangent) (`SplineComponent.GetLocationAndTangentAtSplinePoint` _spline _points "Local"))
  (bind _returnvalue (+ _spacing (`self.Tangent Scale add`)))
  (bind (_location_2 _tangent_2) (`SplineComponent.GetLocationAndTangentAtSplinePoint` _spline (+ _points 1) "Local"))
  (set `self.Conponent 1` null)
  (switch `int` (`self.Spline Mesh Var`)
    (:`Default`
      (for _index (range (+ (- (`SplineComponent.GetNumberOfSplinePoints` (`self.Spline`)) 2) 1)) :!label _label
        (set `self.Points` _index)
        (bind _returnvalue_2 (`AddComponent|NODE_AddSplineMeshComponent-16` :!label _label_2))
        (`StaticMeshComponent.SetStaticMesh` _returnvalue_2 (`self.MainMesh`))
        (bind _output_get (set `self.Conponent 1` _returnvalue_2))
        (`PrimitiveComponent.SetMaterial` _output_get 0 (`self.Material`))
        (`PrimitiveComponent.SetMaterial` _output_get 1 (`self.Material2`))
        (switch `int` (`self.Spline Mesh Var`)
          (:`Default`
            (`SplineMeshComponent.SetStartAndEnd` _conponent_1 _location _tangent _location_2 _tangent_2 true :!label _label_3))
          (:`0`
            (goto _label_3))
          (:`1`
            (bind _returnvalue_3 (* (stale _index_2) _spacing))
            (bind _returnvalue_4 (+ _returnvalue_3 _spacing))
            (`SplineMeshComponent.SetStartAndEnd` _conponent_1 (`SplineComponent.GetLocationAtDistanceAlongSpline` _spline_2 _returnvalue_3 "Local") (* (`SplineComponent.GetDirectionAtDistanceAlongSpline` _spline_2 _returnvalue_3 "Local") _returnvalue) (`SplineComponent.GetLocationAtDistanceAlongSpline` _spline_2 _returnvalue_4 "Local") (* (`SplineComponent.GetDirectionAtDistanceAlongSpline` _spline_2 _returnvalue_4 "Local") _returnvalue) true)))))
    (:`0`
      (goto _label))
    (:`1`
      (for _index_2 (range (+ (`.ReturnValue` (`KismetMathLibrary.FMod` (`SplineComponent.GetSplineLength` _spline_2) _spacing)) 1))
        (goto _label_2)))))