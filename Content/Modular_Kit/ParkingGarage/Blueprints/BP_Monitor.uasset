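; BP_Monitor is a monitor prop that cycles through random screen images and casts a flickering glow from a spot light.
; If active at BeginPlay, it waits a random delay, creates a dynamic material and randomly picks one of two screen sizes.
; A Delay loop then re-randomizes light intensity and screen coordinates every few seconds.
; When Active turns false, the next pass zeroes emissive and light, ending the loop.
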(event `self.ReceiveBeginPlay`
  (bind _returnvalue (`KismetMathLibrary.SelectFloat` 0.0 1.0 (`KismetMathLibrary.RandomBool`)))
  (if (`self.Active`)
    (`KismetSystemLibrary.Delay` (`KismetMathLibrary.RandomFloatInRange` 0.0 3.0))
    (bind _returnvalue_2 (`PrimitiveComponent.CreateDynamicMaterialInstance` (`self.SM_Monitor`) 0 "/Game/Modular_Kit/ParkingGarage/Materials/M_Monitor.M_Monitor" "None"))
    (`MaterialInstanceDynamic.SetScalarParameterValue` _returnvalue_2 "ScreenSize" (`KismetMathLibrary.SelectFloat` 2.0 1.0 (<= (`KismetMathLibrary.RandomIntegerInRange` 0 100) 30)))
    (if (`self.Active`) :!label _label
      (`LightComponent.SetIntensity` (`self.SpotLight`) (`KismetMathLibrary.RandomFloatInRange` 120.0 200.0))
      (`MaterialInstanceDynamic.SetScalarParameterValue` _returnvalue_2 "EmissivePower" 1.5)
      (`KismetSystemLibrary.Delay` 4.0)
      (`MaterialInstanceDynamic.SetScalarParameterValue` _returnvalue_2 "ScreenX" _returnvalue)
      (`MaterialInstanceDynamic.SetScalarParameterValue` _returnvalue_2 "ScreenY" _returnvalue)
      (goto _label)
      (else
        (`MaterialInstanceDynamic.SetScalarParameterValue` _returnvalue_2 "EmissivePower" 0.0)
        (`LightComponent.SetIntensity` (`self.SpotLight`) 0.0)))))

(fn `UserConstructionScript`)