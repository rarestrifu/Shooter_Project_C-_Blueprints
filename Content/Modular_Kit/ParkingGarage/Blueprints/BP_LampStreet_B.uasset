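; Street lamp prop for the modular parking garage kit, with optional active and flickering states.
; The construction script sets the point light's mobility and intensity from its settings, or destroys the light when inactive.
; On play, a dynamic material drives the mesh's emissive color; a flicker timeline scales it and light intensity together.
; Non-flickering active lamps instead play a quiet light sound with steady glow.
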(event `self.ReceiveBeginPlay`
  (if (`self.Active`)
    (bind _returnvalue (`PrimitiveComponent.CreateDynamicMaterialInstance` (`self.SM_LampStreet_B`) 0 "/Game/Modular_Kit/ParkingGarage/Materials/M_Lamp_Street.M_Lamp_Street" "None"))
    (if (`self.Flickering`)
      (bind (_direction _newtrack_0) (`Timeline|FlickerTime` :!via `PlayFromStart`)
        (:`Update`
          (`LightComponent.SetIntensity` (`self.PointLight`) (* (`self.Intensity`) _newtrack_0))
          (`MaterialInstanceDynamic.SetVectorParameterValue` _returnvalue "EmissiveColor" (* (struct :`R` 3.8 :`G` 4.0 :`B` 1.4 :`A` 1.0) _newtrack_0))))
      (else
        (`GameplayStatics.SpawnSoundAtLocation` "/Game/Modular_Kit/ParkingGarage/Sounds/SC_Light_A.SC_Light_A" (`self.K2_GetActorLocation`) (struct) 0.25 1.0 0.0 null null)
        (`MaterialInstanceDynamic.SetVectorParameterValue` _returnvalue "EmissiveColor" (struct :`R` 3.8 :`G` 4.0 :`B` 1.4 :`A` 1.0))))))

(fn `UserConstructionScript`
  (bind _pointlight (`self.PointLight`))
  (if (`self.Active`)
    (if (`self.Stationary`)
      (`SceneComponent.SetMobility` _pointlight "Stationary")
      (elif (`self.Flickering`)
        (`SceneComponent.SetMobility` (`self.PointLight`) "Movable")))
    (`LightComponent.SetIntensity` _pointlight (`self.Intensity`))
    (else
      (`ActorComponent.K2_DestroyComponent` (`self.PointLight`)))))