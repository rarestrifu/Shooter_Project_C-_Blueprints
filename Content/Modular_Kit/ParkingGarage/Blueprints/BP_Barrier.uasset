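; BP_Barrier is a parking garage barrier that either cycles automatically when Active or stays static, optionally posed open.
; A timeline rotates the arm meshes, counter-rotating SMBarrierD, then replays after a random delay.
; A single attached motor sound has its volume switched on only mid-swing.
; Start sounds play at cycle start, after a fixed delay and on finish, with all sounds pitched by global time dilation.
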(event `self.ReceiveBeginPlay`
  (bind _returnvalue (`GameplayStatics.GetGlobalTimeDilation`))
  (if (`self.Active`)
    (`KismetSystemLibrary.Delay` 1.0)
    (`|ExecutionSequence` :!label _label
      (:`then_0`
        (`/Engine/EditorBlueprintResources/StandardMacros.DoOnce` false
          (:`Completed`
            (bind _returnvalue_2 (`GameplayStatics.SpawnSoundAttached` "/Game/Modular_Kit/ParkingGarage/Sounds/SC_Barrier.SC_Barrier" (`self.SM_Barrier_D`) "None" (0.0 0.0 0.0) (struct) "SnapToTarget" true 1.0 _returnvalue 0.0 null null)))))
      (:`then_1`
        (bind (_direction _newtrack_0) (`Timeline|BarrierOperateTime` :!via `PlayFromStart`)
          (:`Update`
            (`SceneComponent.K2_SetRelativeRotation` (`self.SM_Barrier_B`) (`KismetMathLibrary.MakeRotator` _newtrack_0) true false)
            (`SceneComponent.K2_SetRelativeRotation` (`self.SM_Barrier_C`) (`KismetMathLibrary.MakeRotator` _newtrack_0) true false)
            (`SceneComponent.K2_SetRelativeRotation` (`self.SM_Barrier_D`) (`KismetMathLibrary.MakeRotator` (* _newtrack_0 -1.0)) true false)
            (`AudioComponent.SetVolumeMultiplier` _returnvalue_2 (`KismetMathLibrary.SelectFloat` 1.0 0.0 (and (<= _newtrack_0 85.0) (>= _newtrack_0 1.0)))))
          (:`Finished`
            (`|ExecutionSequence`
              (:`then_0`
                (`KismetSystemLibrary.Delay` (`KismetMathLibrary.RandomFloatInRange` 3.0 10.0))
                (goto _label))
              (:`then_1`
                (`GameplayStatics.SpawnSoundAttached` "/Game/Modular_Kit/ParkingGarage/Sounds/SC_BarrierStart.SC_BarrierStart" (`self.SM_Barrier_A`) "None" (0.0 0.0 0.0) (struct) "SnapToTarget" true 1.0 _returnvalue 0.0 null null :!label _label_2))))))
      (:`then_2`
        (`GameplayStatics.SpawnSoundAttached` "/Game/Modular_Kit/ParkingGarage/Sounds/SC_BarrierStart.SC_BarrierStart" (`self.SM_Barrier_A`) "None" (0.0 0.0 0.0) (struct) "SnapToTarget" true 1.0 _returnvalue 0.0 null null)
        (`KismetSystemLibrary.Delay` 5.0)
        (goto _label_2)))
    (elif (`self.Open`)
      (`SceneComponent.K2_SetRelativeRotation` (`self.SM_Barrier_B`) (struct :`Roll` 90.0) false true)
      (`SceneComponent.K2_SetRelativeRotation` (`self.SM_Barrier_C`) (struct :`Roll` 90.0) false true)
      (`SceneComponent.K2_SetRelativeRotation` (`self.SM_Barrier_D`) (struct :`Roll` -90.0) false true))))

(fn `UserConstructionScript`)