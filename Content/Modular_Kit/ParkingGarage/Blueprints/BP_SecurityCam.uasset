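; Parking garage security camera prop that, when Active, pans its head with servo audio.
; After a random startup delay that staggers instances, a timeline drives the camera mesh's yaw.
; The attached sound mutes near the sweep's extremes and takes its initial pitch from global time dilation.
; The construction script offsets the mesh and, for inactive cameras, removes the point light and sets a random static angle.
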(event `self.ReceiveBeginPlay`
  (if (`self.Active`)
    (`KismetSystemLibrary.Delay` (`KismetMathLibrary.RandomFloatInRange` 0.0 10.0))
    (bind _returnvalue (`GameplayStatics.SpawnSoundAttached` "/Game/Modular_Kit/ParkingGarage/Sounds/SC_SecuritryCam.SC_SecuritryCam" (`self.SM_SecurityCam_A`) "None" (0.0 0.0 0.0) (struct) "SnapToTarget" true 1.0 (`GameplayStatics.GetGlobalTimeDilation`) 0.0 null null))
    (bind (_direction _newtrack_0) (`Timeline|CamRotateTime` :!via `PlayFromStart`)
      (:`Update`
        (`SceneComponent.K2_SetRelativeRotation` (`self.SM_SecurityCam_A`) (`KismetMathLibrary.MakeRotator` 0.0 0.0 _newtrack_0) false false)
        (`AudioComponent.SetVolumeMultiplier` _returnvalue (`KismetMathLibrary.SelectFloat` 1.0 0.0 (and (<= _newtrack_0 74.0) (>= _newtrack_0 -74.0))))))))

(fn `UserConstructionScript`
  (`SceneComponent.K2_AddRelativeLocation` (`self.SM_SecurityCam_A`) (27.299999 0.0 0.0) false true)
  (if (`self.Active`)
    (`SceneComponent.K2_AddRelativeRotation` (`self.SM_SecurityCam_A`) (`KismetMathLibrary.MakeRotator` 0.0 0.0 -90.0) false false)
    (else
      (`ActorComponent.K2_DestroyComponent` (`self.PointLight`))
      (`SceneComponent.K2_AddRelativeRotation` (`self.SM_SecurityCam_A`) (`KismetMathLibrary.MakeRotator` 0.0 0.0 (`KismetMathLibrary.RandomFloatInRange` -45.0 45.0)) false false))))